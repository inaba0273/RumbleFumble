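; Animation notify state for a punch attack that plays a swing sound on begin and resolves the hit on end.
; The end event runs a zero-length sphere trace at PunchHitSocket on the Camera channel, with debug drawing, and damages the hit actor.
; Hitting a BP_Player also plays punch sound and particles.
; The attacking player's attack is then disabled if its item is the basic BP_AttackItem, so golden gloves persist.
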(fn ReceivedNotifyEnd
  (params (MeshComp :type Skeletal%20Mesh%20Component%20Object%20Reference) (Animation :type Anim%20Sequence%20Base%20Object%20Reference))
  (bind _returnvalue (Transformation|GetSocketLocation MeshComp "PunchHitSocket"))
  (bind _returnvalue_2 (Components|GetOwner MeshComp))
  (bind (_outhit _returnvalue_3) (Collision|SphereTraceByChannel MeshComp _returnvalue _returnvalue 7e+01 "TraceTypeQuery2" false 0 "ForDuration"))
  (if _returnvalue_3
    (Game|Damage|ApplyDamage (.hitactor _outhit) 1e+01 (Variables|Default|GetEvent%20Instigator) (Components|GetOwner MeshComp))
    (if (== (Utilities|GetClass (.hitactor _outhit)) "/Game/Blueprint/BP_Player.BP_Player_C")
      (Audio|SpawnSoundatLocation _returnvalue_2 "/Game/Assets/Sounds/Punch/Player_Punch_SpounCue.Player_Punch_SpounCue" (Transformation|GetWorldLocation MeshComp) "0, 0, 0" 1.0 1.0 0.0 0 0)
      (Effects|SpawnEmitteratLocation (.hitactor _outhit) "/Game/Assets/Particles/Confetti/Punch_P.Punch_P" (.location _outhit))
      (bind _asbp_player (Utilities|Casting|CastToBP_Player _returnvalue_2))
      ;[1 1 1] 判断是否为金色拳套，若是则攻击后不会消失
      (if (== (Variables|/Game/Blueprint/BP_Player.BP_Player_C|GetCurrentAttackItemClass _asbp_player) "/Game/Blueprint/BP_AttackItem.BP_AttackItem_C")
        (Default|DisableAttack _asbp_player))
      (return false))))

(fn ReceivedNotifyBegin
  (params (MeshComp :type Skeletal%20Mesh%20Component%20Object%20Reference) (Animation :type Anim%20Sequence%20Base%20Object%20Reference) (TotalDuration :type Float%20%28single-precision%29))
  (Audio|SpawnSoundatLocation MeshComp "/Game/Assets/Sounds/Punch/Player_Swing_SoundCue.Player_Swing_SoundCue" (Transformation|GetWorldLocation MeshComp) "0, 0, 0" 1.0 1.0 0.0 0 0)
  (return false))