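; BP_SmallBomb_PVE is a small bomb for PVE mode that arms itself after a short random delay and explodes.
; StartFuze starts the fuse effect and sound, a timeline-driven color flash on a dynamic material, and timers that grow the mesh and trigger detonation.
; Detonation applies full radial damage with effects, decrements the PVE game mode's spawned bomb count, removes the mesh and sets a follow-up timer.
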(event Custom|Destroy
  (Utilities|FlowControl|Delay 2.0)
  (Actor|DestroyActor))

(event Custom|Start%20Fuze
  (Components|Activation|Activate (Variables|Default|GetFuze) false)
  (bind _returnvalue (Audio|SpawnSoundatLocation "/Game/Assets/Sounds/Bomb_Fuze.Bomb_Fuze" (Transformation|GetWorldLocation (Variables|Default|GetBomb_Mesh)) "0, 0, 0" 0.2 1.0 0.0 0 0))
  (Variables|Default|SetFuze%20Sound _returnvalue)
  (Utilities|Time|SetTimerbyFunctionName 0 "Bomb Scale Up" 0.1 true)
  (Utilities|Time|SetTimerbyFunctionName 0 "Bomb Explode" 5.0)
  (CallFunction|BombFlashRed))

(event Custom|Bomb%20Flash%20Red
  (bind _bomb_color (Timeline|Timeline_0 Play)
    (:Update
      (Rendering|Material|SetVectorParameterValue (Variables|Default|GetDynamic%20Material) "Color" (Math|Conversions|ToLinearColor(Vector) _bomb_color) :!class /Script/Engine.MaterialInstanceDynamic))))

(event EventBeginPlay
  (|CallParentFunction)
  (Utilities|FlowControl|Delay (Math|Random|RandomFloatinRange 3.0 5.0))
  (CallFunction|StartFuze))

(event Collision|EventActorBeginOverlap
  (params (OtherActor :type Actor%20Object%20Reference))
  (|CallParentFunction OtherActor) ; This node is disabled and will not be called.\nDrag off pins to build functionality.
)

(event EventTick
  (params (DeltaSeconds :type Float%20%28single-precision%29))
  (|CallParentFunction DeltaSeconds) ; This node is disabled and will not be called.\nDrag off pins to build functionality.
)

(fn ConstructionScript
  (|CallParentFunction)
  (bind _returnvalue (Rendering|Material|CreateDynamicMaterialInstance "/Game/Assets/PickupItemsMB/Materials/RedBomb_Mat.RedBomb_Mat" "None" "None" :!class /Script/Engine.KismetMaterialLibrary))
  (bind _output_get (Variables|Default|SetDynamic%20Material _returnvalue))
  (Rendering|Material|SetMaterial (Variables|Default|GetBomb_Mesh) 0 _output_get))

(fn BombScaleUp
  (Transformation|SetWorldScale3D (Variables|Default|GetBomb_Mesh) (+ (Variables|Default|GetNew%20Scale) "0.050000,0.050000,0.050000"))
  (Variables|Default|SetNew%20Scale (+ (Variables|Default|GetNew%20Scale) "0.050000,0.050000,0.050000")))

(fn BombExplode
  (bind _fuze_sound (Variables|Default|GetFuze%20Sound))
  (Components|Activation|Deactivate (Variables|Default|GetFuze))
  (if (Utilities|IsValid _fuze_sound)
    (Audio|Components|Audio|Stop _fuze_sound))
  (Components|Activation|Activate (Variables|Default|GetExplosion) false)
  (Game|Damage|ApplyRadialDamage 1.0 (Transformation|GetWorldLocation (Variables|Default|GetBomb_Mesh)) 2.4e+02 0 0 self 0 true "ECC_Visibility")
  (Class|KismetSystemLibrary|PauseTimer 0 "Bomb Scale Up")
  (bind _returnvalue (Audio|SpawnSoundatLocation "/Game/Assets/Sounds/EnvironmentSFX/Bomb_Small_Cue.Bomb_Small_Cue" (Transformation|GetWorldLocation (Variables|Default|GetExplosion)) "0, 0, 0" 0.5 1.0 0.0 0 0))
  (Variables|Default|SetExplosion%20Sound _returnvalue)
  (bind _asbp_game_mode_pve (Utilities|Casting|CastToBP_GameMode_PVE (Game|GetGameMode)))
  (Math|Integer|DecrementInt (Variables|/Game/Blueprint/PVEMode/BP_GameMode_PVE.BP_GameMode_PVE_C|GetSpawned%20Bomb%20Count _asbp_game_mode_pve)
    (:%20%20
      (Components|DestroyComponent (Variables|Default|GetBomb_Mesh))
      (Utilities|Time|SetTimerbyEvent (EventDispatchers|CreateEvent :!event Custom|Destroy) 2.0))))