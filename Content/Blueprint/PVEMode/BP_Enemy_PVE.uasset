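; PVE enemy character that is randomly either a traitor or a decoy, with a random player color material, for the player to pick out and hit.
; It wanders to random reachable points after random delays; ActivateMovementAndOverlaps starts a looping timer and enables overlap events.
; A hit traitor adds score, lowers the game mode's traitor count, triggers a win check and dies.
; A hit decoy costs score, disables the player's attack and explodes, damaging them.
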(event Custom|AI%20Start%20Movement
  (Utilities|FlowControl|Delay (Math|Random|RandomFloatinRange (Variables|Default|GetMove%20Frequency%20Min) (Variables|Default|GetMove%20Frequency%20Max)))
  (if (not (or (Variables|Default|GetisMoving) (Variables|Default|GetisDead)))
    (Variables|Default|SetisMoving true)
    (AI|AIMoveTo self (.RandomLocation (AI|Navigation|GetRandomReachablePointinRadius (Transformation|GetActorLocation) (Math|Random|RandomFloatinRange (Variables|Default|GetMovement%20Range%20Min) (Variables|Default|GetMovement%20Range%20Max)) 0 0)) 0 5.0 false
      (:OnSuccess
        _)
      (:OnFail
        _))
    (Variables|Default|SetisMoving false)))

(event Game|Damage|EventAnyDamage
  (params (Damage :type Float%20%28single-precision%29) (DamageType :type Damage%20Type%20Object%20Reference) (InstigatedBy :type Controller%20Object%20Reference) (DamageCauser :type Actor%20Object%20Reference))
  (bind _returnvalue (Transformation|GetActorLocation))
  (if (not (Variables|Default|GetisDead))
    (bind _asbp_player_pve (Utilities|Casting|CastToBP_Player_PVE DamageCauser))
    (if (not (Variables|/Game/Blueprint/PVEMode/BP_Player_PVE.BP_Player_PVE_C|GetisFlickering _asbp_player_pve))
      (Audio|PlaySoundatLocation "/Game/Assets/Sounds/Punch/Player_Punch_SpounCue.Player_Punch_SpounCue" (Transformation|GetActorLocation) "0, 0, 0" 1.0 1.0 0.0 0 0 0)
      (if (Variables|Default|GetisTraitor)
        (Default|IncreaseScore _asbp_player_pve)
        (CallFunction|DecreaseTraitorCount)
        (Default|CheckWinCondition (Variables|Default|GetAs%20BP%20Game%20Mode%20PVE))
        (Components|Animation|PlayAnimation (Variables|Character|GetMesh) "/Game/PartyMonsterRumblePA/Animation/Die01_Anim.Die01_Anim" false)
        (Variables|Default|SetisDead true)
        (Collision|SetActorEnableCollision self false)
        (Class|NavMovementComponent|StopActiveMovement (Variables|Character|GetCharacterMovement))
        (Utilities|FlowControl|Delay 1.0)
        (Default|UpdateScoreUI _asbp_player_pve)
        (Effects|SpawnEmitteratLocation "/Game/Assets/Particles/Poof/P_Poof_GhostSpawn.P_Poof_GhostSpawn" _returnvalue "0, 0, 0" "6.000000,6.000000,6.000000")
        (Audio|PlaySoundatLocation "/Game/Assets/Sounds/EnvironmentSFX/Correct_Sound.Correct_Sound" _returnvalue "0, 0, 0" 1.0 1.0 0.0 0 0 0)
        (Actor|DestroyActor)
        (else
          (Default|DecreaseScore _asbp_player_pve)
          (Variables|/Game/Blueprint/PVEMode/BP_Player_PVE.BP_Player_PVE_C|SetCanAttack _asbp_player_pve false)
          (Utilities|FlowControl|Delay 0.2)
          (Audio|PlaySoundatLocation "/Game/Assets/Sounds/EnvironmentSFX/Incorrect_Sound_Cue.Incorrect_Sound_Cue" (Transformation|GetActorLocation) "0, 0, 0" 1.0 1.0 0.0 0 0 0)
          (Utilities|FlowControl|Delay 0.3)
          (CallFunction|PlayExplosionFX _asbp_player_pve)
          (Default|UpdateScoreUI _asbp_player_pve))))))

(event EventBeginPlay
  (CallFunction|CacheGameMode)
  (CallFunction|RandomizeIdentity)
  (CallFunction|SetPlayerPawnColor)
  (Utilities|FlowControl|Delay 0.2)
  (CallFunction|CacheAnimBP))

(fn ConstructionScript)

(fn SetPlayerPawnColor
  (bind _mesh (Variables|Character|GetMesh))
  (switch int (Math|Random|RandomIntegerinRange 0 7)
    (:0
      (Rendering|Material|SetMaterial _mesh 0 "/Game/PartyMonsterRumblePA/Material/MaterialInstances/PlayerMaterial/PlayerMaterial_Inst.PlayerMaterial_Inst"))
    (:1
      (Rendering|Material|SetMaterial _mesh 0 "/Game/PartyMonsterRumblePA/Material/MaterialInstances/PlayerMaterial/PlayerMaterial_Inst_2.PlayerMaterial_Inst_2"))
    (:2
      (Rendering|Material|SetMaterial _mesh 0 "/Game/PartyMonsterRumblePA/Material/MaterialInstances/PlayerMaterial/PlayerMaterial_Inst_3.PlayerMaterial_Inst_3"))
    (:3
      (Rendering|Material|SetMaterial _mesh 0 "/Game/PartyMonsterRumblePA/Material/MaterialInstances/PlayerMaterial/PlayerMaterial_Inst_4.PlayerMaterial_Inst_4"))
    (:4
      (Rendering|Material|SetMaterial _mesh 0 "/Game/PartyMonsterRumblePA/Material/MaterialInstances/PlayerMaterial/PlayerMaterial_Inst_5.PlayerMaterial_Inst_5"))
    (:5
      (Rendering|Material|SetMaterial _mesh 0 "/Game/PartyMonsterRumblePA/Material/MaterialInstances/PlayerMaterial/PlayerMaterial_Inst_6.PlayerMaterial_Inst_6"))
    (:6
      (Rendering|Material|SetMaterial _mesh 0 "/Game/PartyMonsterRumblePA/Material/MaterialInstances/PlayerMaterial/PlayerMaterial_Inst_7.PlayerMaterial_Inst_7"))
    (:7
      (Rendering|Material|SetMaterial _mesh 0 "/Game/PartyMonsterRumblePA/Material/MaterialInstances/PlayerMaterial/PlayerMaterial_Inst_8.PlayerMaterial_Inst_8")))
  (return))

(fn ConstrutCharacterModel)

(fn CacheAnimBP
  (bind _asanim_bp_player_pve (Utilities|Casting|CastToAnimBP_Player_PVE (Components|SkeletalMesh|GetAnimInstance (Variables|Character|GetMesh))))
  (Variables|Default|SetAs%20Anim%20BP%20Player%20PVE _asanim_bp_player_pve))

(fn CacheGameMode
  (bind _asbp_game_mode_pve (Utilities|Casting|CastToBP_GameMode_PVE (Game|GetGameMode)))
  (Variables|Default|SetAs%20BP%20Game%20Mode%20PVE _asbp_game_mode_pve))

(fn RandomizeIdentity
  (bind _output_get (Variables|Default|SetisTraitor (Math|Random|RandomBoolwithWeight (Variables|Default|GetTraitor%20Spawn%20Rate))))
  (if _output_get
    (Math|Integer|IncrementInt (Variables|/Game/Blueprint/PVEMode/BP_GameMode_PVE.BP_GameMode_PVE_C|GetTraitor%20Count (Variables|Default|GetAs%20BP%20Game%20Mode%20PVE))
      (:%20%20
        _)))
  (return))

(fn PlayExplosionFX
  (params (DamagedActor :type Actor%20Object%20Reference))
  (bind _returnvalue (Transformation|GetActorLocation))
  (Game|Damage|ApplyDamage DamagedActor 1.0 0 0)
  (Effects|SpawnEmitteratLocation "/Game/StylizedVFX_Fire/Effects/P_FireExplosion_Medium.P_FireExplosion_Medium" _returnvalue "0, 0, 0" "4.000000,4.000000,4.000000")
  (Audio|PlaySoundatLocation "/Game/Assets/Sounds/Bomb_Explosion.Bomb_Explosion" _returnvalue "0, 0, 0" 1.0 1.0 0.0 0 0 0))

(fn DecreaseTraitorCount
  (bind _result (Math|Integer|DecrementInt (Variables|/Game/Blueprint/PVEMode/BP_GameMode_PVE.BP_GameMode_PVE_C|GetTraitor%20Count (Variables|Default|GetAs%20BP%20Game%20Mode%20PVE)))
    (:%20%20
      (return (Utilities|String|ToString(Integer) _result)))))

(fn ActivateMovementandOverlaps
  (Utilities|Time|SetTimerbyEvent (EventDispatchers|CreateEvent :!event Custom|AI%20Start%20Movement) (Variables|Default|GetMovement%20Frequency) true)
  (Variables|/Script/Engine.PrimitiveComponent|SetbGenerateOverlapEvents (Variables|Default|GetDetectorCollider) true)
  (Variables|/Script/Engine.PrimitiveComponent|SetbGenerateOverlapEvents (Variables|Collision|GetCapsuleComponent) true))