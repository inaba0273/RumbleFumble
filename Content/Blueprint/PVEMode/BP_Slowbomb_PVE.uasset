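; PVE ice bomb that lights its fuse after a short random delay, then explodes and freezes players in range.
; The fuse phase runs looping scale-up and one-shot explode timers, with a timeline flashing the dynamic material's color.
; The explosion calls PlayerFreeze on overlapping BP_Player_PVE actors, plays effects, decrements the game mode's bomb count, removes the mesh and sets a follow-up timer.
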(event Custom|Start%20Fuze
  (Components|Activation|Activate (Variables|Default|GetFuze) false)
  (bind _returnvalue (Audio|SpawnSoundatLocation "/Game/Assets/Sounds/Bomb_Fuze.Bomb_Fuze" (Transformation|GetWorldLocation (Variables|Default|GetBomb_Mesh)) "0, 0, 0" 0.2 1.0 0.0 0 0))
  (Variables|Default|SetFuze%20Sound _returnvalue)
  (Utilities|Time|SetTimerbyFunctionName 0 "Bomb Scale Up" 0.1 true)
  (Utilities|Time|SetTimerbyFunctionName 0 "Bomb Explode" 3.5)
  (CallFunction|BombFlashWhite))

(event Custom|Bomb%20Flash%20White
  (bind _bomb_color_white (Timeline|Timeline_0 Play)
    (:Update
      (Rendering|Material|SetVectorParameterValue (Variables|Default|GetDynamic%20Material) "Color" (Math|Conversions|ToLinearColor(Vector) _bomb_color_white) :!class /Script/Engine.MaterialInstanceDynamic))))

(event Custom|Destory
  (Utilities|FlowControl|Delay 2.0)
  (Actor|DestroyActor))

(event EventBeginPlay
  (|CallParentFunction)
  (Utilities|FlowControl|Delay (Math|Random|RandomFloatinRange 2.0 3.0))
  (CallFunction|StartFuze))

(event Collision|EventActorBeginOverlap
  (params (OtherActor :type Actor%20Object%20Reference))
  (|CallParentFunction OtherActor) ; This node is disabled and will not be called.\nDrag off pins to build functionality.
)

(event EventTick
  (params (DeltaSeconds :type Float%20%28single-precision%29))
  (|CallParentFunction DeltaSeconds) ; This node is disabled and will not be called.\nDrag off pins to build functionality.
)

(fn ConstructionScript
  (|CallParentFunction)
  (bind _returnvalue (Rendering|Material|CreateDynamicMaterialInstance "/Game/Assets/Inflatable_Parkour/Material/M_IceBomb.M_IceBomb" "None" "None" :!class /Script/Engine.KismetMaterialLibrary))
  (bind _output_get (Variables|Default|SetDynamic%20Material _returnvalue))
  (Rendering|Material|SetMaterial (Variables|Default|GetBomb_Mesh) 0 _output_get))

(fn BombScaleUp
  (Transformation|SetWorldScale3D (Variables|Default|GetBomb_Mesh) (+ (Variables|Default|GetNew%20Scale) "0.005000,0.005000,0.005000"))
  (Variables|Default|SetNew%20Scale (+ (Variables|Default|GetNew%20Scale) "0.005000,0.005000,0.005000")))

(fn BombExplode
  (bind _fuze_sound (Variables|Default|GetFuze%20Sound))
  (Components|Activation|Deactivate (Variables|Default|GetFuze))
  (if (Utilities|IsValid _fuze_sound)
    (Audio|Components|Audio|Stop _fuze_sound))
  (Components|Activation|Activate (Variables|Default|GetExplosion) false)
  (for _array_element (Collision|GetOverlappingActors (Variables|Default|GetBomb%20Range) "/Game/Blueprint/PVEMode/BP_Player_PVE.BP_Player_PVE_C" :!class /Script/Engine.PrimitiveComponent)
    (bind _asbp_player_pve (Utilities|Casting|CastToBP_Player_PVE _array_element))
    (Default|PlayerFreeze _asbp_player_pve)
    (Development|PrintString "PLAYER SLOW DOWN" true true "(R=0.000000,G=0.660000,B=1.000000,A=1.000000)" 8.0))
  (Class|KismetSystemLibrary|PauseTimer 0 "Bomb Scale Up")
  (bind _returnvalue (Audio|SpawnSoundatLocation "/Game/Assets/Sounds/IceBomb_Cue.IceBomb_Cue" (Transformation|GetWorldLocation (Variables|Default|GetExplosion)) "0, 0, 0" 1.0 1.0 0.0 0 0))
  (Variables|Default|SetExplosion%20Sound _returnvalue)
  (bind _asbp_game_mode_pve (Utilities|Casting|CastToBP_GameMode_PVE (Game|GetGameMode)))
  (Math|Integer|DecrementInt (Variables|/Game/Blueprint/PVEMode/BP_GameMode_PVE.BP_GameMode_PVE_C|GetSpawned%20Bomb%20Count _asbp_game_mode_pve)
    (:%20%20
      (Components|DestroyComponent (Variables|Default|GetBomb_Mesh))
      (Utilities|Time|SetTimerbyEvent (EventDispatchers|CreateEvent :!event Custom|Destory) 2.0))))