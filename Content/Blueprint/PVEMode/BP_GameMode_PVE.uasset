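; PVE game mode for local multiplayer that sets up players, enemies, a shared fixed camera and the score UI.
; BeginPlay spawns and possesses one character per GameInstance player count, randomizes player and enemy meshes, then activates enemies and shows the UI after a delay.
; Timers drop bombs at tagged spawn points under an item cap.
; StartGameSequence, uncalled here, gathers those points and sets item timers; CheckWinCondition is a stub.
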(event Custom|Spawn%20Bomb%20Continuely
  (Utilities|FlowControl|Delay (Math|Random|RandomFloatinRange 0.0 3.0))
  (CallFunction|SpawnBomb))

(event Custom|Spawn%20Speed%20Item%20Continuely
  (Utilities|FlowControl|Delay (Math|Random|RandomFloatinRange 0.0 2.0))
  (CallFunction|SpawnSpeedItem))

(event EventBeginPlay
  ;[1 1 1] Use to enable control during development, need to refine later
  (Input|SetInputModeGameOnly (Game|GetPlayerController 0))
  (Variables|Default|SetcanBePaused true)
  (CallFunction|UpdatePlayerCount)
  (Utilities|FlowControl|Sequence
    (:then_0
      (CallFunction|SpawnPlayers)
      (CallFunction|RandomizeCharacterParts)
      (CallFunction|FindCameraActor)
      (CallFunction|InitializePlayerScoreUI))
    (:then_1
      (Game|Player|SetViewTargetwithBlend (Game|GetPlayerController 0) (Variables|Default|GetMainCamera) 0.0 "VTBlend_Linear" 0.0 false)
      (Utilities|Time|SetTimerbyEvent (delegate Custom|Spawn%20Bomb%20Continuely) 5.0 true)
      (Utilities|FlowControl|Delay 5.0)
      ;[1 1 1] Temp Solution, refine later
      (CallFunction|StartGame))))

(fn ConstructionScript)

(fn SpawnPlayers
  (bind _max_player_count (Variables|Default|GetMax%20Player%20Count))
  (bind _returnvalue (- _max_player_count 1))
  ;[1 1 1] Create Player 1, 2, 3
  (for _index (range 1 _returnvalue)
    (Class|GameplayStatics|CreatePlayer _index))
  ;[1 1 1] Spawn and Posses Player Character 0, 1, 2, 3
  (for _index_2 (range 0 _returnvalue)
    (bind _returnvalue_2 (Game|SpawnActorfromClass "/Game/Blueprint/PVEMode/BP_Player_PVE.BP_Player_PVE_C" (Math|Transform|MakeTransform "0, 0,2000.000000") "Undefined" 0 _index_2 1.0 0))
    (Pawn|Possess (Game|GetPlayerController _index_2) _returnvalue_2)
    (Utilities|Array|AddUnique (Variables|Default|GetPlayer%20Array) _returnvalue_2)))

(fn FindCameraActor
  (bind _returnvalue (Actor|GetActorOfClass "/Game/Blueprint/BP_FixedCamera.BP_FixedCamera_C"))
  (Variables|Default|SetMainCamera _returnvalue))

(fn UpdatePlayerCount
  ;[1 1 1] Get Max Player Count from GameInstance
  (bind _asbp_game_instance (Utilities|Casting|CastToBP_GameInstance (Game|GetGameInstance)))
  (Variables|Default|SetMax%20Player%20Count (Variables|/Game/UI/BP_GameInstance.BP_GameInstance_C|GetPlayerCount _asbp_game_instance)))

(fn GetRandomSpawnPoint
  (CallFunction|GetBombSpawnPoints)
  (CallFunction|GetSpeedSpawnPoints))

(fn StartGameSequence
  (Input|SetInputModeGameOnly (Game|GetPlayerController 0))
  (CallFunction|GetRandomSpawnPoint)
  (Utilities|Time|SetTimerbyEvent (EventDispatchers|CreateEvent :!event Custom|Spawn%20Bomb%20Continuely) (Variables|Default|GetBomb%20Item%20Spawn%20Frequency) true)
  (Utilities|Time|SetTimerbyEvent (EventDispatchers|CreateEvent :!event Custom|Spawn%20Speed%20Item%20Continuely) (Variables|Default|GetSpeed%20Item%20Spawn%20Frequency) true)
  (Utilities|Time|SetTimerbyFunctionName 0 "Increase max item count" (Variables|Default|GetIncrease%20Item%20Spawn%20Count%20Frequency) true)
  (Default|CallTutorialEnded)
  (CallFunction|SpawnBomb))

(fn IncreaseMaxItemCount
  (bind _maxspawneditemcount (Variables|Default|GetMaxSpawnedItemCount))
  (if (<= _maxspawneditemcount 10)
    (bind _result (Math|Integer|IncrementInt _maxspawneditemcount)
      (:%20%20
        (Development|PrintString (Utilities|String|Append "Max Spawn Item Count increaded to " (Utilities|String|ToString(Integer) _result)) true true "(R=0.000000,G=0.660000,B=1.000000,A=1.000000)" 3e+01)))))

(fn RandomizeCharacterParts
  ;[1 1 1] Save all part as array
  (Variables|Default|SetOne%20Mesh%20Array (Utilities|Array|MakeArray "/Game/PartyMonsterRumblePA/Mesh/OneMeshCharacter/OneMesh01_SK.OneMesh01_SK" "/Game/PartyMonsterRumblePA/Mesh/OneMeshCharacter/OneMesh02_SK.OneMesh02_SK" "/Game/PartyMonsterRumblePA/Mesh/OneMeshCharacter/OneMesh03_SK.OneMesh03_SK" "/Game/PartyMonsterRumblePA/Mesh/OneMeshCharacter/OneMesh04_SK.OneMesh04_SK" "/Game/PartyMonsterRumblePA/Mesh/OneMeshCharacter/OneMesh05_SK.OneMesh05_SK" "/Game/PartyMonsterRumblePA/Mesh/OneMeshCharacter/OneMesh06_SK.OneMesh06_SK" "/Game/PartyMonsterRumblePA/Mesh/OneMeshCharacter/OneMesh07_SK.OneMesh07_SK" "/Game/PartyMonsterRumblePA/Mesh/OneMeshCharacter/OneMesh08_SK.OneMesh08_SK" "/Game/PartyMonsterRumblePA/Mesh/OneMeshCharacter/OneMesh09_SK.OneMesh09_SK" "/Game/PartyMonsterRumblePA/Mesh/OneMeshCharacter/OneMesh10_SK.OneMesh10_SK" "/Game/PartyMonsterRumblePA/Mesh/OneMeshCharacter/OneMesh11_SK.OneMesh11_SK"))
  (Variables|Default|SetBody%20Mesh%20Array (Utilities|Array|MakeArray "/Game/PartyMonsterRumblePA/Mesh/ModularPart/Body01_SK.Body01_SK" "/Game/PartyMonsterRumblePA/Mesh/ModularPart/Body01_SK.Body01_SK" "/Game/PartyMonsterRumblePA/Mesh/ModularPart/Body03_SK.Body03_SK" "/Game/PartyMonsterRumblePA/Mesh/ModularPart/Body04_SK.Body04_SK" "/Game/PartyMonsterRumblePA/Mesh/ModularPart/Body05_SK.Body05_SK" "/Game/PartyMonsterRumblePA/Mesh/ModularPart/Body06_SK.Body06_SK"))
  (Variables|Default|SetBodyparts%20Mesh%20Array (Utilities|Array|MakeArray "/Game/PartyMonsterRumblePA/Mesh/ModularPart/Bodypart01_SK.Bodypart01_SK" "/Game/PartyMonsterRumblePA/Mesh/ModularPart/Bodypart02_SK.Bodypart02_SK" "/Game/PartyMonsterRumblePA/Mesh/ModularPart/Bodypart03_SK.Bodypart03_SK" "/Game/PartyMonsterRumblePA/Mesh/ModularPart/Bodypart04_SK.Bodypart04_SK" "/Game/PartyMonsterRumblePA/Mesh/ModularPart/Bodypart05_SK.Bodypart05_SK" "/Game/PartyMonsterRumblePA/Mesh/ModularPart/Bodypart06_SK.Bodypart06_SK" "/Game/PartyMonsterRumblePA/Mesh/ModularPart/Bodypart07_SK.Bodypart07_SK" "/Game/PartyMonsterRumblePA/Mesh/ModularPart/Bodypart08_SK.Bodypart08_SK" "/Game/PartyMonsterRumblePA/Mesh/ModularPart/Bodypart09_SK.Bodypart09_SK" "/Game/PartyMonsterRumblePA/Mesh/ModularPart/Bodypart10_SK.Bodypart10_SK" 0))
  (Variables|Default|SetEye%20Mesh%20Array (Utilities|Array|MakeArray "/Game/PartyMonsterRumblePA/Mesh/ModularPart/Eye01_SK.Eye01_SK" "/Game/PartyMonsterRumblePA/Mesh/ModularPart/Eye02_SK.Eye02_SK" "/Game/PartyMonsterRumblePA/Mesh/ModularPart/Eye03_SK.Eye03_SK" "/Game/PartyMonsterRumblePA/Mesh/ModularPart/Eye04_SK.Eye04_SK" "/Game/PartyMonsterRumblePA/Mesh/ModularPart/Eye05_SK.Eye05_SK" "/Game/PartyMonsterRumblePA/Mesh/ModularPart/Eye06_SK.Eye06_SK" "/Game/PartyMonsterRumblePA/Mesh/ModularPart/Eye07_SK.Eye07_SK" "/Game/PartyMonsterRumblePA/Mesh/ModularPart/Eye08_SK.Eye08_SK" "/Game/PartyMonsterRumblePA/Mesh/ModularPart/Eye09_SK.Eye09_SK" "/Game/PartyMonsterRumblePA/Mesh/ModularPart/Eye10_SK.Eye10_SK" "/Game/PartyMonsterRumblePA/Mesh/ModularPart/Eye11_SK.Eye11_SK" "/Game/PartyMonsterRumblePA/Mesh/ModularPart/Eye12_SK.Eye12_SK" "/Game/PartyMonsterRumblePA/Mesh/ModularPart/Eye13_SK.Eye13_SK" "/Game/PartyMonsterRumblePA/Mesh/ModularPart/Eye14_SK.Eye14_SK" "/Game/PartyMonsterRumblePA/Mesh/ModularPart/Eye15_SK.Eye15_SK"))
  (Variables|Default|SetMouth%20Mesh%20Array (Utilities|Array|MakeArray "/Game/PartyMonsterRumblePA/Mesh/ModularPart/Mouth01_SK.Mouth01_SK" "/Game/PartyMonsterRumblePA/Mesh/ModularPart/Mouth02_SK.Mouth02_SK" "/Game/PartyMonsterRumblePA/Mesh/ModularPart/Mouth03_SK.Mouth03_SK" "/Game/PartyMonsterRumblePA/Mesh/ModularPart/Mouth04_SK.Mouth04_SK" "/Game/PartyMonsterRumblePA/Mesh/ModularPart/Mouth05_SK.Mouth05_SK" "/Game/PartyMonsterRumblePA/Mesh/ModularPart/Mouth06_SK.Mouth06_SK" "/Game/PartyMonsterRumblePA/Mesh/ModularPart/Mouth07_SK.Mouth07_SK" "/Game/PartyMonsterRumblePA/Mesh/ModularPart/Mouth08_SK.Mouth08_SK" "/Game/PartyMonsterRumblePA/Mesh/ModularPart/Mouth09_SK.Mouth09_SK" "/Game/PartyMonsterRumblePA/Mesh/ModularPart/Mouth15_SK.Mouth15_SK" 0))
  (Variables|Default|SetTail%20Mesh%20Array (Utilities|Array|MakeArray "/Game/PartyMonsterRumblePA/Mesh/ModularPart/Tail01_SK.Tail01_SK" "/Game/PartyMonsterRumblePA/Mesh/ModularPart/Tail02_SK.Tail02_SK" "/Game/PartyMonsterRumblePA/Mesh/ModularPart/Tail03_SK.Tail03_SK" "/Game/PartyMonsterRumblePA/Mesh/ModularPart/Tail04_SK.Tail04_SK" "/Game/PartyMonsterRumblePA/Mesh/ModularPart/Tail05_SK.Tail05_SK" "/Game/PartyMonsterRumblePA/Mesh/ModularPart/Tail06_SK.Tail06_SK" "/Game/PartyMonsterRumblePA/Mesh/ModularPart/Tail07_SK.Tail07_SK" "/Game/PartyMonsterRumblePA/Mesh/ModularPart/Tail08_SK.Tail08_SK" 0))
  (Variables|Default|SetHeadpart%20Mesh%20Array (Utilities|Array|MakeArray "/Game/PartyMonsterRumblePA/Mesh/ModularPart/Grass15_SK.Grass15_SK" "/Game/PartyMonsterRumblePA/Mesh/ModularPart/Hair06_SK.Hair06_SK" "/Game/PartyMonsterRumblePA/Mesh/ModularPart/Hair07_SK.Hair07_SK" "/Game/PartyMonsterRumblePA/Mesh/ModularPart/Hair08_SK.Hair08_SK" "/Game/PartyMonsterRumblePA/Mesh/ModularPart/Hair09_SK.Hair09_SK" "/Game/PartyMonsterRumblePA/Mesh/ModularPart/Horn10_SK.Horn10_SK" "/Game/PartyMonsterRumblePA/Mesh/ModularPart/Horn11_SK.Horn11_SK" "/Game/PartyMonsterRumblePA/Mesh/ModularPart/Horn12_SK.Horn12_SK" "/Game/PartyMonsterRumblePA/Mesh/ModularPart/Horn13_SK.Horn13_SK" "/Game/PartyMonsterRumblePA/Mesh/ModularPart/Hat16_SK.Hat16_SK" "/Game/PartyMonsterRumblePA/Mesh/ModularPart/Hat17_SK.Hat17_SK" "/Game/PartyMonsterRumblePA/Mesh/ModularPart/Hat18_SK.Hat18_SK" "/Game/PartyMonsterRumblePA/Mesh/ModularPart/Hat19_SK.Hat19_SK" "/Game/PartyMonsterRumblePA/Mesh/ModularPart/Hat20_SK.Hat20_SK" "/Game/PartyMonsterRumblePA/Mesh/ModularPart/Hat21_SK.Hat21_SK" "/Game/PartyMonsterRumblePA/Mesh/ModularPart/Ear01_SK.Ear01_SK" "/Game/PartyMonsterRumblePA/Mesh/ModularPart/Ear02_SK.Ear02_SK" "/Game/PartyMonsterRumblePA/Mesh/ModularPart/Ear03_SK.Ear03_SK" "/Game/PartyMonsterRumblePA/Mesh/ModularPart/Ear04_SK.Ear04_SK" "/Game/PartyMonsterRumblePA/Mesh/ModularPart/Ear05_SK.Ear05_SK" 0))
  ;[1 1 1] Randomize Player Mesh
  (for _array_element (Variables|Default|GetPlayer%20Array)
    (Class|SkinnedMeshComponent|SetSkeletalMesh (Variables|/Script/Engine.Character|GetMesh _array_element) (.OutItem (Utilities|Array|Random (Variables|Default|GetBody%20Mesh%20Array))) true)
    (Class|SkinnedMeshComponent|SetSkeletalMesh (Variables|/Game/Blueprint/PVEMode/BP_Player_PVE.BP_Player_PVE_C|GetBodyparts _array_element) (.OutItem (Utilities|Array|Random (Variables|Default|GetBodyparts%20Mesh%20Array))) true)
    (Class|SkinnedMeshComponent|SetSkeletalMesh (Variables|/Game/Blueprint/PVEMode/BP_Player_PVE.BP_Player_PVE_C|GetEyes _array_element) (.OutItem (Utilities|Array|Random (Variables|Default|GetEye%20Mesh%20Array))) true)
    (Class|SkinnedMeshComponent|SetSkeletalMesh (Variables|/Game/Blueprint/PVEMode/BP_Player_PVE.BP_Player_PVE_C|GetMouths _array_element) (.OutItem (Utilities|Array|Random (Variables|Default|GetMouth%20Mesh%20Array))) true)
    (Class|SkinnedMeshComponent|SetSkeletalMesh (Variables|/Game/Blueprint/PVEMode/BP_Player_PVE.BP_Player_PVE_C|GetHeadparts _array_element) (.OutItem (Utilities|Array|Random (Variables|Default|GetHeadpart%20Mesh%20Array))) true)
    (Class|SkinnedMeshComponent|SetSkeletalMesh (Variables|/Game/Blueprint/PVEMode/BP_Player_PVE.BP_Player_PVE_C|GetTails _array_element) (.OutItem (Utilities|Array|Random (Variables|Default|GetTail%20Mesh%20Array))) true))
  ;[1 1 1] Randomize Enemy Mesh
  (bind _outactors (Actor|GetAllActorsOfClass "/Game/Blueprint/PVEMode/BP_Enemy_PVE.BP_Enemy_PVE_C"))
  (bind _output_get (Variables|Default|SetEnemy%20Array _outactors))
  (for _array_element_2 _output_get
    (Class|SkinnedMeshComponent|SetSkeletalMesh (Variables|/Script/Engine.Character|GetMesh _array_element_2) (.OutItem (Utilities|Array|Random (Variables|Default|GetOne%20Mesh%20Array))) true))
  (return))

(fn PlayLevelMusic
  (bind _returnvalue (Audio|CreateSound2D "/Game/Assets/Sounds/BGM/in_game_bgm_Cue.in_game_bgm_Cue" 1.0 1.0 0.0 0))
  (bind _output_get (Variables|Default|SetIn%20Game%20Music _returnvalue))
  (Audio|Components|Audio|Play _output_get 0.0))

(fn SpawnBomb
  (bind _bomb_item_spawn_points (Variables|Default|GetBomb%20Item%20Spawn%20Points))
  (bind _outitem (Utilities|Array|Random _bomb_item_spawn_points))
  (bind _returnvalue (Transformation|GetActorTransform _outitem))
  (if (and (< (Variables|Default|GetSpawnedItemCount) (Variables|Default|GetMaxSpawnedItemCount)) (Variables|Default|GetcanBePaused))
    (Utilities|IsValid _outitem
      (:Is%20Valid
        (Game|SpawnActorfromClass "/Game/Blueprint/BP_KillBomb.BP_KillBomb_C" (Math|Transform|MakeTransform (.location _returnvalue) (Math|Random|RandomRotator false) "8.000000,8.000000,8.000000") "Undefined" 0 0)
        (Math|Integer|IncrementInt (Variables|Default|GetSpawnedItemCount)
          (:%20%20
            (Development|PrintString "Bomb Spawned")
            (Audio|PlaySoundatLocation "/Game/Assets/Sounds/Item_Drop.Item_Drop" (.location _returnvalue) "0, 0, 0" 0.5 1.0 0.0 0 0 0)))))))

(fn SpawnSpeedItem
  (bind _speed_item_spawn_points (Variables|Default|GetSpeed%20Item%20Spawn%20Points))
  (bind _outitem (Utilities|Array|Random _speed_item_spawn_points))
  (bind _returnvalue (Transformation|GetActorTransform _outitem))
  (if (and (< (Variables|Default|GetSpawnedItemCount) (Variables|Default|GetMaxSpawnedItemCount)) (Variables|Default|GetcanBePaused))
    (Utilities|IsValid _outitem
      (:Is%20Valid
        (Game|SpawnActorfromClass "/Game/Blueprint/BP_SpeedItem.BP_SpeedItem_C" (Math|Transform|MakeTransform (.location _returnvalue) "0, 0, 0" "2.000000,2.000000,2.000000") "Undefined" 0 0)
        (Math|Integer|IncrementInt (Variables|Default|GetSpawnedItemCount)
          (:%20%20
            (Development|PrintString "Glove Spawned")
            (Audio|PlaySoundatLocation "/Game/Assets/Sounds/Item_Drop.Item_Drop" (.location _returnvalue) "0, 0, 0" 0.5 1.0 0.0 0 0 0)))))))

(fn GetBombSpawnPoints
  (bind _outactors (Actor|GetAllActorsOfClasswithTag "/Game/Blueprint/BP_ItemSpawnPoint.BP_ItemSpawnPoint_C" "Bomb"))
  (Variables|Default|SetBomb%20Item%20Spawn%20Points _outactors))

(fn GetSpeedSpawnPoints
  (bind _outactors (Actor|GetAllActorsOfClasswithTag "/Game/Blueprint/BP_ItemSpawnPoint.BP_ItemSpawnPoint_C" "Speed"))
  (Variables|Default|SetSpeed%20Item%20Spawn%20Points _outactors))

(fn StartGame
  (bind _outactors (Actor|GetAllActorsOfClass "/Game/Blueprint/PVEMode/BP_Enemy_PVE.BP_Enemy_PVE_C"))
  (for _array_element _outactors
    (Default|ActivateMovementandOverlaps _array_element)
    (Widget|SetVisibility (Variables|Default|GetAs%20Player%20Score%20UI) "Visible")))

(fn CheckWinCondition
  (if (== (Variables|Default|GetTraitor%20Count) 0)
    _
    (else
      _))
  (return))

(fn InitializePlayerScoreUI
  (bind _returnvalue (UserInterface|CreateWidget "/Game/Blueprint/PVEMode/PlayerScoreUI.PlayerScoreUI_C"))
  (UserInterface|Viewport|AddtoViewport _returnvalue 0)
  (bind _output_get (Variables|Default|SetAs%20Player%20Score%20UI _returnvalue))
  (Widget|SetVisibility _output_get "Hidden"))