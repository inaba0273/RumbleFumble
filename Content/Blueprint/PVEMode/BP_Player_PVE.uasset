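; Player character for PVE mode, using PlayerInt to select spawn point, color, name, controller and score slot.
; Handles movement, two-step montage attacks, and sphere-traced item pickup with socket attachment and physics throws, coordinated with the AnimBP.
; Hits, damage and sped-up collisions cause dizziness, while freeze and speed items scale MoveSpeed temporarily.
; A detector collider counts overlapping traitor enemies to loop controller vibration, and helpers adjust score with a first-to-score bonus.
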(event OnComponentBeginOverlap(HeadCollision)
  (params (OverlappedComponent :type Primitive%20Component%20Object%20Reference) (OtherActor :type Actor%20Object%20Reference) (OtherComp :type Primitive%20Component%20Object%20Reference) (OtherBodyIndex :type Integer) (bFromSweep :type Boolean) (SweepResult :type Hit%20Result%20Structure%20%28by%20ref%29))
  (bind _asbp_pickup_item (Utilities|Casting|CastToBP_PickupItem OtherActor))
  (if (not (Variables|/Game/Blueprint/BP_PickupItem.BP_PickupItem_C|GetisPickedUp _asbp_pickup_item))
    (if (not (or (Variables|Default|GetisDizzy) (Variables|Default|GetIn%20Animation)))
      (CallFunction|PlayHitFX (Transformation|GetWorldLocation (Variables|Default|GetHit%20Particle)))
      (CallFunction|PlayerDizzy (Variables|Character|GetMesh)))))

(event OnComponentBeginOverlap(ItemPickupRange)
  (params (OverlappedComponent :type Primitive%20Component%20Object%20Reference) (OtherActor :type Actor%20Object%20Reference) (OtherComp :type Primitive%20Component%20Object%20Reference) (OtherBodyIndex :type Integer) (bFromSweep :type Boolean) (SweepResult :type Hit%20Result%20Structure%20%28by%20ref%29))
  (if (== (Utilities|GetClass OtherActor) "/Game/Blueprint/BP_SpeedItem.BP_SpeedItem_C")
    (CallFunction|SpeedUp OtherActor)
    (Utilities|FlowControl|RetriggerableDelay (Variables|Default|GetSpeed%20Item%20Duration))
    (CallFunction|SpeedDown)))

(event OnComponentBeginOverlap(DetectorCollider)
  (params (OverlappedComponent :type Primitive%20Component%20Object%20Reference) (OtherActor :type Actor%20Object%20Reference) (OtherComp :type Primitive%20Component%20Object%20Reference) (OtherBodyIndex :type Integer) (bFromSweep :type Boolean) (SweepResult :type Hit%20Result%20Structure%20%28by%20ref%29))
  (bind _asbp_enemy_pve (Utilities|Casting|CastToBP_Enemy_PVE OtherActor))
  (if (Variables|/Game/Blueprint/PVEMode/BP_Enemy_PVE.BP_Enemy_PVE_C|GetisTraitor _asbp_enemy_pve)
    (bind _result (Math|Integer|IncrementInt (Variables|Default|GetOverlap%20Traitor%20Count))
      (:%20%20
        (if (== _result 1)
          (CallFunction|ControllerStartVibration))))))

(event OnComponentEndOverlap(DetectorCollider)
  (params (OverlappedComponent :type Primitive%20Component%20Object%20Reference) (OtherActor :type Actor%20Object%20Reference) (OtherComp :type Primitive%20Component%20Object%20Reference) (OtherBodyIndex :type Integer))
  (bind _asbp_enemy_pve (Utilities|Casting|CastToBP_Enemy_PVE OtherActor))
  (if (Variables|/Game/Blueprint/PVEMode/BP_Enemy_PVE.BP_Enemy_PVE_C|GetisTraitor _asbp_enemy_pve)
    (bind _result (Math|Integer|DecrementInt (Variables|Default|GetOverlap%20Traitor%20Count))
      (:%20%20
        (if (== _result 0)
          (CallFunction|ControllerStopVibration))))))

(event Custom|Player%20Freeze
  (CallFunction|ReleaseObject "0, 0, 0")
  (Animation|Montage|PlayMontage (Variables|Character|GetMesh) "/Game/PartyMonsterRumblePA/Animation/AnimMontage_PlayerGetHit.AnimMontage_PlayerGetHit"
    (:then
      (if (Variables|Default|GetisSlowDown)
        _
        (else
          (Variables|Default|SetisSlowDown true)
          (Components|Activation|Activate (Variables|Default|GetFreeze%20Particle) false)
          (bind _output_get (Variables|Default|SetmoveSpeed (* (Variables|Default|GetmoveSpeed) (Variables|Default|GetSlowDownSpeedMultiplier))))
          (Development|PrintString (Utilities|String|Append "Player " (Utilities|String|ToString(Integer) (Variables|Default|GetplayerInt)) " current move speed: " (Utilities|String|ToString(Float) _output_get)) true true "(R=0.000000,G=0.660000,B=1.000000,A=1.000000)" 1e+01)))
      (Utilities|FlowControl|RetriggerableDelay (Variables|Default|GetSlowDownDuration))
      (Development|PrintString "***Speed Reduction Ended***")
      (Variables|Default|SetisSlowDown false)
      (bind _output_get_2 (Variables|Default|SetmoveSpeed (/ (Variables|Default|GetmoveSpeed) (Variables|Default|GetSlowDownSpeedMultiplier))))
      (Components|Activation|Deactivate (Variables|Default|GetFreeze%20Particle))
      (Development|PrintString (Utilities|String|Append "Player " (Utilities|String|ToString(Integer) (Variables|Default|GetplayerInt)) " current move speed: " (Utilities|String|ToString(Float) _output_get_2)) true true "(R=0.000000,G=0.660000,B=1.000000,A=1.000000)" 1e+01))))

(event Custom|Lifting
  ;[1 1 1] Pick Up And Throw Stuff
  (CallFunction|AttachObjecttoPlayer)
  (Variables|Default|SetIn%20Animation false))

(event Custom|Throwing
  ;[1 1 1] Pick Up And Throw Stuff
  (CallFunction|ReleaseObject (CallFunction|ApplyThrowForce)))

(event Custom|PlayerDizzy
  (params (InSkeletalMeshComponent :type Skeletal%20Mesh%20Component%20Object%20Reference))
  (CallFunction|ReleaseObject "0, 0, 0")
  (Variables|Default|SetisDizzy true)
  (Animation|Montage|PlayMontage InSkeletalMeshComponent "/Game/PartyMonsterRumblePA/Animation/AnimMontage_PlayerGetHit.AnimMontage_PlayerGetHit"
    (:OnCompleted
      (Audio|PlaySoundatLocation "/Game/Assets/Sounds/EnvironmentSFX/DizzySound_Cue.DizzySound_Cue" (Transformation|GetWorldLocation InSkeletalMeshComponent) "0, 0, 0" 1.0 1.0 0.0 0 0 0)
      (Components|Activation|Activate (Variables|Default|GetDizzy%20Particle) false)
      (Animation|Montage|PlayMontage InSkeletalMeshComponent "/Game/PartyMonsterRumblePA/Animation/Dizzy_Anim_Montage.Dizzy_Anim_Montage" 0.5
        (:OnCompleted
          (Variables|Default|SetisDizzy false)
          (Variables|Default|SetCanAttack true)
          (Components|Activation|Deactivate (Variables|Default|GetDizzy%20Particle)))))))

(event Collision|EventHit
  (params (MyComp :type Primitive%20Component%20Object%20Reference) (Other :type Actor%20Object%20Reference) (OtherComp :type Primitive%20Component%20Object%20Reference) (bSelfMoved :type Boolean) (HitLocation :type Vector :default "0, 0, 0") (HitNormal :type Vector :default "0, 0, 0") (NormalImpulse :type Vector :default "0, 0, 0") (Hit :type Hit%20Result%20Structure%20%28by%20ref%29))
  (if (and bSelfMoved (Variables|Default|GetIsSpeedUp))
    (bind _asbp_player_pve (Utilities|Casting|CastToBP_Player_PVE Other))
    (if (not (Variables|BP_Player_PVE_C|GetisDizzy _asbp_player_pve))
      (Utilities|FlowControl|DoOnce false :!label _label
        (:Completed
          (CallFunction|PlayHitFX HitLocation)
          (CallFunction|PlayerDizzy (Variables|/Script/Engine.Character|GetMesh _asbp_player_pve))
          (Utilities|FlowControl|Delay 0.2)
          (goto _label Reset))))))

(event Game|Damage|EventAnyDamage
  (params (Damage :type Float%20%28single-precision%29) (DamageType :type Damage%20Type%20Object%20Reference) (InstigatedBy :type Controller%20Object%20Reference) (DamageCauser :type Actor%20Object%20Reference))
  (CallFunction|PlayerDizzy (Variables|Character|GetMesh)))

(event EventBeginPlay
  (CallFunction|CacheGameMode)
  (CallFunction|ConstrutCharacterModel)
  (CallFunction|SpawnFunction)
  (CallFunction|SetPlayerPawnColor)
  (Utilities|FlowControl|Delay 0.2)
  (CallFunction|DisplayPlayerNameUI)
  (CallFunction|CacheAnimBP)
  (Utilities|FlowControl|Delay 5.0)
  (Development|PrintString "GAME START"))

(event Input|ActionEvents|InputActionPickUpBomb
  (params (Key :type Key%20Structure :default "None"))
  ;[1 1 1] Pick Up And Throw Stuff
  (:Pressed
    (if (not (Variables|Default|GetIn%20Animation))
      (Utilities|IsValid (Variables|Default|GetPicked%20Up%20Mesh)
        (:Is%20Valid
          (CallFunction|StartThrowing))
        (:Is%20Not%20Valid
          (CallFunction|FindItemtoPickUp)
          (CallFunction|StartPickingUp))))))

(event Input|ActionEvents|InputActionPlayerAttack
  (params (Key :type Key%20Structure :default "None"))
  (:Pressed
    (if (not (Math|Boolean|ORBoolean (CallFunction|IsAttacking) (Variables|Default|GetDead) (not (Variables|Default|GetCanAttack)) (Variables|Default|GetisDizzy) (Utilities|IsValid (Variables|Default|GetPicked%20Up%20Mesh))))
      (switch int (Variables|Default|GetAttackCounter)
        (:0
          (Variables|Default|SetAttackCounter 1)
          (Animation|Montage|PlayMontage (Variables|Character|GetMesh) "/Game/PartyMonsterRumblePA/Animation/AnimMontage_PlayerAtk_1.AnimMontage_PlayerAtk_1"
            (:OnCompleted
              (Variables|Default|SetAttackCounter 0))))
        (:1
          (Variables|Default|SetAttackCounter 0)
          (Animation|Montage|PlayMontage (Variables|Character|GetMesh) "/Game/PartyMonsterRumblePA/Animation/AnimMontage_PlayerAtk_2.AnimMontage_PlayerAtk_2"))))))

(event Input|AxisEvents|InputAxisMoveForward
  (params (AxisValue :type Float%20%28single-precision%29))
  ;[1 1 1] Basic Movements
  (if (Math|Boolean|ANDBoolean (CallFunction|IsMoveJoystickAboveDeadZone) (CallFunction|IsAlive) (not (CallFunction|IsAttacking)) (not (Variables|Default|GetisDizzy)) (not (Variables|Default|GetIn%20Animation)))
    (Pawn|Input|AddMovementInput (Math|Vector|MakeVector (Variables|Default|GetmoveSpeed) 0.0 0.0) AxisValue false)
    (CallFunction|CharacterRotation)))

(event Input|AxisEvents|InputAxisMoveRight
  (params (AxisValue :type Float%20%28single-precision%29))
  ;[1 1 1] Basic Movements
  (if (Math|Boolean|ANDBoolean (CallFunction|IsMoveJoystickAboveDeadZone) (CallFunction|IsAlive) (not (CallFunction|IsAttacking)) (not (Variables|Default|GetisDizzy)) (not (Variables|Default|GetIn%20Animation)))
    (Pawn|Input|AddMovementInput (Math|Vector|MakeVector 0.0 (Variables|Default|GetmoveSpeed) 0.0) AxisValue false)
    (CallFunction|CharacterRotation)))

(fn ConstructionScript)

(fn SpawnFunction
  ;[1 1 1] Get All Possible Spawn Point In The Level
  (bind _outactors (Actor|GetAllActorsOfClass "/Script/Engine.PlayerStart"))
  (for _array_element _outactors
    ;[1 1 1] Set Player Spawn Point
    (if (Utilities|Name|Equal(Name) (Variables|/Script/Engine.PlayerStart|GetPlayerStartTag _array_element) (Utilities|String|StringToName (Utilities|String|Append "player" (Utilities|String|ToString(Integer) (Variables|Default|GetplayerInt)))))
      (bind _output_get (Variables|Default|SetspawnLocation (Transformation|GetActorTransform _array_element)))
      (Transformation|SetActorTransform _output_get false true))))

(fn SetPlayerPawnColor
  (bind _mesh (Variables|Character|GetMesh))
  (switch int (Variables|Default|GetplayerInt)
    (:0
      (Rendering|Material|SetMaterial _mesh 0 "/Game/PartyMonsterRumblePA/Material/MaterialInstances/PlayerMaterial/PlayerMaterial_Inst.PlayerMaterial_Inst"))
    (:1
      (Rendering|Material|SetMaterial _mesh 0 "/Game/PartyMonsterRumblePA/Material/MaterialInstances/PlayerMaterial/PlayerMaterial_Inst_2.PlayerMaterial_Inst_2"))
    (:2
      (Rendering|Material|SetMaterial _mesh 0 "/Game/PartyMonsterRumblePA/Material/MaterialInstances/PlayerMaterial/PlayerMaterial_Inst_3.PlayerMaterial_Inst_3"))
    (:3
      (Rendering|Material|SetMaterial _mesh 0 "/Game/PartyMonsterRumblePA/Material/MaterialInstances/PlayerMaterial/PlayerMaterial_Inst_4.PlayerMaterial_Inst_4"))
    (:4
      (Rendering|Material|SetMaterial _mesh 0 "/Game/PartyMonsterRumblePA/Material/MaterialInstances/PlayerMaterial/PlayerMaterial_Inst_5.PlayerMaterial_Inst_5"))
    (:5
      (Rendering|Material|SetMaterial _mesh 0 "/Game/PartyMonsterRumblePA/Material/MaterialInstances/PlayerMaterial/PlayerMaterial_Inst_6.PlayerMaterial_Inst_6"))
    (:6
      (Rendering|Material|SetMaterial _mesh 0 "/Game/PartyMonsterRumblePA/Material/MaterialInstances/PlayerMaterial/PlayerMaterial_Inst_7.PlayerMaterial_Inst_7"))
    (:7
      (Rendering|Material|SetMaterial _mesh 0 "/Game/PartyMonsterRumblePA/Material/MaterialInstances/PlayerMaterial/PlayerMaterial_Inst_8.PlayerMaterial_Inst_8")))
  (return))

(fn DealDamage
  (params (DamagedActor :type Actor%20Object%20Reference))
  (Game|Damage|ApplyDamage DamagedActor (Variables|Default|GetDamage%20Amount) 0 0))

(fn DecreaseHealth
  (params (Damage :type Float%20%28single-precision%29))
  (bind _output_get (Variables|Default|SetPlayer%20Health (- (Variables|Default|GetPlayer%20Health) Damage)))
  (return _output_get))

(fn CharacterRotation
  (Pawn|SetControlRotation (Game|GetPlayerController (Variables|Default|GetplayerInt)) (Math|Rotator|MakeRotator 0.0 0.0 (Class|KismetMathLibrary|DegAtan2 (Input|AxisValues|GetAimRight) (Input|AxisValues|GetAimUp)))))

(fn IsAlive
  (return (not (Variables|Default|GetDead))))

(fn DisplayPlayerNameUI
  (bind _asplayer_name_ui (Utilities|Casting|CastToPlayerNameUI (UserInterface|GetUserWidgetObject (Variables|Default|GetPlayer%20Name%20Widget))))
  (bind _output_get (Variables|Default|SetPlayerName%20REF _asplayer_name_ui))
  (bind _asbp_game_instance (Utilities|Casting|CastToBP_GameInstance (Game|GetGameInstance)))
  (bind _array (Default|MakePlayerNameArray _asbp_game_instance))
  (Variables|/Game/UI/PlayerNameUI.PlayerNameUI_C|SetPlayerName _output_get (Utilities|Array|Get(acopy) _array (Variables|Default|GetplayerInt))))

(fn ControllerStartVibration
  (Game|Feedback|ClientPlayForceFeedback (Game|GetPlayerController (Variables|Default|GetplayerInt)) "/Game/Assets/vibration.vibration" "Vibration" true false false)
  (Development|PrintString "Vibration Started"))

(fn ControllerStopVibration
  (Game|Feedback|ClientStopForceFeedback (Game|GetPlayerController (Variables|Default|GetplayerInt)) "/Game/Assets/vibration.vibration" "None")
  (Development|PrintString "Vibration Stopped"))

(fn IsAimJoystickAboveDeadZone
  (return (> (Math|Vector2D|Vector2DLength (Math|Vector2D|MakeVector2D (Input|AxisValues|GetAimUp) (Input|AxisValues|GetAimRight))) (Variables|Default|GetJoyStickDeadZone))))

(fn IsMoveJoystickAboveDeadZone
  (return (> (Math|Vector2D|Vector2DLength (Math|Vector2D|MakeVector2D (Input|AxisValues|GetAimUp) (Input|AxisValues|GetAimRight))) (+ (Variables|Default|GetJoyStickDeadZone) 0.01))))

(fn ConstrutCharacterModel
  (Class|SkinnedMeshComponent|SetMasterPoseComponent (Variables|Default|GetGloves) (Variables|Character|GetMesh) false))

(fn IsAttacking
  (bind _mesh (Variables|Character|GetMesh))
  (bind _returnvalue (Components|SkeletalMesh|GetAnimInstance _mesh))
  (return (or (Animation|Montage|MontageIsPlaying _returnvalue "/Game/PartyMonsterRumblePA/Animation/AnimMontage_PlayerAtk_1.AnimMontage_PlayerAtk_1") (Animation|Montage|MontageIsPlaying _returnvalue "/Game/PartyMonsterRumblePA/Animation/AnimMontage_PlayerAtk_2.AnimMontage_PlayerAtk_2"))))

(fn IsPlayerActiveinThisRound
  (bind _asbp_game_instance (Utilities|Casting|CastToBP_GameInstance (Game|GetGameInstance)))
  (return false))

(fn ConsumeItem
  (params (Item%20REF :type Actor%20Object%20Reference))
  (Math|Integer|DecrementInt (Variables|/Game/Blueprint/BP_GameMode.BP_GameMode_C|GetSpawnedItemCount (Variables|Default|GetAs%20BP%20Game%20Mode))
    (:%20%20
      (Actor|DestroyActor Item%20REF))))

(fn StopAllAudio
  (bind _detector_item_pick_up_sound (Variables|Default|GetDetector%20Item%20Pick%20Up%20Sound))
  (Utilities|IsValid _detector_item_pick_up_sound
    (:Is%20Valid
      (Audio|Components|Audio|Stop _detector_item_pick_up_sound))
    (:Is%20Not%20Valid
      _))
  (return))

(fn ResumeGameSpeed
  (Development|ExecuteConsoleCommand "slomo 1" 0))

(fn PlayWinAnimation
  (switch int (Math|Random|RandomIntegerinRange 0 1)
    (:0
      (Animation|PlayAnimMontage "/Game/PartyMonsterRumblePA/Animation/Victory01_Anim_Montage.Victory01_Anim_Montage" 1.0 "None"))
    (:1
      (Animation|PlayAnimMontage "/Game/PartyMonsterRumblePA/Animation/Victory02_Anim_Montage.Victory02_Anim_Montage" 1.0 "None"))))

(fn SpeedUp
  (params (Item%20REF :type Actor%20Object%20Reference))
  (Audio|PlaySoundatLocation "/Game/Assets/Sounds/EnvironmentSFX/SpeedUp_Cue.SpeedUp_Cue" (Transformation|GetActorLocation) "0, 0, 0" 1.3 1.0 0.0 0 0 0)
  (Components|Activation|Activate (Variables|Default|GetSpeedUp%20Particle) false)
  (Development|PrintString (Utilities|String|Append "Player " (Utilities|String|ToString(Integer) (Variables|Default|GetplayerInt)) " Speed Up"))
  (if (Variables|Default|GetIsSpeedUp)
    _
    (else
      (Variables|Default|SetIsSpeedUp true)
      (Variables|Default|SetmoveSpeed (* (Variables|Default|GetmoveSpeed) (Variables|Default|GetSprint%20Multiplier)))))
  (CallFunction|ConsumeItem Item%20REF)
  (Variables|/Game/Blueprint/PVEMode/AnimBP_Player_PVE.AnimBP_Player_PVE_C|SetisSpeedUp%20REF (Variables|Default|GetAs%20Anim%20BP%20Player%20PVE) true)
  (return))

(fn SpeedDown
  (Variables|Default|SetmoveSpeed (/ (Variables|Default|GetmoveSpeed) (Variables|Default|GetSprint%20Multiplier)))
  (Variables|Default|SetIsSpeedUp false)
  (Variables|/Game/Blueprint/PVEMode/AnimBP_Player_PVE.AnimBP_Player_PVE_C|SetisSpeedUp%20REF (Variables|Default|GetAs%20Anim%20BP%20Player%20PVE) false))

(fn CacheAnimBP
  (bind _asanim_bp_player_pve (Utilities|Casting|CastToAnimBP_Player_PVE (Components|SkeletalMesh|GetAnimInstance (Variables|Character|GetMesh))))
  (Variables|Default|SetAs%20Anim%20BP%20Player%20PVE _asanim_bp_player_pve))

(fn CacheGameMode
  (bind _asbp_game_mode_pve (Utilities|Casting|CastToBP_GameMode_PVE (Game|GetGameMode)))
  (Variables|Default|SetAs%20BP%20Game%20Mode%20PVE _asbp_game_mode_pve))

(fn ApplyThrowForce
  (return (* (+ (Transformation|GetActorForwardVector) "0, 0,0.400000") (Math|Random|RandomFloatinRange (Variables|Default|GetThrow%20Force%20Min) (Variables|Default|GetThrow%20Force%20Max)))))

(fn ReleaseObject
  (params (ThrowForce :type Vector))
  (Utilities|IsValid (Variables|Default|GetPicked%20Up%20Mesh)
    (:Is%20Valid
      (Transformation|DetachFromActor (Variables|Default|GetPicked%20Up%20Mesh) "KeepWorld" "KeepWorld" "KeepWorld")
      (Collision|SetCollisionEnabled (Variables|/Game/Blueprint/BP_PickupItem.BP_PickupItem_C|GetBomb_Mesh (Variables|Default|GetPicked%20Up%20Mesh)) "QueryAndPhysics")
      (Physics|SetSimulatePhysics (Variables|/Game/Blueprint/BP_PickupItem.BP_PickupItem_C|GetBomb_Mesh (Variables|Default|GetPicked%20Up%20Mesh)) true)
      (Class|PrimitiveComponent|SetAllPhysicsLinearVelocity (Variables|/Game/Blueprint/BP_PickupItem.BP_PickupItem_C|GetBomb_Mesh (Variables|Default|GetPicked%20Up%20Mesh)) ThrowForce true)
      (Default|ResetPickupableStatus (Variables|Default|GetPicked%20Up%20Mesh))
      (Variables|Default|SetPicked%20Up%20Mesh 0)
      (Variables|Default|SetIn%20Animation false)
      (CallFunction|CancelHoldingAnimations)
      (Variables|Default|SetmoveSpeed (/ (Variables|Default|GetmoveSpeed) (Variables|Default|GetMovespeed%20penality)))
      (return))
    (:Is%20Not%20Valid
      (CallFunction|CancelHoldingAnimations)
      (Variables|Default|SetPicked%20Up%20Mesh 0))))

(fn FindItemtoPickUp
  (bind _returnvalue (Transformation|GetActorLocation))
  (bind _returnvalue_2 (- _returnvalue "0,0.000000,30.000000"))
  (Utilities|IsValid (Variables|Default|GetPicked%20Up%20Mesh)
    (:Is%20Not%20Valid
      (bind (_outhit _returnvalue_3) (Collision|SphereTraceByChannel _returnvalue_2 (+ _returnvalue_2 (* (Transformation|GetActorForwardVector) (Variables|Default|GetPickup%20Range))) 35.0 "TraceTypeQuery1" false 0 "None"))
      (if _returnvalue_3
        (bind _asbp_pickup_item (Utilities|Casting|CastToBP_PickupItem (.HitActor (Collision|BreakHitResult _outhit)))
          (:then
            (if (not (== _asbp_pickup_item (Variables|Default|GetPickup%20Target)))
              (if (Variables|/Game/Blueprint/BP_PickupItem.BP_PickupItem_C|GetisPickedUp _asbp_pickup_item)
                (Variables|Default|SetPickup%20Target 0)
                (Development|PrintString "THE BOMB IS PICKED UP")
                (else
                  (bind _output_get (Variables|Default|SetPickup%20Target _asbp_pickup_item))
                  (Development|PrintString (Utilities|GetDisplayName _output_get))))))
          (:CastFailed
            (Development|PrintString "***CAST FAILED***")
            (Utilities|IsValid (Variables|Default|GetPickup%20Target) :!label _label
              (:Is%20Valid
                (Variables|Default|SetPickup%20Target 0)
                (Development|PrintString "***IS VALID***"))
              (:Is%20Not%20Valid
                (Variables|Default|SetPickup%20Target 0)
                (Development|PrintString "***NOT VALID***")))))
        (else
          (goto _label))))))

(fn StartPickingUp
  (bind _pickup_target (Variables|Default|GetPickup%20Target))
  (Utilities|IsValid _pickup_target
    (:Is%20Valid
      (Variables|/Game/Blueprint/BP_PickupItem.BP_PickupItem_C|SetisPickedUp _pickup_target true)
      (Variables|/Game/Blueprint/PVEMode/AnimBP_Player_PVE.AnimBP_Player_PVE_C|SetisLifting (Variables|Default|GetAs%20Anim%20BP%20Player%20PVE) true)
      (bind _output_get (Variables|Default|SetPicked%20Up%20Mesh _pickup_target))
      (Physics|SetSimulatePhysics (Variables|/Game/Blueprint/BP_PickupItem.BP_PickupItem_C|GetBomb_Mesh _output_get) false)
      (Collision|SetCollisionEnabled (Variables|/Game/Blueprint/BP_PickupItem.BP_PickupItem_C|GetBomb_Mesh _output_get) "NoCollision")
      (Variables|Default|SetIn%20Animation true)
      (Variables|Default|SetmoveSpeed (* (Variables|Default|GetmoveSpeed) (Variables|Default|GetMovespeed%20penality))))))

(fn StartThrowing
  (Variables|/Game/Blueprint/PVEMode/AnimBP_Player_PVE.AnimBP_Player_PVE_C|SetisLifting (Variables|Default|GetAs%20Anim%20BP%20Player%20PVE) false))

(fn AttachObjecttoPlayer
  (bind _picked_up_mesh (Variables|Default|GetPicked%20Up%20Mesh))
  (Utilities|IsValid _picked_up_mesh
    (:Is%20Valid
      (Transformation|SetActorRotation _picked_up_mesh)
      (Transformation|AttachComponentToComponent _picked_up_mesh (Variables|Character|GetMesh) "Lifting Socket" "SnapToTarget" "KeepRelative" "KeepWorld" true))
    (:Is%20Not%20Valid
      (CallFunction|CancelHoldingAnimations))))

(fn CancelHoldingAnimations
  (bind _as_anim_bp_player_pve (Variables|Default|GetAs%20Anim%20BP%20Player%20PVE))
  (Variables|/Game/Blueprint/PVEMode/AnimBP_Player_PVE.AnimBP_Player_PVE_C|SetisLifting _as_anim_bp_player_pve false)
  (Variables|/Game/Blueprint/PVEMode/AnimBP_Player_PVE.AnimBP_Player_PVE_C|SetisThrowing _as_anim_bp_player_pve false))

(fn PlayHitFX
  (params (Location :type Vector))
  (Audio|PlaySoundatLocation "/Game/Assets/Sounds/EnvironmentSFX/Bump.Bump" Location "0, 0, 0" 1.0 1.0 0.0 0 0 0)
  (Effects|SpawnEmitteratLocation "/Game/Assets/Particles/Confetti/HitHead_P.HitHead_P" Location))

(fn IncreaseScore
  (if (Variables|/Game/Blueprint/PVEMode/BP_GameMode_PVE.BP_GameMode_PVE_C|GetFirstToScore (Variables|Default|GetAs%20BP%20Game%20Mode%20PVE))
    ;[1 1 1] Double Score for first punch
    (Variables|/Game/Blueprint/PVEMode/BP_GameMode_PVE.BP_GameMode_PVE_C|SetFirstToScore (Variables|Default|GetAs%20BP%20Game%20Mode%20PVE) false)
    (Variables|Default|SetScore (+ (Variables|Default|GetScore) (* (Variables|Default|GetCorrect%20Score) (Variables|Default|GetFirstToScoreMultiplier))))
    (else
      (Variables|Default|SetScore (+ (Variables|Default|GetScore) (Variables|Default|GetCorrect%20Score)))))
  (return))

(fn DecreaseScore
  (bind _output_get (Variables|Default|SetScore (- (Variables|Default|GetScore) (Variables|Default|GetIncorrect%20Score))))
  (Development|PrintString (Utilities|String|ToString(Integer) _output_get))
  (return))

(fn UpdateScoreUI
  (bind _score (Variables|Default|GetScore))
  (bind _as_bp_game_mode_pve (Variables|Default|GetAs%20BP%20Game%20Mode%20PVE))
  (bind _as_player_score_ui (Variables|/Game/Blueprint/PVEMode/BP_GameMode_PVE.BP_GameMode_PVE_C|GetAs%20Player%20Score%20UI _as_bp_game_mode_pve))
  (switch int (Variables|Default|GetplayerInt)
    (:0
      (Variables|/Game/Blueprint/PVEMode/PlayerScoreUI.PlayerScoreUI_C|SetPlayer%201%20Score%20Points _as_player_score_ui _score))
    (:1
      (Variables|/Game/Blueprint/PVEMode/PlayerScoreUI.PlayerScoreUI_C|SetPlayer%202%20Score%20Points _as_player_score_ui _score))
    (:2
      (Variables|/Game/Blueprint/PVEMode/PlayerScoreUI.PlayerScoreUI_C|SetPlayer%203%20Score%20Points _as_player_score_ui _score))
    (:3
      (Variables|/Game/Blueprint/PVEMode/PlayerScoreUI.PlayerScoreUI_C|SetPlayer%204%20Score%20Points _as_player_score_ui _score)))
  (return))