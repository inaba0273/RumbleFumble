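; BP_Bomb is a self-triggering bomb actor that starts its detonation sequence after a delay from BeginPlay.
; Explode lights the fuze effect and runs a looping timer that grows the bomb mesh until detonation.
; It then fires the explosion effect, applies radial falloff damage and destroys only the Bomb component, leaving the actor.
; Finally, it decrements SpawnedItemCount on BP_GameMode.
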(event Custom|Explode
  (Components|Activation|Activate (Variables|Default|GetFuze) false)
  (Utilities|Time|SetTimerbyFunctionName 0 "Bomb Scale Up" 0.1 true)
  (Utilities|FlowControl|Delay 5.0)
  (Components|Activation|Deactivate (Variables|Default|GetFuze))
  (Components|Activation|Activate (Variables|Default|GetExplosion) false)
  (Class|GameplayStatics|ApplyRadialDamagewithFalloff 55.0 2e+01 (Transformation|GetActorLocation) 5.0 5.6 2e+01 0 0 0 0 "ECC_Visibility")
  (Class|KismetSystemLibrary|PauseTimer 0 "Bomb Scale Up")
  (Components|DestroyComponent (Variables|Default|GetBomb))
  (bind _asbp_game_mode (Utilities|Casting|CastToBP_GameMode (Game|GetGameMode)))
  (Math|Integer|DecrementInt (Variables|/Game/Blueprint/BP_GameMode.BP_GameMode_C|GetSpawnedItemCount _asbp_game_mode)))

(event EventBeginPlay
  (Utilities|FlowControl|Delay 5.0)
  (CallFunction|Explode))

(event EventTick
  (params (DeltaSeconds :type Float%20%28single-precision%29)))

(fn ConstructionScript)

(fn BombScaleUp
  (Transformation|SetWorldScale3D (Variables|Default|GetBomb) (+ (Variables|Default|GetNew%20Scale) "0.100000,0.100000,0.100000"))
  (Variables|Default|SetNew%20Scale (+ (Variables|Default|GetNew%20Scale) "0.100000,0.100000,0.100000")))