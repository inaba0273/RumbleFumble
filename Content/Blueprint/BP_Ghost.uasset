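; Player-controlled ghost pawn that moves above a joystick dead zone and drops small bombs at its position.
; On BeginPlay it is possessed by its indexed controller and shows that player's name from the GameInstance, with aim material color set at construction.
; Bombs spawn at random heights, inherit scaled ghost velocity and are cooldown-gated by a DoOnce.
; A traitor ghost counts overlapping traitor players, looping controller vibration until none remain.
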(event OnComponentBeginOverlap(CollisionComponent)
  (params (OverlappedComponent :type Primitive%20Component%20Object%20Reference) (OtherActor :type Actor%20Object%20Reference) (OtherComp :type Primitive%20Component%20Object%20Reference) (OtherBodyIndex :type Integer) (bFromSweep :type Boolean) (SweepResult :type Hit%20Result%20Structure%20%28by%20ref%29))
  (bind _overlap_traitor_count (Variables|Default|GetOverlap%20Traitor%20Count))
  (if (Variables|Default|GetisTraitor)
    (bind _asbp_player (Utilities|Casting|CastToBP_Player OtherActor))
    (if (Variables|/Game/Blueprint/BP_Player.BP_Player_C|GetIsTraitor _asbp_player)
      (Math|Integer|IncrementInt _overlap_traitor_count
        (:%20%20
          (if (== _overlap_traitor_count 1)
            (CallFunction|StartVibration)))))))

(event OnComponentEndOverlap(CollisionComponent)
  (params (OverlappedComponent :type Primitive%20Component%20Object%20Reference) (OtherActor :type Actor%20Object%20Reference) (OtherComp :type Primitive%20Component%20Object%20Reference) (OtherBodyIndex :type Integer))
  (bind _overlap_traitor_count (Variables|Default|GetOverlap%20Traitor%20Count))
  (if (Variables|Default|GetisTraitor)
    (bind _asbp_player (Utilities|Casting|CastToBP_Player OtherActor))
    (if (Variables|/Game/Blueprint/BP_Player.BP_Player_C|GetIsTraitor _asbp_player)
      (Math|Integer|DecrementInt _overlap_traitor_count
        (:%20%20
          (if (== _overlap_traitor_count 0)
            (CallFunction|StopVibration)))))))

(event EventBeginPlay
  (CallFunction|PossesbyPlayer)
  (CallFunction|GetPlayerName)
  (CallFunction|GetPlayerColor))

(event Collision|EventActorBeginOverlap
  (params (OtherActor :type Actor%20Object%20Reference)))

(event EventTick
  (params (DeltaSeconds :type Float%20%28single-precision%29)))

(event Input|ActionEvents|InputActionPlayerAttack
  (params (Key :type Key%20Structure :default "None"))
  (bind _returnvalue (Transformation|GetActorLocation))
  (:Pressed
    (Utilities|FlowControl|DoOnce false :!label _label
      (:Completed
        (bind _returnvalue_2 (Game|SpawnActorfromClass "/Game/Blueprint/BP_SmallBomb.BP_SmallBomb_C" (Math|Transform|MakeTransform (Math|Vector|MakeVector (.x _returnvalue) (.y _returnvalue) (Math|Random|RandomFloatinRange (Variables|Default|GetSpawn%20Height%20Min) (Variables|Default|GetSpawn%20Height%20Max))) (Math|Random|RandomRotator false) "8.000000,8.000000,8.000000") "Undefined" 0 0))
        (Physics|SetPhysicsLinearVelocity (Variables|/Game/Blueprint/BP_PickupItem.BP_PickupItem_C|GetBomb_Mesh _returnvalue_2) (* (Transformation|GetVelocity) (Variables|Default|GetVelocity%20Multiplier)) false "None")
        (Utilities|FlowControl|Delay (Variables|Default|GetSpawn%20Cooldown))
        (goto _label Reset)))))

(event Input|AxisEvents|InputAxisMoveForward
  (params (AxisValue :type Float%20%28single-precision%29))
  (if (CallFunction|IsMoveJoystickAboveDeadZone)
    (Pawn|Input|AddMovementInput (Math|Vector|MakeVector (Variables|Default|GetmoveSpeed) 0.0 0.0) AxisValue false)))

(event Input|AxisEvents|InputAxisMoveRight
  (params (AxisValue :type Float%20%28single-precision%29))
  (if (CallFunction|IsMoveJoystickAboveDeadZone)
    (Pawn|Input|AddMovementInput (Math|Vector|MakeVector 0.0 (Variables|Default|GetmoveSpeed) 0.0) AxisValue false)))

(fn ConstructionScript
  (bind _returnvalue (Rendering|Material|CreateDynamicMaterialInstance (Variables|GetMeshComponent) 0 "/Game/Assets/Particles/AimTarget/M_Aim.M_Aim" "None" :!class /Script/Engine.PrimitiveComponent))
  (bind _output_get (Variables|Default|SetMaterial%20Instance _returnvalue))
  (Rendering|Material|SetVectorParameterValue _output_get "Color" (Variables|Default|GetColor) :!class /Script/Engine.MaterialInstanceDynamic))

(fn IsMoveJoystickAboveDeadZone
  (return (> (Math|Vector2D|Vector2DLength (Math|Vector2D|MakeVector2D (Input|AxisValues|GetAimUp) (Input|AxisValues|GetAimRight))) (+ (Variables|Default|GetJoyStickDeadZone) 0.01))))

(fn PossesbyPlayer
  (bind _player_int (Variables|Default|GetPlayer%20Int))
  (Pawn|Possess (Game|GetPlayerController _player_int) self)
  (Development|PrintString (Utilities|String|Append "Player " (Utilities|String|ToString(Integer) _player_int) " Possesed")))

(fn GetPlayerName
  (bind _asbp_game_instance (Utilities|Casting|CastToBP_GameInstance (Game|GetGameInstance)))
  (bind _output_get (Variables|Default|SetPlayer%20Name (Utilities|Array|Get(acopy) (Variables|/Game/UI/BP_GameInstance.BP_GameInstance_C|GetPlayer%20Name%20Array _asbp_game_instance) (Variables|Default|GetPlayer%20Int))))
  (bind _asplayer_name_ui (Utilities|Casting|CastToPlayerNameUI (UserInterface|GetUserWidgetObject (Variables|Default|GetWidget))))
  (Variables|/Game/UI/PlayerNameUI.PlayerNameUI_C|SetPlayerName _asplayer_name_ui _output_get))

(fn GetPlayerColor)

(fn StartVibration
  (Game|Feedback|ClientPlayForceFeedback (Game|GetPlayerController (Variables|Default|GetPlayer%20Int)) "/Game/Assets/vibration.vibration" "Vibration" true false false))

(fn StopVibration
  (Game|Feedback|ClientStopForceFeedback (Game|GetPlayerController (Variables|Default|GetPlayer%20Int)) "/Game/Assets/vibration.vibration" "Vibration"))