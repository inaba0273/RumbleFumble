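; BP_Player_Male is the male player character Blueprint, extending a parent class that supplies its BeginPlay and construction behavior.
; It adds a melee attack on the PlayerAttack input action, playing an attack montage on the mesh.
; The attack is blocked while the character is already attacking, dead, carrying a bomb or not allowed to attack.
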(event EventBeginPlay
  (|CallParentFunction))

(event Collision|EventActorBeginOverlap
  (params (OtherActor :type Actor%20Object%20Reference)))

(event EventTick
  (params (DeltaSeconds :type Float%20%28single-precision%29)))

(event Input|ActionEvents|InputActionPlayerAttack
  (params (Key :type Key%20Structure :default "None"))
  (:Pressed
    (if (not (Math|Boolean|ORBoolean (CallFunction|IsAttacking) (Variables|Default|GetDead) (Variables|Default|GetHas%20Bomb) (not (Variables|Default|GetCanAttack))))
      (Animation|Montage|PlayMontage (Variables|Character|GetMesh) "/Game/Toony_Tiny_Citizens/Animations/Male/melee/Anim_m_melee_combat_attack_A_Montage.Anim_m_melee_combat_attack_A_Montage"))))

(fn ConstructionScript
  (|CallParentFunction))