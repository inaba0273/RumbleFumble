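; Four-sided pipe actor that teleports overlapping actors through to the opposite side.
; Each of the left, right, top and down entry boxes passes its opposite exit box and arrow to a shared Teleport function.
; Teleport plays a sound at the entry location, moves any actor to the exit without sweeping, then launches only BP_Player along the exit arrow, scaled by TeleportForce.
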(event OnComponentBeginOverlap(Box_In_Left)
  (params (OverlappedComponent :type Primitive%20Component%20Object%20Reference) (OtherActor :type Actor%20Object%20Reference) (OtherComp :type Primitive%20Component%20Object%20Reference) (OtherBodyIndex :type Integer) (bFromSweep :type Boolean) (SweepResult :type Hit%20Result%20Structure%20%28by%20ref%29))
  (CallFunction|Teleport OtherActor (Variables|Default|GetBox_Out_Right) (Variables|Default|GetArrow_Right)))

(event OnComponentBeginOverlap(Box_In_Top)
  (params (OverlappedComponent :type Primitive%20Component%20Object%20Reference) (OtherActor :type Actor%20Object%20Reference) (OtherComp :type Primitive%20Component%20Object%20Reference) (OtherBodyIndex :type Integer) (bFromSweep :type Boolean) (SweepResult :type Hit%20Result%20Structure%20%28by%20ref%29))
  (CallFunction|Teleport OtherActor (Variables|Default|GetBox_Out_Down) (Variables|Default|GetArrow_Down)))

(event OnComponentBeginOverlap(Box_In_Down)
  (params (OverlappedComponent :type Primitive%20Component%20Object%20Reference) (OtherActor :type Actor%20Object%20Reference) (OtherComp :type Primitive%20Component%20Object%20Reference) (OtherBodyIndex :type Integer) (bFromSweep :type Boolean) (SweepResult :type Hit%20Result%20Structure%20%28by%20ref%29))
  (CallFunction|Teleport OtherActor (Variables|Default|GetBox_Out_Top) (Variables|Default|GetArrow_Top)))

(event OnComponentBeginOverlap(Box_In_Right)
  (params (OverlappedComponent :type Primitive%20Component%20Object%20Reference) (OtherActor :type Actor%20Object%20Reference) (OtherComp :type Primitive%20Component%20Object%20Reference) (OtherBodyIndex :type Integer) (bFromSweep :type Boolean) (SweepResult :type Hit%20Result%20Structure%20%28by%20ref%29))
  (CallFunction|Teleport OtherActor (Variables|Default|GetBox_Out_Left) (Variables|Default|GetArrow_Left)))

(event EventBeginPlay)

(event Collision|EventActorBeginOverlap
  (params (OtherActor :type Actor%20Object%20Reference)))

(event EventTick
  (params (DeltaSeconds :type Float%20%28single-precision%29)))

(fn ConstructionScript)

(fn Teleport
  (params (Teleport%20Actor :type Actor%20Object%20Reference) (Out%20Destination :type Scene%20Component%20Object%20Reference) (Out%20Direction :type Scene%20Component%20Object%20Reference))
  (LocalVariables|SetTeleport%20Actor%20REF Teleport%20Actor)
  (LocalVariables|SetTeleport%20Direction%20REF Out%20Direction)
  (LocalVariables|SetTeleport%20Destination%20REF Out%20Destination)
  (Audio|SpawnSoundatLocation "/Game/Assets/Sounds/Teleport_SoundCue.Teleport_SoundCue" (Transformation|GetActorLocation (LocalVariables|GetTeleport%20Actor%20REF)) "0, 0, 0" 1.0 1.0 0.0 0 0)
  (Transformation|SetActorLocation Teleport%20Actor (Transformation|GetWorldLocation (LocalVariables|GetTeleport%20Destination%20REF)) false true)
  (bind _asbp_player (Utilities|Casting|CastToBP_Player (LocalVariables|GetTeleport%20Actor%20REF)))
  (Character|LaunchCharacter _asbp_player (* (Math|Vector|GetForwardVector (LocalVariables|GetTeleport%20Direction%20REF)) (Variables|Default|GetTeleport%20Force)) false false))