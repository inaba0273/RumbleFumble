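; BP_Boundary is a boundary actor that handles players and items overlapping it.
; An overlapping BP_Player takes heavy fixed damage.
; An overlapping attack item or traitor detector is destroyed, and SpawnedItemCount on the BP_GameMode cached at BeginPlay is decremented.
; The IsPlayer and IsItem helpers use exact class comparisons, so subclasses do not match.
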(event EventBeginPlay
  (bind _asbp_game_mode (Utilities|Casting|CastToBP_GameMode (Game|GetGameMode)))
  (Variables|Default|SetAs%20BP%20Game%20Mode _asbp_game_mode))

(event EventTick
  (params (DeltaSeconds :type Float%20%28single-precision%29)))

(event Collision|EventActorBeginOverlap
  (params (OtherActor :type Actor%20Object%20Reference))
  (if (CallFunction|IsPlayer OtherActor)
    (Game|Damage|ApplyDamage OtherActor 1e+03 0 0)
    (elif (CallFunction|IsItem OtherActor)
      (Actor|DestroyActor OtherActor)
      (Math|Integer|DecrementInt (Variables|/Game/Blueprint/BP_GameMode.BP_GameMode_C|GetSpawnedItemCount (Variables|Default|GetAs%20BP%20Game%20Mode))))))

(fn ConstructionScript)

(fn IsItem
  (params (Object :type Object%20Object%20Reference))
  (bind _returnvalue (Utilities|GetClass Object))
  (return (or (== _returnvalue "/Game/Blueprint/BP_AttackItem.BP_AttackItem_C") (== _returnvalue "/Game/Blueprint/BP_TraitorDetector.BP_TraitorDetector_C"))))

(fn IsPlayer
  (params (Object :type Object%20Object%20Reference))
  (return (== (Utilities|GetClass Object) "/Game/Blueprint/BP_Player.BP_Player_C")))