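; BP_SpinTable is an actor that starts spinning slowly around its yaw axis once the tutorial ends.
; On BeginPlay it binds to the tutorial-ended event of BP_GameMode, or BP_GameMode_PVE as fallback, then randomizes its minimum and maximum spin step.
; When that event fires, a looping timer at roughly 60 Hz adds a random local yaw within those bounds, independent of Tick.
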(event Custom|On%20Tutprial%20Ends
  (Utilities|Time|SetTimerbyEvent (delegate Custom|Start%20Rotation) 0.0166 true))

(event Custom|Start%20Rotation
  (Transformation|AddActorLocalRotation (Math|Rotator|MakeRotator 0.0 0.0 (Math|Random|RandomFloatinRange (Variables|Default|GetMin) (Variables|Default|GetMax))) false false))

(event EventBeginPlay
  (bind _returnvalue (Game|GetGameMode))
  (bind _asbp_game_mode (Utilities|Casting|CastToBP_GameMode _returnvalue)
    (:then
      (EventDispatchers|BindEventtoTutorialEnded _asbp_game_mode (delegate Custom|On%20Tutprial%20Ends)))
    (:CastFailed
      (bind _asbp_game_mode_pve (Utilities|Casting|CastToBP_GameMode_PVE _returnvalue))
      (EventDispatchers|BindEventtoTutorialEnded _asbp_game_mode_pve (delegate Custom|On%20Tutprial%20Ends))))
  (Variables|Default|SetMin (Math|Random|RandomFloatinRange 0.15 0.2))
  (Variables|Default|SetMax (Math|Random|RandomFloatinRange 0.25 0.3)))

(event Collision|EventActorBeginOverlap
  (params (OtherActor :type Actor%20Object%20Reference)))

(fn ConstructionScript)