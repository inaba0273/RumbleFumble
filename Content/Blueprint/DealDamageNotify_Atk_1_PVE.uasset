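; Anim notify state for a PVE melee attack that plays a swing sound on begin and deals damage on end.
; At the end, a sphere trace between the right hand and right lower-jaw sockets applies fixed damage to whatever it hits.
; Punch sound and particles follow only for hit players, or enemies hit by a player, and only while that player is not flickering; the damage itself ignores flickering.
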(fn ReceivedNotifyEnd
  (params (MeshComp :type Skeletal%20Mesh%20Component%20Object%20Reference) (Animation :type Anim%20Sequence%20Base%20Object%20Reference))
  (bind _returnvalue (Components|GetOwner MeshComp))
  (bind (_outhit _returnvalue_2) (Collision|SphereTraceByChannel MeshComp (Transformation|GetSocketLocation MeshComp "hand_r") (Transformation|GetSocketLocation MeshComp "LowerJaw_r") 35.0 "TraceTypeQuery2" false 0 "None"))
  (if _returnvalue_2
    (Game|Damage|ApplyDamage (.hitactor _outhit) 1e+01 (Variables|Default|GetEvent%20Instigator) (Components|GetOwner MeshComp))
    (if (== (Utilities|GetClass (.hitactor _outhit)) "/Game/Blueprint/PVEMode/BP_Player_PVE.BP_Player_PVE_C")
      (bind _asbp_player_pve (Utilities|Casting|CastToBP_Player_PVE (.hitactor _outhit)))
      (if (not (Variables|/Game/Blueprint/PVEMode/BP_Player_PVE.BP_Player_PVE_C|GetisFlickering _asbp_player_pve))
        (Audio|SpawnSoundatLocation _returnvalue "/Game/Assets/Sounds/Punch/Player_Punch_SpounCue.Player_Punch_SpounCue" (Transformation|GetWorldLocation MeshComp) "0, 0, 0" 1.0 1.0 0.0 0 0 :!label _label)
        (Effects|SpawnEmitteratLocation (.hitactor _outhit) "/Game/Assets/Particles/Confetti/Punch_P.Punch_P" (.location _outhit))
        (return false))
      (else
        (bind _asbp_player_pve_2 (Utilities|Casting|CastToBP_Player_PVE _returnvalue))
        (if (and (not (Variables|/Game/Blueprint/PVEMode/BP_Player_PVE.BP_Player_PVE_C|GetisFlickering _asbp_player_pve_2)) (== (Utilities|GetClass (.hitactor _outhit)) "/Game/Blueprint/PVEMode/BP_Enemy_PVE.BP_Enemy_PVE_C"))
          (goto _label))))))

(fn ReceivedNotifyBegin
  (params (MeshComp :type Skeletal%20Mesh%20Component%20Object%20Reference) (Animation :type Anim%20Sequence%20Base%20Object%20Reference) (TotalDuration :type Float%20%28single-precision%29))
  (Audio|SpawnSoundatLocation MeshComp "/Game/Assets/Sounds/Punch/Player_Swing_SoundCue.Player_Swing_SoundCue" (Transformation|GetWorldLocation MeshComp) "0, 0, 0" 1.0 1.0 0.0 0 0)
  (return false))