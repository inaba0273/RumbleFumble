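; Player character for a local multiplayer innocents-versus-traitors game, identified by PlayerInt for spawn point, color, modular-mesh material and controller.
; It handles movement, a two-montage attack combo, health UI, and death that decrements GameMode team counts to show the win message.
; Overlap counting rumbles the pad near traitors for traitors or holders of the timed detective power.
; Bombs are grabbed by sphere trace, carried by a timer-updated PhysicsHandle, then thrown.
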(event Custom|PlayerHasDetecivePower
  (bind _playerint (Variables|Default|GetplayerInt))
  ;[1 1 1] Gets the effect, last for a duration of time then lost the effect, force stop vibration
  (Variables|Default|SethasDetectiveItem true)
  (Rendering|SetVisibility (Variables|Default|GetDetectorCollider) true false)
  (Development|PrintString (Utilities|String|Append "Player " (Utilities|String|ToString(Integer) _playerint) " Get the Detecive Power!") true true "(R=0.000000,G=0.660000,B=1.000000,A=1.000000)" 5.0)
  (Utilities|FlowControl|RetriggerableDelay (Variables|Default|GetDetective%20Item%20Duration))
  (bind _asbp_game_mode (Utilities|Casting|CastToBP_GameMode (Game|GetGameMode)))
  (Variables|/Game/UI/LoseItemUI.LoseItemUI_C|SetPlayer%20Int%20REF (Variables|/Game/Blueprint/BP_GameMode.BP_GameMode_C|GetLoseItemUI%20REF _asbp_game_mode) (Variables|Default|GetplayerInt))
  (if (UserInterface|Viewport|IsinViewport (Variables|/Game/Blueprint/BP_GameMode.BP_GameMode_C|GetLoseItemUI%20REF _asbp_game_mode))
    _
    (else
      (UserInterface|Viewport|AddtoViewport (Variables|/Game/Blueprint/BP_GameMode.BP_GameMode_C|GetLoseItemUI%20REF _asbp_game_mode) 0)))
  (Variables|Default|SethasDetectiveItem false)
  (Rendering|SetVisibility (Variables|Default|GetDetectorCollider) false false)
  (Development|PrintString (Utilities|String|Append "Player " (Utilities|String|ToString(Integer) _playerint) " Lost the Detecive Power!") true true "(R=0.000000,G=0.660000,B=1.000000,A=1.000000)" 5.0)
  (CallFunction|ControllerStopVibration))

(event Collision|EventActorBeginOverlap
  (params (OtherActor :type Actor%20Object%20Reference))
  ;[1 1 1] Check if overlap with traitor
  (bind _asbp_player (Utilities|Casting|CastToBP_Player OtherActor))
  (if (Variables|BP_Player_C|GetIsTraitor _asbp_player)
    ;[1 1 1] Handle if player overlap with traitor before getting the item
    (Variables|Default|SetIsOverlappingWithTraitor true)
    ;[1 1 1] Increase Overlapping traitor count
    (bind _result (Math|Integer|IncrementInt (Variables|Default|GetOverlap%20Traitor%20Count))
      (:%20%20
        ;[1 1 1] Only start vibration for the 1st overlap
        (if (== _result 1)
          ;[1 1 1] Controller vibrates only when have the detective power
          (if (or (Variables|Default|GethasDetectiveItem) (Variables|Default|GetIsTraitor))
            (CallFunction|ControllerStartVibration)))))))

(event Game|Damage|EventAnyDamage
  (params (Damage :type Float%20%28single-precision%29) (DamageType :type Damage%20Type%20Object%20Reference) (InstigatedBy :type Controller%20Object%20Reference) (DamageCauser :type Actor%20Object%20Reference))
  (bind _mesh (Variables|Character|GetMesh))
  (if (Animation|Montage|MontageIsPlaying (Components|SkeletalMesh|GetAnimInstance _mesh) "/Game/PartyMonsterRumblePA/Animation/AnimMontage_PlayerGetHit.AnimMontage_PlayerGetHit")
    _
    (else
      (Animation|Montage|PlayMontage _mesh "/Game/PartyMonsterRumblePA/Animation/AnimMontage_PlayerGetHit.AnimMontage_PlayerGetHit"
        (:then
          _))))
  ;[1 1 1] Decrease Health when damaged
  (bind _health (CallFunction|DecreaseHealth Damage))
  (Development|PrintString (Utilities|String|Append "Player " (Utilities|String|ToString(Integer) (Variables|Default|GetplayerInt)) "  health decreased by " (Utilities|String|ToString(Float) Damage) ", current health is " (Utilities|String|ToString(Float) _health)))
  (CallFunction|UpdateHealthUI)
  (if (<= _health 0.0)
    (CallFunction|PlayerDead)
    (CallFunction|CheckWinCondition)))

(event Collision|EventActorEndOverlap
  (params (OtherActor :type Actor%20Object%20Reference))
  ;[1 1 1] Check if overlap with traitor
  (bind _asbp_player (Utilities|Casting|CastToBP_Player OtherActor))
  (if (Variables|BP_Player_C|GetIsTraitor _asbp_player)
    ;[1 1 1] Decrease Overlapping traitor count
    (bind _result (Math|Integer|DecrementInt (Variables|Default|GetOverlap%20Traitor%20Count))
      (:%20%20
        ;[1 1 1] Only stop vibration for the last overlap
        (if (== _result 0)
          (Variables|Default|SetIsOverlappingWithTraitor false)
          (if (or (Variables|Default|GethasDetectiveItem) (Variables|Default|GetIsTraitor))
            (CallFunction|ControllerStopVibration)))))))

(event EventBeginPlay
  (CallFunction|ConstrutCharacterModel)
  ;[1 1 1] Spawn Player and Set Player Color
  (CallFunction|SpawnFunction)
  (CallFunction|SetPlayerPawnColor)
  ;[1 1 1] Cast to HealthUI and set Health Bar color
  (CallFunction|GetHealthUIReference)
  ;[1 1 1] Cast to Player Name UI and set Player Name
  (Utilities|FlowControl|Delay 0.2)
  (CallFunction|DisplayPlayerNameUI))

(event Input|ActionEvents|InputActionPickUpBomb
  (params (Key :type Key%20Structure :default "None"))
  (bind _self self)
  (bind _pick_up_bomb_ref (Variables|Default|GetPick%20Up%20Bomb%20REF))
  (bind _returnvalue (Transformation|GetActorForwardVector _self))
  (:Pressed
    (if (Variables|Default|GetHas%20Bomb)
      (Physics|Components|PhysicsHandle|ReleaseComponent (Variables|Default|GetPhysicsHandle))
      (Variables|Default|SetHas%20Bomb false)
      (Class|PrimitiveComponent|SetAllPhysicsLinearVelocity _pick_up_bomb_ref (Math|Vector|MakeVector (* 1000 (.x _returnvalue)) (* 1000 (.y _returnvalue)) 5e+02) true)
      (Utilities|FlowControl|Delay 0.3)
      (Utilities|IsValid _pick_up_bomb_ref
        (:Is%20Valid
          (Collision|SetCollisionResponsetoChannel _pick_up_bomb_ref "ECC_Pawn" "ECR_Block")))
      (else
        (CallFunction|PickUpBomb)))))

(event Input|ActionEvents|InputActionPlayerAttack
  (params (Key :type Key%20Structure :default "None"))
  (:Pressed
    (if (not (Math|Boolean|ORBoolean (CallFunction|IsAttacking) (Variables|Default|GetDead) (Variables|Default|GetHas%20Bomb)))
      (switch int (Variables|Default|GetAttackCounter)
        (:0
          (Variables|Default|SetAttackCounter 1)
          (Animation|Montage|PlayMontage (Variables|Character|GetMesh) "/Game/PartyMonsterRumblePA/Animation/AnimMontage_PlayerAtk_1.AnimMontage_PlayerAtk_1" 1.1
            (:OnCompleted
              (Variables|Default|SetAttackCounter 0))))
        (:1
          (Variables|Default|SetAttackCounter 0)
          (Animation|Montage|PlayMontage (Variables|Character|GetMesh) "/Game/PartyMonsterRumblePA/Animation/AnimMontage_PlayerAtk_2.AnimMontage_PlayerAtk_2" 1.1))))))

(event Input|AxisEvents|InputAxisMoveForward
  (params (AxisValue :type Float%20%28single-precision%29))
  ;[1 1 1] Basic Movements
  (if (Math|Boolean|ANDBoolean (CallFunction|IsMoveJoystickAboveDeadZone) (CallFunction|IsAlive) (not (CallFunction|IsAttacking)))
    (Pawn|Input|AddMovementInput (Math|Vector|MakeVector (Variables|Default|GetmoveSpeed) 0.0 0.0) AxisValue false)
    (CallFunction|CharacterRotation)))

(event Input|AxisEvents|InputAxisMoveRight
  (params (AxisValue :type Float%20%28single-precision%29))
  ;[1 1 1] Basic Movements
  (if (Math|Boolean|ANDBoolean (CallFunction|IsMoveJoystickAboveDeadZone) (CallFunction|IsAlive) (not (CallFunction|IsAttacking)))
    (Pawn|Input|AddMovementInput (Math|Vector|MakeVector 0.0 (Variables|Default|GetmoveSpeed) 0.0) AxisValue false)
    (CallFunction|CharacterRotation)))

(fn ConstructionScript)

(fn SpawnFunction
  ;[1 1 1] Get All Possible Spawn Point In The Level
  (bind _outactors (Actor|GetAllActorsOfClass "/Script/Engine.PlayerStart"))
  (for _array_element _outactors
    ;[1 1 1] Set Player Spawn Point
    (if (Utilities|Name|Equal(Name) (Variables|/Script/Engine.PlayerStart|GetPlayerStartTag _array_element) (Utilities|String|StringToName (Utilities|String|Append "player" (Utilities|String|ToString(Integer) (Variables|Default|GetplayerInt)))))
      (bind _output_get (Variables|Default|SetspawnLocation (Transformation|GetActorTransform _array_element)))
      (Transformation|SetActorTransform _output_get false true))))

(fn SetPlayerPawnColor
  (switch int (Variables|Default|GetplayerInt)
    (:0
      (Variables|Default|SetCurrentPlayerColor (Variables|Default|GetPlayer1Color))
      (return))
    (:1
      (Variables|Default|SetCurrentPlayerColor (Variables|Default|GetPlayer2Color))
      (return))
    (:2
      (Variables|Default|SetCurrentPlayerColor (Variables|Default|GetPlayer3Color))
      (return))
    (:3
      (Variables|Default|SetCurrentPlayerColor (Variables|Default|GetPlayer4Color))
      (return))
    (:4
      (Variables|Default|SetCurrentPlayerColor (Variables|Default|GetPlayer5Color))
      (return))
    (:5
      (Variables|Default|SetCurrentPlayerColor (Variables|Default|GetPlayer6Color))
      (return))
    (:6
      (Variables|Default|SetCurrentPlayerColor (Variables|Default|GetPlayer7Color)))
    (:7
      (Variables|Default|SetCurrentPlayerColor (Variables|Default|GetPlayer8Color))
      (return))))

(fn DealDamage
  (params (DamagedActor :type Actor%20Object%20Reference))
  (Game|Damage|ApplyDamage DamagedActor (Variables|Default|GetDamage%20Amount) 0 0))

(fn DecreaseHealth
  (params (Damage :type Float%20%28single-precision%29))
  (bind _output_get (Variables|Default|SetPlayer%20Health (- (Variables|Default|GetPlayer%20Health) Damage)))
  (return _output_get))

(fn CharacterRotation
  (Pawn|SetControlRotation (Game|GetPlayerController (Variables|Default|GetplayerInt)) (Math|Rotator|MakeRotator 0.0 0.0 (Class|KismetMathLibrary|DegAtan2 (Input|AxisValues|GetAimRight) (Input|AxisValues|GetAimUp)))))

(fn IsAlive
  (return (not (Variables|Default|GetDead))))

(fn GetReferencefromHealthUI
  (bind _ashealth_ui (Utilities|Casting|CastToHealthUI (UserInterface|GetUserWidgetObject (Variables|Default|GetHealth%20Bar))))
  (Variables|Default|SetHealth%20Widget%20REF _ashealth_ui))

(fn SetHealthBarColor
  (Appearance|SetColorandOpacity (Variables|Default|GetHealth%20Widget%20REF) (Variables|Default|GetCurrentPlayerColor) :!class /Script/UMG.UserWidget))

(fn DisplayPlayerNameUI
  (bind _asplayer_name_ui (Utilities|Casting|CastToPlayerNameUI (UserInterface|GetUserWidgetObject (Variables|Default|GetPlayer%20Name%20Widget))))
  (bind _output_get (Variables|Default|SetPlayerName%20REF _asplayer_name_ui))
  (Variables|/Game/UI/PlayerNameUI.PlayerNameUI_C|SetPlayerName _output_get (Utilities|Text|ToText(String) (Utilities|String|Append "Player " (Utilities|String|ToString(Integer) (Variables|Default|GetplayerInt))))))

(fn GetHealthUIReference
  (bind _ashealth_ui (Utilities|Casting|CastToHealthUI (UserInterface|GetUserWidgetObject (Variables|Default|GetHealth%20Bar))))
  (bind _output_get (Variables|Default|SetHealth%20Widget%20REF _ashealth_ui))
  (Appearance|SetColorandOpacity _output_get (Variables|Default|GetCurrentPlayerColor) :!class /Script/UMG.UserWidget))

(fn ControllerStartVibration
  (Game|Feedback|ClientPlayForceFeedback (Game|GetPlayerController (Variables|Default|GetplayerInt)) "/Game/Assets/vibration.vibration" "Vibration" true false false)
  (Development|PrintString "Vibration Started"))

(fn ControllerStopVibration
  (Game|Feedback|ClientStopForceFeedback (Game|GetPlayerController (Variables|Default|GetplayerInt)) "/Game/Assets/vibration.vibration" "None")
  (Development|PrintString "Vibration Stopped"))

(fn CheckifAnyTraitorNearby
  (params (Object :type Object%20Object%20Reference))
  (bind _asbp_player (Utilities|Casting|CastToBP_Player Object))
  (if (Variables|BP_Player_C|GetIsTraitor _asbp_player)
    (bind _output_get (Variables|Default|SetOverlap%20Traitor%20Count (+ (Variables|Default|GetOverlap%20Traitor%20Count) 1)))
    (if (== _output_get 1)
      (return))))

(fn CheckifNoTraitorNearby
  (params (Object :type Object%20Object%20Reference))
  (bind _asbp_player (Utilities|Casting|CastToBP_Player Object))
  (if (Variables|BP_Player_C|GetIsTraitor _asbp_player)
    (bind _output_get (Variables|Default|SetOverlap%20Traitor%20Count (- (Variables|Default|GetOverlap%20Traitor%20Count) 1)))
    (if (== _output_get 0)
      (return))))

(fn InnocentCountDecrease
  (bind _asbp_game_mode (Utilities|Casting|CastToBP_GameMode (Game|GetGameMode)))
  (bind _result (Math|Integer|DecrementInt (Variables|/Game/Blueprint/BP_GameMode.BP_GameMode_C|GetInnocent%20Count _asbp_game_mode))
    (:%20%20
      (return _result))))

(fn TraitorCountDecrease
  (bind _asbp_game_mode (Utilities|Casting|CastToBP_GameMode (Game|GetGameMode)))
  (bind _result (Math|Integer|DecrementInt (Variables|/Game/Blueprint/BP_GameMode.BP_GameMode_C|GetTraitor%20Count _asbp_game_mode))
    (:%20%20
      (return _result))))

(fn IsAimJoystickAboveDeadZone
  (return (> (Math|Vector2D|Vector2DLength (Math|Vector2D|MakeVector2D (Input|AxisValues|GetAimUp) (Input|AxisValues|GetAimRight))) (Variables|Default|GetJoyStickDeadZone))))

(fn IsMoveJoystickAboveDeadZone
  (return (> (Math|Vector2D|Vector2DLength (Math|Vector2D|MakeVector2D (Input|AxisValues|GetAimUp) (Input|AxisValues|GetAimRight))) (+ (Variables|Default|GetJoyStickDeadZone) 0.01))))

(fn PlayerDead
  (Variables|Default|SetDead true)
  (Pawn|Components|CharacterMovement|DisableMovement (Variables|Character|GetCharacterMovement))
  (Components|Animation|PlayAnimation (Variables|Character|GetMesh) "/Game/PartyMonsterRumblePA/Animation/Die01_Anim.Die01_Anim" false)
  (Collision|SetActorEnableCollision self false)
  (Rendering|SetVisibility (Variables|Default|GetHealth%20Bar) false false))

(fn ConstrutCharacterModel
  (bind _mesh (Variables|Character|GetMesh))
  (Variables|Default|SetModular%20Parts (Utilities|Array|MakeArray (Variables|Default|GetGloves) (Variables|Default|GetBodyparts) (Variables|Default|GetEyes) (Variables|Default|GetMouths) (Variables|Default|GetNoses) (Variables|Default|GetTails) (Variables|Default|GetHeadparts) _mesh))
  (Class|SkinnedMeshComponent|SetMasterPoseComponent (Variables|Default|GetGloves) _mesh false)
  (switch int (Variables|Default|GetplayerInt)
    (:0
      (Rendering|Material|SetMaterial (Variables|Default|GetModular%20Parts) 0 "/Game/PartyMonsterRumblePA/Material/MaterialInstances/PlayerMaterial/PlayerMaterial_Inst.PlayerMaterial_Inst"))
    (:1
      (Rendering|Material|SetMaterial (Variables|Default|GetModular%20Parts) 0 "/Game/PartyMonsterRumblePA/Material/MaterialInstances/PlayerMaterial/PlayerMaterial_Inst_2.PlayerMaterial_Inst_2"))
    (:2
      (Rendering|Material|SetMaterial (Variables|Default|GetModular%20Parts) 0 "/Game/PartyMonsterRumblePA/Material/MaterialInstances/PlayerMaterial/PlayerMaterial_Inst_3.PlayerMaterial_Inst_3"))
    (:3
      (Rendering|Material|SetMaterial (Variables|Default|GetModular%20Parts) 0 "/Game/PartyMonsterRumblePA/Material/MaterialInstances/PlayerMaterial/PlayerMaterial_Inst_4.PlayerMaterial_Inst_4"))
    (:4
      (Rendering|Material|SetMaterial (Variables|Default|GetModular%20Parts) 0 "/Game/PartyMonsterRumblePA/Material/MaterialInstances/PlayerMaterial/PlayerMaterial_Inst_5.PlayerMaterial_Inst_5"))
    (:5
      (Rendering|Material|SetMaterial (Variables|Default|GetModular%20Parts) 0 "/Game/PartyMonsterRumblePA/Material/MaterialInstances/PlayerMaterial/PlayerMaterial_Inst_6.PlayerMaterial_Inst_6"))
    (:6
      (Rendering|Material|SetMaterial (Variables|Default|GetModular%20Parts) 0 "/Game/PartyMonsterRumblePA/Material/MaterialInstances/PlayerMaterial/PlayerMaterial_Inst_7.PlayerMaterial_Inst_7"))
    (:7
      (Rendering|Material|SetMaterial (Variables|Default|GetModular%20Parts) 0 "/Game/PartyMonsterRumblePA/Material/MaterialInstances/PlayerMaterial/PlayerMaterial_Inst_8.PlayerMaterial_Inst_8"))))

(fn IsAttacking
  (bind _mesh (Variables|Character|GetMesh))
  (bind _returnvalue (Components|SkeletalMesh|GetAnimInstance _mesh))
  (return (or (Animation|Montage|MontageIsPlaying _returnvalue "/Game/PartyMonsterRumblePA/Animation/AnimMontage_PlayerAtk_1.AnimMontage_PlayerAtk_1") (Animation|Montage|MontageIsPlaying _returnvalue "/Game/PartyMonsterRumblePA/Animation/AnimMontage_PlayerAtk_2.AnimMontage_PlayerAtk_2"))))

(fn CheckWinCondition
  (if (Variables|Default|GetIsTraitor)
    (bind _traitor_count (CallFunction|TraitorCountDecrease))
    (if (== _traitor_count 0)
      (Development|PrintString "The Innocent Win!")
      (bind _returnvalue (UserInterface|CreateWidget "/Game/UI/MainMenu/WinMessage_UI.WinMessage_UI_C" (Game|GetPlayerController 0)))
      (Variables|/Game/UI/MainMenu/WinMessage_UI.WinMessage_UI_C|SetWinMessageText _returnvalue "The Innocent Wins!")
      (UserInterface|Viewport|AddtoViewport _returnvalue 0))
    (else
      (bind _innocent_count (CallFunction|InnocentCountDecrease))
      (if (== _innocent_count 0)
        (Development|PrintString "The Traitors Win!")
        (bind _returnvalue_2 (UserInterface|CreateWidget "/Game/UI/MainMenu/WinMessage_UI.WinMessage_UI_C" (Game|GetPlayerController 0)))
        (Variables|/Game/UI/MainMenu/WinMessage_UI.WinMessage_UI_C|SetWinMessageText _returnvalue_2 "The Traitor Wins!")
        (UserInterface|Viewport|AddtoViewport _returnvalue_2 0)))))

(fn UpdateHealthUI
  (Variables|/Game/UI/HealthUI.HealthUI_C|SetHealth (Variables|Default|GetHealth%20Widget%20REF) (/ (Variables|Default|GetPlayer%20Health) 1e+02)))

(fn HoldBomb
  (if (Utilities|IsValid (Variables|Default|GetPick%20Up%20Bomb%20REF))
    (Physics|Components|PhysicsHandle|SetTargetLocation (Variables|Default|GetPhysicsHandle) (Transformation|GetWorldLocation (Variables|Default|GetGrab%20Location)))
    (else
      (Variables|Default|SetHas%20Bomb false)
      (Class|KismetSystemLibrary|PauseTimer 0 "Hold Bomb")
      (Development|PrintString "Lost Bomb, Funtion Paused"))))

(fn PickUpBomb
  (bind _mesh (Variables|Character|GetMesh))
  (bind _outhit (Collision|SphereTraceByChannel (Transformation|GetSocketLocation _mesh "Lowerjaw_l") (Transformation|GetSocketLocation _mesh "Lowerjaw_r") 5e+01 "TraceTypeQuery1" false 0 "ForDuration"))
  (if (Utilities|Enum|Equal(Enum) (Utilities|GetClassDisplayName (Utilities|GetClass (.hitactor _outhit))) "BP_Bomb_C")
    (Variables|Default|SetHas%20Bomb true)
    (bind _output_get (Variables|Default|SetPick%20Up%20Bomb%20REF (.hitcomponent _outhit)))
    (Class|PhysicsHandleComponent|GrabComponentatLocation (Variables|Default|GetPhysicsHandle) _output_get "None" (.location _outhit))
    (Utilities|Time|SetTimerbyFunctionName 0 "Hold Bomb" 0.033 true)
    (Collision|SetCollisionResponsetoChannel (Variables|Default|GetPick%20Up%20Bomb%20REF) "ECC_Pawn" "ECR_Overlap")))