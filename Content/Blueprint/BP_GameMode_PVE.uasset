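; Game mode for a local multiplayer hidden-traitor game with item pickups.
; BeginPlay reads the player count from the GameInstance, spawns and possesses players with randomized meshes, assigns random traitors, and shows a fixed camera and tutorial.
; StartGameSequence runs looping timers spawning bombs, gloves, detectors and speed items at tagged points under a growing cap, raised sharply by a delayed chaos mode.
; Helpers rumble traitors' controllers and spawn player ghosts.
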(event Custom|Spawn%20Bomb%20Continuely
  (Utilities|FlowControl|Delay (Math|Random|RandomFloatinRange 0.0 3.0))
  (CallFunction|SpawnBomb))

(event Custom|Spawn%20Attack%20Item%20Continuely
  (Utilities|FlowControl|Delay (Math|Random|RandomFloatinRange 0.0 2.0))
  (CallFunction|SpawnAttackItem))

(event Custom|Spawn%20Detector%20Item%20Continuely
  (Utilities|FlowControl|Delay (Math|Random|RandomFloatinRange 0.0 2.0))
  (CallFunction|SpawnDetectorItem))

(event Custom|Spawn%20Bomb%20Everywhere
  (if (Math|Boolean|ANDBoolean (< (Variables|Default|GetSpawnedItemCount) (Variables|Default|GetMaxSpawnedItemCount)) (Variables|Default|GetcanBePaused) (== (Variables|Default|GetTraitor%20Count) 1) (== (Variables|Default|GetInnocent%20Count) 1))
    (for _array_element (Variables|Default|GetSpawn%20Point%20Cache%20Reference)
      (Game|SpawnActorfromClass "/Game/Blueprint/BP_KillBomb.BP_KillBomb_C" (Math|Transform|MakeTransform (Transformation|GetActorLocation _array_element) (Math|Random|RandomRotator false) "8.000000,8.000000,8.000000") "Undefined" _array_element 0)
      (Math|Integer|IncrementInt (Variables|Default|GetSpawnedItemCount)))))

(event Custom|Spawn%20Speed%20Item%20Continuely
  (Utilities|FlowControl|Delay (Math|Random|RandomFloatinRange 0.0 2.0))
  (CallFunction|SpawnSpeedItem))

(event EventBeginPlay
  (Variables|Default|SetcanBePaused true)
  (CallFunction|UpdatePlayerCount)
  (Utilities|FlowControl|Sequence
    (:then_0
      (CallFunction|SetInnocentandTraitorCount)
      (CallFunction|SpawnPlayers)
      (CallFunction|RandomizePlayerParts)
      (CallFunction|AssignTraitors)
      (CallFunction|FindCameraActor))
    (:then_1
      (Game|Player|SetViewTargetwithBlend (Game|GetPlayerController 0) (Variables|Default|GetMainCamera) 0.0 "VTBlend_Linear" 0.0 false)
      (bind _returnvalue (UserInterface|CreateWidget "/Game/UI/Tutorial/TutorialUI.TutorialUI_C"))
      (UserInterface|Viewport|AddtoViewport _returnvalue 0)
      (Development|PrintString (Utilities|String|Append (Utilities|String|ToString(Integer) (Variables|Default|GetTraitor%20Count)) "Traitors"))
      (Development|PrintString (Utilities|String|Append (Utilities|String|ToString(Integer) (Variables|Default|GetInnocent%20Count)) "Innocents")))))

(fn ConstructionScript)

(fn SpawnPlayers
  (bind _max_player_count (Variables|Default|GetMax%20Player%20Count))
  (bind _returnvalue (- _max_player_count 1))
  ;[1 1 1] Create Player 1, 2, 3
  (for _index (range 1 _returnvalue)
    (Class|GameplayStatics|CreatePlayer _index))
  ;[1 1 1] Spawn and Posses Player Character 0, 1, 2, 3
  (for _index_2 (range 0 _returnvalue)
    (bind _returnvalue_2 (Game|SpawnActorfromClass "/Game/Blueprint/BP_Player.BP_Player_C" (Math|Transform|MakeTransform "0, 0,2000.000000") "Undefined" 0 _index_2 1.0 0))
    (Pawn|Possess (Game|GetPlayerController _index_2) _returnvalue_2)
    (Utilities|Array|AddUnique (Variables|Default|GetPlayers) _returnvalue_2)))

(fn SetInnocentandTraitorCount
  (switch int (Variables|Default|GetMax%20Player%20Count)
    (:4
      (Variables|Default|SetTraitor%20Count 1))
    (:5
      (Variables|Default|SetTraitor%20Count 2))
    (:6
      (Variables|Default|SetTraitor%20Count 2))
    (:7
      (Variables|Default|SetTraitor%20Count 3))
    (:8
      (Variables|Default|SetTraitor%20Count 3)))
  (Variables|Default|SetInnocent%20Count (- (Variables|Default|GetMax%20Player%20Count) (Variables|Default|GetTraitor%20Count))))

(fn AssignPlayerIdentity(4Players)
  (bind _output_get (Variables|Default|SetTraitor1%20Player%20Int (Math|Random|RandomIntegerinRange 0 (- (Variables|Default|GetMax%20Player%20Count) 1))))
  (for _array_element (Variables|Default|GetPlayers)
    (if (== (Variables|/Game/Blueprint/BP_Player.BP_Player_C|GetplayerInt _array_element) _output_get)
      (Variables|/Game/Blueprint/BP_Player.BP_Player_C|SetIsTraitor _array_element true)
      (Development|PrintString (Utilities|String|Append "Player " (Utilities|String|ToString(Integer) (+ (Variables|/Game/Blueprint/BP_Player.BP_Player_C|GetplayerInt _array_element) 1)) " is a traitor"))
      (else
        (Variables|/Game/Blueprint/BP_Player.BP_Player_C|SetIsTraitor _array_element false)
        (Development|PrintString (Utilities|String|Append "Player " (Utilities|String|ToString(Integer) (+ (Variables|/Game/Blueprint/BP_Player.BP_Player_C|GetplayerInt _array_element) 1)) " is not a traitor"))))))

(fn FindCameraActor
  (bind _returnvalue (Actor|GetActorOfClass "/Game/Blueprint/BP_FixedCamera.BP_FixedCamera_C"))
  (Variables|Default|SetMainCamera _returnvalue))

(fn AssignPlayerIdentity(5-6Players)
  (CallFunction|Generate2TraitorIndex)
  ;[1 1 1] Compare Player Inedx with the 2 Traitor Index
  (for _array_element (Variables|Default|GetPlayers)
    (if (or (== (Variables|/Game/Blueprint/BP_Player.BP_Player_C|GetplayerInt _array_element) (Variables|Default|GetTraitor1%20Player%20Int)) (== (Variables|/Game/Blueprint/BP_Player.BP_Player_C|GetplayerInt _array_element) (Variables|Default|GetTraitor2%20Player%20Int)))
      (Variables|/Game/Blueprint/BP_Player.BP_Player_C|SetIsTraitor _array_element true)
      ;[1 1 1] Debug Text
      (Development|PrintString (Utilities|String|Append "Player " (Utilities|String|ToString(Integer) (+ (Variables|/Game/Blueprint/BP_Player.BP_Player_C|GetplayerInt _array_element) 1)) " is a traitor") true true "(R=0.000000,G=0.660000,B=1.000000,A=1.000000)" 2.2e+02)
      (else
        (Variables|/Game/Blueprint/BP_Player.BP_Player_C|SetIsTraitor _array_element false)
        (Development|PrintString (Utilities|String|Append "Player " (Utilities|String|ToString(Integer) (+ (Variables|/Game/Blueprint/BP_Player.BP_Player_C|GetplayerInt _array_element) 1)) " is not a traitor") true true "(R=0.000000,G=0.660000,B=1.000000,A=1.000000)" 2.2e+02)))))

(fn AssignPlayerIdentity(7-8Players)
  (CallFunction|Generate3TraitorIndex)
  ;[1 1 1] Compare Player Index with the 3 Traitor Index
  (for _array_element (Variables|Default|GetPlayers)
    (if (Math|Boolean|ORBoolean (== (Variables|/Game/Blueprint/BP_Player.BP_Player_C|GetplayerInt _array_element) (Variables|Default|GetTraitor1%20Player%20Int)) (== (Variables|/Game/Blueprint/BP_Player.BP_Player_C|GetplayerInt _array_element) (Variables|Default|GetTraitor2%20Player%20Int)) (== (Variables|/Game/Blueprint/BP_Player.BP_Player_C|GetplayerInt _array_element) (Variables|Default|GetTraitor3%20Player%20Int)))
      (Variables|/Game/Blueprint/BP_Player.BP_Player_C|SetIsTraitor _array_element true)
      ;[1 1 1] Debug Text
      (Development|PrintString (Utilities|String|Append "Player " (Utilities|String|ToString(Integer) (+ (Variables|/Game/Blueprint/BP_Player.BP_Player_C|GetplayerInt _array_element) 1)) " is a traitor") true true "(R=0.000000,G=0.660000,B=1.000000,A=1.000000)" 2.2e+02)
      (else
        (Variables|/Game/Blueprint/BP_Player.BP_Player_C|SetIsTraitor _array_element false)
        (Development|PrintString (Utilities|String|Append "Player " (Utilities|String|ToString(Integer) (+ (Variables|/Game/Blueprint/BP_Player.BP_Player_C|GetplayerInt _array_element) 1)) " is not a traitor") true true "(R=0.000000,G=0.660000,B=1.000000,A=1.000000)" 2.2e+02)))))

(fn GenerateARandomNumber
  (return (Math|Random|RandomIntegerinRange 0 (- (Variables|Default|GetMax%20Player%20Count) 1))))

(fn Generate2TraitorIndex
  (bind _output_get (Variables|Default|SetTraitor1%20Player%20Int (CallFunction|GenerateARandomNumber)))
  (bind _output_get_2 (Variables|Default|SetTraitor2%20Player%20Int (CallFunction|GenerateARandomNumber) :!label _label))
  (if (== _output_get_2 _output_get)
    (goto _label)))

(fn Generate3TraitorIndex
  ;[1 1 1] Generate the 1st Random Number
  (bind _output_get (Variables|Default|SetTraitor1%20Player%20Int (CallFunction|GenerateARandomNumber)))
  ;[1 1 1] Loop Until Generate the 2nd Unique Random Number
  (bind _output_get_2 (Variables|Default|SetTraitor2%20Player%20Int (CallFunction|GenerateARandomNumber) :!label _label))
  (if (== _output_get_2 _output_get)
    (goto _label)
    (else
      ;[1 1 1] Loop Until Generate the 3rd Unique Random Number
      (bind _output_get_3 (Variables|Default|SetTraitor3%20Player%20Int (CallFunction|GenerateARandomNumber) :!label _label_2))
      (if (or (== _output_get_3 (Variables|Default|GetTraitor2%20Player%20Int)) (== _output_get_3 (Variables|Default|GetTraitor1%20Player%20Int)))
        (goto _label_2)))))

(fn UpdatePlayerCount
  ;[1 1 1] Get Max Player Count from GameInstance
  (bind _asbp_game_instance (Utilities|Casting|CastToBP_GameInstance (Game|GetGameInstance)))
  (Variables|Default|SetMax%20Player%20Count (Variables|/Game/UI/BP_GameInstance.BP_GameInstance_C|GetPlayerCount _asbp_game_instance)))

(fn AssignTraitors
  (switch int (Variables|Default|GetTraitor%20Count)
    (:1
      (CallFunction|AssignPlayerIdentity(4Players)))
    (:2
      (CallFunction|AssignPlayerIdentity(5-6Players)))
    (:3
      (CallFunction|AssignPlayerIdentity(7-8Players)))))

(fn GetRandomSpawnPoint
  (CallFunction|GetBombSpawnPoints)
  (CallFunction|GetGloveSpawnPoints)
  (CallFunction|GetRadarSpawnPoints)
  (CallFunction|GetSpeedSpawnPoints))

(fn StartGameSequence
  (Input|SetInputModeGameOnly (Game|GetPlayerController 0))
  (CallFunction|GetRandomSpawnPoint)
  (Utilities|Time|SetTimerbyEvent (EventDispatchers|CreateEvent :!event Custom|Spawn%20Bomb%20Continuely) (Variables|Default|GetBomb%20Item%20Spawn%20Frequency) true)
  (Utilities|Time|SetTimerbyEvent (EventDispatchers|CreateEvent :!event Custom|Spawn%20Detector%20Item%20Continuely) (Variables|Default|GetDetector%20Item%20Spawn%20Frequency) true)
  (Utilities|Time|SetTimerbyEvent (EventDispatchers|CreateEvent :!event Custom|Spawn%20Attack%20Item%20Continuely) (Variables|Default|GetAttack%20Item%20Spawn%20Frequency) true)
  (Utilities|Time|SetTimerbyEvent (EventDispatchers|CreateEvent :!event Custom|Spawn%20Speed%20Item%20Continuely) (Variables|Default|GetSpeed%20Item%20Spawn%20Frequency) true)
  (Utilities|Time|SetTimerbyFunctionName 0 "Increase max item count" (Variables|Default|GetIncrease%20Item%20Spawn%20Count%20Frequency) true)
  (Utilities|Time|SetTimerbyFunctionName 0 "Start Chaos Mode" (Variables|Default|GetChaos%20Mode%20Timer))
  (Default|CallTutorialEnded)
  (CallFunction|SpawnBomb))

(fn AllTraitorControllerStartRumble
  (for (_array_element _array_index) (Variables|Default|GetPlayers)
    (if (Variables|/Game/Blueprint/BP_Player.BP_Player_C|GetIsTraitor _array_element)
      (Game|Feedback|ClientPlayForceFeedback (Game|GetPlayerController _array_index) "/Game/Assets/vibration.vibration" "None" true false false))))

(fn AllTraitorControllerStopRumble
  (for (_array_element _array_index) (Variables|Default|GetPlayers)
    (if (Variables|/Game/Blueprint/BP_Player.BP_Player_C|GetIsTraitor _array_element)
      (Game|Feedback|ClientStopForceFeedback (Game|GetPlayerController _array_index) "/Game/Assets/vibration.vibration" "None"))))

(fn IncreaseMaxItemCount
  (bind _maxspawneditemcount (Variables|Default|GetMaxSpawnedItemCount))
  (if (<= _maxspawneditemcount 10)
    (bind _result (Math|Integer|IncrementInt _maxspawneditemcount)
      (:%20%20
        (Development|PrintString (Utilities|String|Append "Max Spawn Item Count increaded to " (Utilities|String|ToString(Integer) _result)) true true "(R=0.000000,G=0.660000,B=1.000000,A=1.000000)" 3e+01)))))

(fn RandomizePlayerParts
  (Variables|Default|SetBody%20Mesh%20Array (Utilities|Array|MakeArray "/Game/PartyMonsterRumblePA/Mesh/ModularPart/Body01_SK.Body01_SK" "/Game/PartyMonsterRumblePA/Mesh/ModularPart/Body01_SK.Body01_SK" "/Game/PartyMonsterRumblePA/Mesh/ModularPart/Body03_SK.Body03_SK" "/Game/PartyMonsterRumblePA/Mesh/ModularPart/Body04_SK.Body04_SK" "/Game/PartyMonsterRumblePA/Mesh/ModularPart/Body05_SK.Body05_SK" "/Game/PartyMonsterRumblePA/Mesh/ModularPart/Body06_SK.Body06_SK"))
  (Variables|Default|SetBodyparts%20Mesh%20Array (Utilities|Array|MakeArray "/Game/PartyMonsterRumblePA/Mesh/ModularPart/Bodypart01_SK.Bodypart01_SK" "/Game/PartyMonsterRumblePA/Mesh/ModularPart/Bodypart02_SK.Bodypart02_SK" "/Game/PartyMonsterRumblePA/Mesh/ModularPart/Bodypart03_SK.Bodypart03_SK" "/Game/PartyMonsterRumblePA/Mesh/ModularPart/Bodypart04_SK.Bodypart04_SK" "/Game/PartyMonsterRumblePA/Mesh/ModularPart/Bodypart05_SK.Bodypart05_SK" "/Game/PartyMonsterRumblePA/Mesh/ModularPart/Bodypart06_SK.Bodypart06_SK" "/Game/PartyMonsterRumblePA/Mesh/ModularPart/Bodypart07_SK.Bodypart07_SK" "/Game/PartyMonsterRumblePA/Mesh/ModularPart/Bodypart08_SK.Bodypart08_SK" "/Game/PartyMonsterRumblePA/Mesh/ModularPart/Bodypart09_SK.Bodypart09_SK" "/Game/PartyMonsterRumblePA/Mesh/ModularPart/Bodypart10_SK.Bodypart10_SK" 0))
  (Variables|Default|SetEye%20Mesh%20Array (Utilities|Array|MakeArray "/Game/PartyMonsterRumblePA/Mesh/ModularPart/Eye01_SK.Eye01_SK" "/Game/PartyMonsterRumblePA/Mesh/ModularPart/Eye02_SK.Eye02_SK" "/Game/PartyMonsterRumblePA/Mesh/ModularPart/Eye03_SK.Eye03_SK" "/Game/PartyMonsterRumblePA/Mesh/ModularPart/Eye04_SK.Eye04_SK" "/Game/PartyMonsterRumblePA/Mesh/ModularPart/Eye05_SK.Eye05_SK" "/Game/PartyMonsterRumblePA/Mesh/ModularPart/Eye06_SK.Eye06_SK" "/Game/PartyMonsterRumblePA/Mesh/ModularPart/Eye07_SK.Eye07_SK" "/Game/PartyMonsterRumblePA/Mesh/ModularPart/Eye08_SK.Eye08_SK" "/Game/PartyMonsterRumblePA/Mesh/ModularPart/Eye09_SK.Eye09_SK" "/Game/PartyMonsterRumblePA/Mesh/ModularPart/Eye10_SK.Eye10_SK" "/Game/PartyMonsterRumblePA/Mesh/ModularPart/Eye11_SK.Eye11_SK" "/Game/PartyMonsterRumblePA/Mesh/ModularPart/Eye12_SK.Eye12_SK" "/Game/PartyMonsterRumblePA/Mesh/ModularPart/Eye13_SK.Eye13_SK" "/Game/PartyMonsterRumblePA/Mesh/ModularPart/Eye14_SK.Eye14_SK" "/Game/PartyMonsterRumblePA/Mesh/ModularPart/Eye15_SK.Eye15_SK"))
  (Variables|Default|SetMouth%20Mesh%20Array (Utilities|Array|MakeArray "/Game/PartyMonsterRumblePA/Mesh/ModularPart/Mouth01_SK.Mouth01_SK" "/Game/PartyMonsterRumblePA/Mesh/ModularPart/Mouth02_SK.Mouth02_SK" "/Game/PartyMonsterRumblePA/Mesh/ModularPart/Mouth03_SK.Mouth03_SK" "/Game/PartyMonsterRumblePA/Mesh/ModularPart/Mouth04_SK.Mouth04_SK" "/Game/PartyMonsterRumblePA/Mesh/ModularPart/Mouth05_SK.Mouth05_SK" "/Game/PartyMonsterRumblePA/Mesh/ModularPart/Mouth06_SK.Mouth06_SK" "/Game/PartyMonsterRumblePA/Mesh/ModularPart/Mouth07_SK.Mouth07_SK" "/Game/PartyMonsterRumblePA/Mesh/ModularPart/Mouth08_SK.Mouth08_SK" "/Game/PartyMonsterRumblePA/Mesh/ModularPart/Mouth09_SK.Mouth09_SK" "/Game/PartyMonsterRumblePA/Mesh/ModularPart/Mouth15_SK.Mouth15_SK" 0))
  (Variables|Default|SetTail%20Mesh%20Array (Utilities|Array|MakeArray "/Game/PartyMonsterRumblePA/Mesh/ModularPart/Tail01_SK.Tail01_SK" "/Game/PartyMonsterRumblePA/Mesh/ModularPart/Tail02_SK.Tail02_SK" "/Game/PartyMonsterRumblePA/Mesh/ModularPart/Tail03_SK.Tail03_SK" "/Game/PartyMonsterRumblePA/Mesh/ModularPart/Tail04_SK.Tail04_SK" "/Game/PartyMonsterRumblePA/Mesh/ModularPart/Tail05_SK.Tail05_SK" "/Game/PartyMonsterRumblePA/Mesh/ModularPart/Tail06_SK.Tail06_SK" "/Game/PartyMonsterRumblePA/Mesh/ModularPart/Tail07_SK.Tail07_SK" "/Game/PartyMonsterRumblePA/Mesh/ModularPart/Tail08_SK.Tail08_SK" 0))
  (Variables|Default|SetHeadpart%20Mesh%20Array (Utilities|Array|MakeArray "/Game/PartyMonsterRumblePA/Mesh/ModularPart/Grass15_SK.Grass15_SK" "/Game/PartyMonsterRumblePA/Mesh/ModularPart/Hair06_SK.Hair06_SK" "/Game/PartyMonsterRumblePA/Mesh/ModularPart/Hair07_SK.Hair07_SK" "/Game/PartyMonsterRumblePA/Mesh/ModularPart/Hair08_SK.Hair08_SK" "/Game/PartyMonsterRumblePA/Mesh/ModularPart/Hair09_SK.Hair09_SK" "/Game/PartyMonsterRumblePA/Mesh/ModularPart/Horn10_SK.Horn10_SK" "/Game/PartyMonsterRumblePA/Mesh/ModularPart/Horn11_SK.Horn11_SK" "/Game/PartyMonsterRumblePA/Mesh/ModularPart/Horn12_SK.Horn12_SK" "/Game/PartyMonsterRumblePA/Mesh/ModularPart/Horn13_SK.Horn13_SK" "/Game/PartyMonsterRumblePA/Mesh/ModularPart/Hat16_SK.Hat16_SK" "/Game/PartyMonsterRumblePA/Mesh/ModularPart/Hat17_SK.Hat17_SK" "/Game/PartyMonsterRumblePA/Mesh/ModularPart/Hat18_SK.Hat18_SK" "/Game/PartyMonsterRumblePA/Mesh/ModularPart/Hat19_SK.Hat19_SK" "/Game/PartyMonsterRumblePA/Mesh/ModularPart/Hat20_SK.Hat20_SK" "/Game/PartyMonsterRumblePA/Mesh/ModularPart/Hat21_SK.Hat21_SK" "/Game/PartyMonsterRumblePA/Mesh/ModularPart/Ear01_SK.Ear01_SK" "/Game/PartyMonsterRumblePA/Mesh/ModularPart/Ear02_SK.Ear02_SK" "/Game/PartyMonsterRumblePA/Mesh/ModularPart/Ear03_SK.Ear03_SK" "/Game/PartyMonsterRumblePA/Mesh/ModularPart/Ear04_SK.Ear04_SK" "/Game/PartyMonsterRumblePA/Mesh/ModularPart/Ear05_SK.Ear05_SK" 0))
  (for _array_element (Variables|Default|GetPlayers)
    (Class|SkinnedMeshComponent|SetSkeletalMesh (Variables|/Script/Engine.Character|GetMesh _array_element) (.OutItem (Utilities|Array|Random (Variables|Default|GetBody%20Mesh%20Array))) true)
    (Class|SkinnedMeshComponent|SetSkeletalMesh (Variables|/Game/Blueprint/BP_Player.BP_Player_C|GetBodyparts _array_element) (.OutItem (Utilities|Array|Random (Variables|Default|GetBodyparts%20Mesh%20Array))) true)
    (Class|SkinnedMeshComponent|SetSkeletalMesh (Variables|/Game/Blueprint/BP_Player.BP_Player_C|GetEyes _array_element) (.OutItem (Utilities|Array|Random (Variables|Default|GetEye%20Mesh%20Array))) true)
    (Class|SkinnedMeshComponent|SetSkeletalMesh (Variables|/Game/Blueprint/BP_Player.BP_Player_C|GetMouths _array_element) (.OutItem (Utilities|Array|Random (Variables|Default|GetMouth%20Mesh%20Array))) true)
    (Class|SkinnedMeshComponent|SetSkeletalMesh (Variables|/Game/Blueprint/BP_Player.BP_Player_C|GetHeadparts _array_element) (.OutItem (Utilities|Array|Random (Variables|Default|GetHeadpart%20Mesh%20Array))) true)
    (Class|SkinnedMeshComponent|SetSkeletalMesh (Variables|/Game/Blueprint/BP_Player.BP_Player_C|GetTails _array_element) (.OutItem (Utilities|Array|Random (Variables|Default|GetTail%20Mesh%20Array))) true))
  (return))

(fn PlayLevelMusic
  (bind _returnvalue (Audio|CreateSound2D "/Game/Assets/Sounds/BGM/in_game_bgm_Cue.in_game_bgm_Cue" 1.0 1.0 0.0 0))
  (bind _output_get (Variables|Default|SetIn%20Game%20Music _returnvalue))
  (Audio|Components|Audio|Play _output_get 0.0))

(fn StartChaosMode
  (Variables|Default|SetMaxSpawnedItemCount 50)
  (Utilities|Time|SetTimerbyEvent (EventDispatchers|CreateEvent :!event Custom|Spawn%20Bomb%20Everywhere) (Variables|Default|GetChaos%20Mode%20Frequency) true)
  (Development|PrintString "Chaos Mode Started"))

(fn SpawnBomb
  (bind _bomb_item_spawn_points (Variables|Default|GetBomb%20Item%20Spawn%20Points))
  (bind _outitem (Utilities|Array|Random _bomb_item_spawn_points))
  (bind _returnvalue (Transformation|GetActorTransform _outitem))
  (if (and (< (Variables|Default|GetSpawnedItemCount) (Variables|Default|GetMaxSpawnedItemCount)) (Variables|Default|GetcanBePaused))
    (Utilities|IsValid _outitem
      (:Is%20Valid
        (Game|SpawnActorfromClass "/Game/Blueprint/BP_KillBomb.BP_KillBomb_C" (Math|Transform|MakeTransform (.location _returnvalue) (Math|Random|RandomRotator false) "8.000000,8.000000,8.000000") "Undefined" 0 0)
        (Math|Integer|IncrementInt (Variables|Default|GetSpawnedItemCount)
          (:%20%20
            (Development|PrintString "Bomb Spawned")
            (Audio|PlaySoundatLocation "/Game/Assets/Sounds/Item_Drop.Item_Drop" (.location _returnvalue) "0, 0, 0" 0.5 1.0 0.0 0 0 0)))))))

(fn SpawnAttackItem
  (bind _glove_spawn_points (Variables|Default|GetGlove%20Spawn%20Points))
  (bind _outitem (Utilities|Array|Random _glove_spawn_points))
  (bind _returnvalue (Transformation|GetActorTransform _outitem))
  (if (and (< (Variables|Default|GetSpawnedItemCount) (Variables|Default|GetMaxSpawnedItemCount)) (Variables|Default|GetcanBePaused))
    (Utilities|IsValid _outitem
      (:Is%20Valid
        (Game|SpawnActorfromClass "/Game/Blueprint/BP_AttackItem.BP_AttackItem_C" (Math|Transform|MakeTransform (.location _returnvalue) (Math|Random|RandomRotator false) "0.150000,0.150000,0.150000") "Undefined" 0 0)
        (Math|Integer|IncrementInt (Variables|Default|GetSpawnedItemCount)
          (:%20%20
            (Development|PrintString "Glove Spawned")
            (Audio|PlaySoundatLocation "/Game/Assets/Sounds/Item_Drop.Item_Drop" (.location _returnvalue) "0, 0, 0" 0.5 1.0 0.0 0 0 0)))))))

(fn SpawnSpeedItem
  (bind _speed_item_spawn_points (Variables|Default|GetSpeed%20Item%20Spawn%20Points))
  (bind _outitem (Utilities|Array|Random _speed_item_spawn_points))
  (bind _returnvalue (Transformation|GetActorTransform _outitem))
  (if (and (< (Variables|Default|GetSpawnedItemCount) (Variables|Default|GetMaxSpawnedItemCount)) (Variables|Default|GetcanBePaused))
    (Utilities|IsValid _outitem
      (:Is%20Valid
        (Game|SpawnActorfromClass "/Game/Blueprint/BP_SpeedItem.BP_SpeedItem_C" (Math|Transform|MakeTransform (.location _returnvalue) "0, 0, 0" "2.000000,2.000000,2.000000") "Undefined" 0 0)
        (Math|Integer|IncrementInt (Variables|Default|GetSpawnedItemCount)
          (:%20%20
            (Development|PrintString "Glove Spawned")
            (Audio|PlaySoundatLocation "/Game/Assets/Sounds/Item_Drop.Item_Drop" (.location _returnvalue) "0, 0, 0" 0.5 1.0 0.0 0 0 0)))))))

(fn SpawnDetectorItem
  (bind _radar_spawn_points (Variables|Default|GetRadar%20Spawn%20Points))
  (bind _outitem (Utilities|Array|Random _radar_spawn_points))
  (bind _returnvalue (Transformation|GetActorTransform _outitem))
  (if (and (< (Variables|Default|GetSpawnedItemCount) (Variables|Default|GetMaxSpawnedItemCount)) (Variables|Default|GetcanBePaused))
    (Utilities|IsValid _outitem
      (:Is%20Valid
        (Game|SpawnActorfromClass "/Game/Blueprint/BP_TraitorDetector.BP_TraitorDetector_C" (Math|Transform|MakeTransform (.location _returnvalue) (Math|Random|RandomRotator false) "0.200000,0.200000,0.200000") "Undefined" 0 0)
        (Math|Integer|IncrementInt (Variables|Default|GetSpawnedItemCount)
          (:%20%20
            (Development|PrintString "Item Spawned")
            (Audio|PlaySoundatLocation "/Game/Assets/Sounds/Item_Drop.Item_Drop" (.location _returnvalue) "0, 0, 0" 0.5 1.0 0.0 0 0 0)))))))

(fn GetBombSpawnPoints
  (bind _outactors (Actor|GetAllActorsOfClasswithTag "/Game/Blueprint/BP_ItemSpawnPoint.BP_ItemSpawnPoint_C" "Bomb"))
  (Variables|Default|SetBomb%20Item%20Spawn%20Points _outactors))

(fn GetGloveSpawnPoints
  (bind _outactors (Actor|GetAllActorsOfClasswithTag "/Game/Blueprint/BP_ItemSpawnPoint.BP_ItemSpawnPoint_C" "Glove"))
  (Variables|Default|SetGlove%20Spawn%20Points _outactors))

(fn GetRadarSpawnPoints
  (bind _outactors (Actor|GetAllActorsOfClasswithTag "/Game/Blueprint/BP_ItemSpawnPoint.BP_ItemSpawnPoint_C" "Radar"))
  (Variables|Default|SetRadar%20Spawn%20Points _outactors))

(fn GetSpeedSpawnPoints
  (bind _outactors (Actor|GetAllActorsOfClasswithTag "/Game/Blueprint/BP_ItemSpawnPoint.BP_ItemSpawnPoint_C" "Speed"))
  (Variables|Default|SetSpeed%20Item%20Spawn%20Points _outactors))

(fn SpawnGhost
  (params (Spawn%20Transform%20Location :type Vector) (Player%20Int :type Integer) (isTraitor :type Boolean) (Color :type Linear%20Color%20Structure))
  (bind _returnvalue (Game|SpawnActorfromClass "/Game/Blueprint/BP_Ghost.BP_Ghost_C" (Math|Transform|MakeTransform Spawn%20Transform%20Location "0, 0, 0" "1,1,1") "AlwaysSpawn" 0 Player%20Int isTraitor Color 0))
  (Utilities|Array|AddUnique (Variables|Default|GetPlayer%20Ghost%20Array) _returnvalue))