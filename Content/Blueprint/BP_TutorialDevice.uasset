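; Tutorial device that sets an overlapping player's traitor identity to match its own Traitor flag.
; On overlap with its CollisionRange, it updates BP_Player's IsTraitor and identity widget text if they differ; the VFX/SFX function currently only prints a string.
; A Traitor device also starts controller vibration when that player is flagged as overlapping with a traitor.
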(event Custom|Overlap%20Event
  (params (OverlappedComponent :type Primitive%20Component%20Object%20Reference) (OtherActor :type Actor%20Object%20Reference) (OtherComp :type Primitive%20Component%20Object%20Reference) (OtherBodyIndex :type Integer) (bFromSweep :type Boolean) (SweepResult :type Hit%20Result%20Structure%20%28by%20ref%29))
  (bind _outputpin (CallFunction|ChangeOverlappedPlayerIdentity OtherActor))
  (if (Variables|Default|GetbTraitor)
    (CallFunction|CheckifIsOverlapping _outputpin)))

(event EventBeginPlay
  (Collision|BindEventtoOnComponentBeginOverlap (Variables|Default|GetCollision%20Range) (delegate Custom|Overlap%20Event)))

(event Collision|EventActorBeginOverlap
  (params (OtherActor :type Actor%20Object%20Reference)))

(event EventTick
  (params (DeltaSeconds :type Float%20%28single-precision%29)))

(fn ConstructionScript)

(fn PLAYVFXANDSFX
  (params (BP_Player :type BP%20Player%20Object%20Reference))
  (Development|PrintString (Utilities|String|Append (Utilities|GetObjectName BP_Player) " become " (Utilities|String|ToString(Boolean) (Variables|Default|GetbTraitor)))))

(fn ChangeOverlappedPlayerIdentity
  (params (Overlapped%20Actor :type Object%20Object%20Reference))
  (bind _asbp_player (Utilities|Casting|CastToBP_Player Overlapped%20Actor))
  (if (Math|Boolean|Equal(Boolean) (Variables|/Game/Blueprint/BP_Player.BP_Player_C|GetIsTraitor _asbp_player) (Variables|Default|GetbTraitor))
    _
    (else
      (CallFunction|PLAYVFXANDSFX _asbp_player)
      (Variables|/Game/Blueprint/BP_Player.BP_Player_C|SetIsTraitor _asbp_player (Variables|Default|GetbTraitor))
      (bind _asplayer_identity_ui (Utilities|Casting|CastToPlayerIdentityUI (UserInterface|GetUserWidgetObject (Variables|/Game/Blueprint/BP_Player.BP_Player_C|GetPlayer%20Identity%20Widget _asbp_player))))
      (Default|UpdatePlayerIdentityText _asplayer_identity_ui _asbp_player)))
  (return _asbp_player))

(fn CheckifIsOverlapping
  (params (Incoming :type BP%20Player%20Object%20Reference))
  (Utilities|IsValid Incoming
    (:Is%20Valid
      (if (Variables|/Game/Blueprint/BP_Player.BP_Player_C|GetIsOverlappingWithTraitor Incoming)
        (if (Variables|/Game/Blueprint/BP_Player.BP_Player_C|GetIsTraitor Incoming)
          (Default|ControllerStartVibration Incoming))))))