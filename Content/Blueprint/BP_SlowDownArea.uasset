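; BP_SlowDownArea is a grass area that changes the player's movement speed while they are inside it.
; Begin overlap multiplies BP_Player's MoveSpeed by SlowDownMultiplier, and end overlap divides by the same value to undo it.
; Both transitions play a walk-in-grass sound at the player's location.
; PlayGrassVFX is called for every overlapping actor, but is a stub that spawns no effect.
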(event EventBeginPlay)

(event Collision|EventActorBeginOverlap
  (params (OtherActor :type Actor%20Object%20Reference))
  (CallFunction|PlayGrassVFX OtherActor)
  (if (== (Utilities|GetClass OtherActor) "/Game/Blueprint/BP_Player.BP_Player_C")
    (bind _asbp_player (Utilities|Casting|CastToBP_Player OtherActor))
    (Variables|/Game/Blueprint/BP_Player.BP_Player_C|SetmoveSpeed _asbp_player (* (Variables|/Game/Blueprint/BP_Player.BP_Player_C|GetmoveSpeed _asbp_player) (Variables|Default|GetSlowDownMultiplier)))
    (Audio|PlaySoundatLocation "/Game/Assets/Sounds/EnvironmentSFX/Walk_in_grass_SoundCue.Walk_in_grass_SoundCue" (Transformation|GetActorLocation OtherActor) "0, 0, 0" 1.0 1.0 0.0 0 0 0)))

(event EventTick
  (params (DeltaSeconds :type Float%20%28single-precision%29)))

(event Collision|EventActorEndOverlap
  (params (OtherActor :type Actor%20Object%20Reference))
  (CallFunction|PlayGrassVFX OtherActor)
  (if (== (Utilities|GetClass OtherActor) "/Game/Blueprint/BP_Player.BP_Player_C")
    (bind _asbp_player (Utilities|Casting|CastToBP_Player OtherActor))
    (Variables|/Game/Blueprint/BP_Player.BP_Player_C|SetmoveSpeed _asbp_player (/ (Variables|/Game/Blueprint/BP_Player.BP_Player_C|GetmoveSpeed _asbp_player) (Variables|Default|GetSlowDownMultiplier)))
    (Audio|PlaySoundatLocation "/Game/Assets/Sounds/EnvironmentSFX/Walk_in_grass_SoundCue.Walk_in_grass_SoundCue" (Transformation|GetActorLocation OtherActor) "0, 0, 0" 1.0 1.0 0.0 0 0 0)))

(fn ConstructionScript)

(fn PlayGrassVFX
  (params (Incoming%20Actor :type Actor%20Object%20Reference))
  (return Incoming%20Actor))