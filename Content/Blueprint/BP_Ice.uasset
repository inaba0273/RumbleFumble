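; BP_Ice is an ice surface actor that makes BP_Player faster and slippery while inside its Box trigger.
; On begin overlap it scales the player's MoveSpeed by SpeedMultiplier, removes ground friction and lowers walking braking deceleration.
; On end overlap it divides MoveSpeed back and sets friction and braking to hardcoded values rather than saved originals.
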(event OnComponentBeginOverlap(Box)
  (params (OverlappedComponent :type Primitive%20Component%20Object%20Reference) (OtherActor :type Actor%20Object%20Reference) (OtherComp :type Primitive%20Component%20Object%20Reference) (OtherBodyIndex :type Integer) (bFromSweep :type Boolean) (SweepResult :type Hit%20Result%20Structure%20%28by%20ref%29))
  (bind _asbp_player (Utilities|Casting|CastToBP_Player OtherActor))
  (Variables|/Game/Blueprint/BP_Player.BP_Player_C|SetmoveSpeed _asbp_player (* (Variables|/Game/Blueprint/BP_Player.BP_Player_C|GetmoveSpeed _asbp_player) (Variables|Default|GetSpeed%20Multiplier)))
  (Variables|/Script/Engine.CharacterMovementComponent|SetGroundFriction (Variables|/Script/Engine.Character|GetCharacterMovement _asbp_player) 0.0)
  (Variables|/Script/Engine.CharacterMovementComponent|SetBrakingDecelerationWalking (Variables|/Script/Engine.Character|GetCharacterMovement _asbp_player) 2.5e+02))

(event OnComponentEndOverlap(Box)
  (params (OverlappedComponent :type Primitive%20Component%20Object%20Reference) (OtherActor :type Actor%20Object%20Reference) (OtherComp :type Primitive%20Component%20Object%20Reference) (OtherBodyIndex :type Integer))
  (bind _asbp_player (Utilities|Casting|CastToBP_Player OtherActor))
  (Variables|/Game/Blueprint/BP_Player.BP_Player_C|SetmoveSpeed _asbp_player (/ (Variables|/Game/Blueprint/BP_Player.BP_Player_C|GetmoveSpeed _asbp_player) (Variables|Default|GetSpeed%20Multiplier)))
  (Variables|/Script/Engine.CharacterMovementComponent|SetGroundFriction (Variables|/Script/Engine.Character|GetCharacterMovement _asbp_player) 8.0)
  (Variables|/Script/Engine.CharacterMovementComponent|SetBrakingDecelerationWalking (Variables|/Script/Engine.Character|GetCharacterMovement _asbp_player) 2048.0))

(event EventBeginPlay)

(event Collision|EventActorBeginOverlap
  (params (OtherActor :type Actor%20Object%20Reference)))

(event EventTick
  (params (DeltaSeconds :type Float%20%28single-precision%29)))

(fn ConstructionScript)