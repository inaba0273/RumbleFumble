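; A Behavior Tree node that picks an item for an AI-controlled pawn to go after, storing it in the MoveTarget Blackboard key.
; On each AI tick without a valid target, it looks for any BP_AttackItem, then falls back to any BP_TraitorDetector, without comparing distances.
; If neither exists, it clears the key and issues a simple move to the pawn itself.
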(event EventReceiveTickAI
  (params (OwnerController :type AI%20Controller%20Object%20Reference) (ControlledPawn :type Pawn%20Object%20Reference) (DeltaSeconds :type Float%20%28single-precision%29))
  ;[1 1 1] Only has one target at one time
  (Utilities|IsValid (Class|BTFunctionLibrary|GetBlackboardValueasObject (Variables|Default|GetMoveTarget))
    (:Is%20Not%20Valid
      (bind _returnvalue (Actor|GetActorOfClass "/Game/Blueprint/BP_AttackItem.BP_AttackItem_C"))
      (Utilities|IsValid _returnvalue
        (:Is%20Valid
          (Class|BTFunctionLibrary|SetBlackboardValueasObject (Variables|Default|GetMoveTarget) _returnvalue)
          (Development|PrintString "FOUND ITEM"))
        (:Is%20Not%20Valid
          (bind _returnvalue_2 (Actor|GetActorOfClass "/Game/Blueprint/BP_TraitorDetector.BP_TraitorDetector_C"))
          (Utilities|IsValid _returnvalue_2
            (:Is%20Valid
              (Class|BTFunctionLibrary|SetBlackboardValueasObject (Variables|Default|GetMoveTarget) _returnvalue_2)
              (Development|PrintString "FOUND ITEM"))
            (:Is%20Not%20Valid
              (Class|BTFunctionLibrary|SetBlackboardValueasObject (Variables|Default|GetMoveTarget))
              (AI|Navigation|SimpleMovetoActor OwnerController ControlledPawn))))))))