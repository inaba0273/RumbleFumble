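; FindRandomLocation is a behavior tree task that picks a wander destination for an AI-controlled BP_Player and writes it to the MoveToLocation blackboard key.
; Most runs query a random reachable point within Radius of the pawn, falling back to its current location if none is found.
; Occasionally it idles for a short random delay, then sets the current location.
; Every path finishes with success.
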(event EventReceiveExecuteAI
  (params (OwnerController :type AI%20Controller%20Object%20Reference) (ControlledPawn :type Pawn%20Object%20Reference))
  (bind _asbp_player (Utilities|Casting|CastToBP_Player ControlledPawn))
  (bind _radius (Variables|Default|GetRadius))
  (bind _returnvalue (Transformation|GetActorLocation _asbp_player))
  (bind (_randomlocation _returnvalue_2) (AI|Navigation|GetRandomReachablePointinRadius _returnvalue _radius 0 0))
  ;[1 1 1] Idle Or Move
  (if (Math|Random|RandomBoolwithWeight 0.85)
    (if _returnvalue_2
      (AI|BehaviorTree|SetBlackboardValueasVector (Variables|Default|GetMoveToLocation) _randomlocation)
      (else
        (AI|BehaviorTree|SetBlackboardValueasVector (Variables|Default|GetMoveToLocation) _returnvalue :!label _label)))
    (else
      (Utilities|FlowControl|Delay (Math|Random|RandomFloatinRange 2.0 3.0))
      (goto _label)))
  (AI|BehaviorTree|FinishExecute true))