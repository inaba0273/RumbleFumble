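; AI controller for bot players in a traitor-versus-innocents brawl, driving punches, bomb throws and accusation dialogue.
; After the tutorial it runs BT_PlayerAI, feeding it targets and state through blackboard setters.
; Randomized looping timers roll attack intent from Aggressiveness and trigger chatter; innocents also gain Wisdom and Aggressiveness, with Wisdom rolls setting CheatMode.
; The final countdown enables duel mode, forcing attack intent and targeting living players.
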(event Custom|Look%20for%20target
  (Utilities|FlowControl|Delay (Math|Random|RandomFloatinRange 5.0 8.0))
  (CallFunction|RollWisdom))

(event Custom|Increase%20Wisdom
  (Variables|Default|SetWisdom (+ (Variables|Default|GetWisdom) (Variables|Default|GetWisdom%20Delta)))
  (Variables|Default|SetAggressiveness (+ (Variables|Default|GetAggressiveness) (Variables|Default|GetAggressiveness%20Delta))))

(event Custom|Aim%20And%20Attack
  (params (Object :type Object%20Object%20Reference))
  (AI|SetFocus (Variables|Default|GetAttack%20Target))
  (bind _asbp_player (Utilities|Casting|CastToBP_Player Object))
  (Default|Punch _asbp_player)
  (Utilities|FlowControl|Delay 0.3)
  (AI|ClearFocus))

(event Custom|Change%20Attack%20Mode
  (Utilities|FlowControl|Delay (Math|Random|RandomFloatinRange 2.0 6.0))
  (CallFunction|RollWanttoAttack))

(event Custom|Start%20Game
  (Utilities|FlowControl|Delay (Math|Random|RandomFloatinRange 0.0 2.0))
  (AI|RunBehaviorTree "/Game/Blueprint/PlayerAI/BT_PlayerAI.BT_PlayerAI")
  (CallFunction|TriggerInitialDialogue)
  (Utilities|Time|SetTimerbyEvent (delegate Custom|Change%20Attack%20Mode) (Math|Random|RandomFloatinRange 12.0 15.0) true)
  (Utilities|Time|SetTimerbyEvent (delegate Custom|Trigger%20Dialogues) (Math|Random|RandomFloatinRange 1e+01 15.0) true)
  (bind _asbp_player (Utilities|Casting|CastToBP_Player (Pawn|GetControlledPawn)))
  (if (not (Variables|/Game/Blueprint/BP_Player.BP_Player_C|GetIsTraitor _asbp_player))
    (Utilities|Time|SetTimerbyEvent (delegate Custom|Look%20for%20target) 1e+01 true)
    (Utilities|Time|SetTimerbyEvent (delegate Custom|Increase%20Wisdom) (Math|Random|RandomFloatinRange 8.0 11.0) true)))

(event Custom|Trigger%20Dialogues
  (Utilities|FlowControl|Delay (Math|Random|RandomFloatinRange 0.0 12.0))
  (if (Math|Random|RandomBoolwithWeight 0.85)
    (CallFunction|TriggerAccuseDialogue false)))

(event Custom|Pick%20Up%20And%20Throw%20Bomb
  (bind _attack_target (Variables|Default|GetAttack%20Target))
  (AI|Components|Blackboard|SetValueasBool (Variables|Default|GetPlayerAI_Blackboard) (Variables|Default|GetHasBombKeyName) true)
  (AI|SetFocus (Variables|Default|GetObject%20To%20Be%20Picked%20Up))
  (bind _asbp_player (Utilities|Casting|CastToBP_Player (Pawn|GetControlledPawn)))
  (bind _success (Default|PlayerPickUp&ThrowBomb _asbp_player))
  (AI|ClearFocus)
  (if _success
    (Utilities|FlowControl|Delay (Math|Random|RandomFloatinRange 1.0 1.3))
    (Utilities|IsValid _attack_target
      (:Is%20Valid
        (AI|SetFocus _attack_target))
      (:Is%20Not%20Valid
        (Transformation|SetActorRotation _asbp_player (Math|Rotator|MakeRotator 0.0 0.0 (Math|Random|RandomFloat)))))
    (Utilities|FlowControl|Delay 0.2)
    (Default|PlayerPickUp&ThrowBomb _asbp_player)
    (AI|ClearFocus)
    (Utilities|FlowControl|Delay 1.0)
    (CallFunction|RemoveBombTarget)
    (AI|Components|Blackboard|SetValueasBool (Variables|Default|GetPlayerAI_Blackboard) (Variables|Default|GetHasBombKeyName) false)))

(event Custom|Duel%20Mode
  (Development|PrintString "FINAL COUNT DOWN!!!")
  (CallFunction|EnableDuelMode)
  (CallFunction|WanttoAttackMode)
  (bind _outactors (Actor|GetAllActorsOfClass "/Game/Blueprint/BP_Player.BP_Player_C"))
  (for _array_element _outactors
    (if (and (not (Variables|/Game/Blueprint/BP_Player.BP_Player_C|GetDead _array_element)) (not (== _array_element (Pawn|GetControlledPawn))))
      (CallFunction|FindAttackTarget _array_element)
      (Utilities|FlowControl|Delay (Math|Random|RandomFloatinRange 1.0 2.0))
      (CallFunction|TriggerDuelDialogue))))

(event EventBeginPlay
  (CallFunction|CacheGameInstance)
  (CallFunction|SetInitialValue)
  (bind _asbp_game_mode (CallFunction|CacheGameMode))
  (EventDispatchers|BindEventtoTutorialEnded _asbp_game_mode (delegate Custom|Start%20Game))
  (EventDispatchers|BindEventtoFinalCountDown _asbp_game_mode (delegate Custom|Duel%20Mode)))

(fn ConstructionScript)

(fn FindAttackTarget
  (params (Attack%20Target :type BP%20Player%20Object%20Reference))
  (Variables|Default|SetAttack%20Target Attack%20Target)
  (AI|Components|Blackboard|SetValueasObject (Variables|Default|GetPlayerAI_Blackboard) (Variables|Default|GetAttackTargetKeyName) Attack%20Target)
  (Development|PrintString "Attack Target Updated"))

(fn GetTargetPlayerList
  (bind _asbp_player (Utilities|Casting|CastToBP_Player (Pawn|GetControlledPawn)))
  (bind _outactors (Actor|GetAllActorsOfClass "/Game/Blueprint/BP_Player.BP_Player_C"))
  (for _array_element _outactors
    (if (not (Math|Boolean|Equal(Boolean) (Variables|/Game/Blueprint/BP_Player.BP_Player_C|GetIsTraitor _array_element) (Variables|/Game/Blueprint/BP_Player.BP_Player_C|GetIsTraitor _asbp_player)))
      (Utilities|Array|AddUnique (Variables|Default|GetOpponent%20Players) _array_element)))
  (return (Variables|Default|GetOpponent%20Players)))

(fn FindAllOtherActors
  (bind _outactors (Actor|GetAllActorsOfClass "/Game/Blueprint/BP_Player.BP_Player_C"))
  (for _array_element _outactors
    (if (not (== (AI|Components|Blackboard|GetValueasObject (Variables|Default|GetPlayerAI_Blackboard) (Variables|Default|GetSelfActorKeyName)) _array_element))
      (if (not (Variables|/Game/Blueprint/BP_Player.BP_Player_C|GetDead _array_element))
        (Utilities|Array|AddUnique (Variables|Default|GetOther%20Players) _array_element))))
  (return (Variables|Default|GetOther%20Players)))

(fn RemoveDeadTarget
  (if (Variables|/Game/Blueprint/BP_Player.BP_Player_C|GetDead (Variables|Default|GetAttack%20Target))
    (bind _output_get (Variables|Default|SetAttack%20Target 0))
    (AI|Components|Blackboard|SetValueasObject (Variables|Default|GetPlayerAI_Blackboard) (Variables|Default|GetKey%20Name) _output_get)))

(fn WanttoAttackMode
  (bind _output_get (Variables|Default|SetWantToAttack true))
  (AI|Components|Blackboard|SetValueasBool (Variables|Default|GetPlayerAI_Blackboard) (Variables|Default|GetWantToAttackKeyName) _output_get))

(fn DontWanttoAttackMode
  (Variables|Default|SetWantToAttack false)
  (AI|Components|Blackboard|SetValueasBool (Variables|Default|GetPlayerAI_Blackboard) (Variables|Default|GetAttackTargetKeyName) false))

(fn StartDizzy
  (AI|Components|Blackboard|SetValueasBool (Variables|Default|GetPlayerAI_Blackboard) (Variables|Default|GetDizzyKeyName) true))

(fn EndDizzy
  (AI|Components|Blackboard|SetValueasBool (Variables|Default|GetPlayerAI_Blackboard) (Variables|Default|GetDizzyKeyName) false))

(fn SetInitialValue
  (bind _asbp_player (Utilities|Casting|CastToBP_Player (Pawn|GetControlledPawn)))
  (if (Variables|/Game/Blueprint/BP_Player.BP_Player_C|GetIsTraitor _asbp_player)
    (Variables|Default|SetAggressiveness (Math|Random|RandomFloatinRange (Variables|Default|GetTraitor%20Agg%20Min) (Variables|Default|GetTraitor%20Agg%20Max)))
    (else
      (Variables|Default|SetWisdom (Math|Random|RandomFloatinRange (Variables|Default|GetWisdom%20Min) (Variables|Default|GetWisdom%20Max)))
      (Variables|Default|SetAggressiveness (Math|Random|RandomFloatinRange (Variables|Default|GetInnocent%20Agg%20Min) (Variables|Default|GetInnocent%20Agg%20Max)))
      (Variables|Default|SetCheatMode (Math|Random|RandomBoolwithWeight 0.3)))))

(fn RollWanttoAttack
  (if (not (Variables|Default|GetWantToAttack))
    (if (Math|Random|RandomBoolwithWeight (/ (Variables|Default|GetAggressiveness) 1e+02))
      (CallFunction|WanttoAttackMode)
      (Development|PrintString "AI want to attack")
      (else
        (Development|PrintString "AI dont want to attack")))))

(fn RollWisdom
  (Utilities|IsValid (Variables|Default|GetAttack%20Target)
    (:Is%20Not%20Valid
      (bind _output_get (Variables|Default|SetCheatMode (Math|Random|RandomBoolwithWeight (/ (Variables|Default|GetWisdom) 1e+02))))
      (if _output_get
        (Development|PrintString "Cheat Mode On")
        (CallFunction|RemoveAttackTarget)
        (else
          (Development|PrintString "Cheat Mode Off"))))))

(fn RemoveAttackTarget
  (bind _output_get (Variables|Default|SetAttack%20Target 0))
  (AI|Components|Blackboard|SetValueasObject (Variables|Default|GetPlayerAI_Blackboard) (Variables|Default|GetKey%20Name) _output_get)
  (Development|PrintString "Attack Target Removed"))

(fn AIStopMoving
  (AI|Components|Blackboard|SetValueasBool (Variables|Default|GetPlayerAI_Blackboard) (Variables|Default|GetisDeadKey) true))

(fn FindBomb
  (params (Object%20to%20be%20picked%20up :type Actor%20Object%20Reference))
  (Utilities|IsValid (Variables|Default|GetObject%20To%20Be%20Picked%20Up)
    (:Is%20Not%20Valid
      (Variables|Default|SetObject%20To%20Be%20Picked%20Up Object%20to%20be%20picked%20up)
      (AI|Components|Blackboard|SetValueasObject (Variables|Default|GetPlayerAI_Blackboard) (Variables|Default|GetPickUpTargetKeyName) Object%20to%20be%20picked%20up))))

(fn RemoveBombTarget
  (Variables|Default|SetObject%20To%20Be%20Picked%20Up 0)
  (AI|Components|Blackboard|SetValueasObject (Variables|Default|GetPlayerAI_Blackboard) (Variables|Default|GetPickUpTargetKeyName) 0))

(fn EnableGlove
  (AI|Components|Blackboard|SetValueasBool (Variables|Default|GetPlayerAI_Blackboard) (Variables|Default|GetHasGloveKeyName) true))

(fn DisableGlove
  (AI|Components|Blackboard|SetValueasBool (Variables|Default|GetPlayerAI_Blackboard) (Variables|Default|GetHasGloveKeyName) false))

(fn GetDialoguePlayerName
  (bind _attack_target (Variables|Default|GetAttack%20Target))
  (Utilities|IsValid _attack_target
    (:Is%20Valid
      (bind _asbp_game_instance (Utilities|Casting|CastToBP_GameInstance (Game|GetGameInstance)))
      (Variables|Default|SetDialogue%20Target%20Name (Utilities|Array|Get(acopy) (Variables|/Game/UI/BP_GameInstance.BP_GameInstance_C|GetPlayer%20Name%20Array _asbp_game_instance) (Variables|/Game/Blueprint/BP_Player.BP_Player_C|GetplayerInt _attack_target)))
      (return))))

(fn TriggerAccuseDialogue
  (params (Sure :type Boolean))
  (bind _as_bp_game_instance (Variables|Default|GetAs%20BP%20Game%20Instance))
  (bind _attack_target (Variables|Default|GetAttack%20Target))
  (bind _isnamelessmode (Variables|/Game/UI/BP_GameInstance.BP_GameInstance_C|GetisNamelessMode _as_bp_game_instance))
  (Utilities|IsValid _attack_target
    (:Is%20Valid
      (if (not (Variables|/Game/Blueprint/BP_Player.BP_Player_C|GetDead _attack_target))
        (CallFunction|GetDialoguePlayerName)
        (bind _asbp_player (Utilities|Casting|CastToBP_Player (Pawn|GetControlledPawn)))
        (bind _asdialogue_box_ui (Utilities|Casting|CastToDialogueBoxUI (UserInterface|GetUserWidgetObject (Variables|/Game/Blueprint/BP_Player.BP_Player_C|GetDialogueWidget _asbp_player))))
        (if Sure
          (Default|ForceUpdateDialogueText _asdialogue_box_ui (.OutItem (Utilities|Array|Random (Utilities|Array|MakeArray (Utilities|Text|ToText(String) (Utilities|String|Append (Utilities|String|ToString(Text) (Variables|Default|GetDialogue%20Target%20Name)) (Utilities|String|ToString(Text) (Variables|Default|GetIs)) (Utilities|String|ToString(Text) (Variables|Default|GetSus)))) (Utilities|Text|ToText(String) (Utilities|String|Append (Utilities|String|ToString(Text) (Variables|Default|GetIt's)) (Utilities|String|ToString(Text) (Variables|Default|GetDialogue%20Target%20Name)) (Utilities|String|ToString(Text) (Variables|Default|Get!!!))))))) false _isnamelessmode)
          (else
            (Default|UpdateDialogueText _asdialogue_box_ui (Utilities|Text|ToText(String) (Utilities|String|Append (Utilities|String|ToString(Text) (.OutItem (Utilities|Array|Random (Utilities|Array|MakeArray (Variables|Default|GetIThink) (Variables|Default|GetIGuess))))) (Utilities|String|ToString(Text) (Variables|Default|GetDialogue%20Target%20Name)) (Utilities|String|ToString(Text) (.OutItem (Utilities|Array|Random (Utilities|Array|MakeArray (Variables|Default|GetIsSus) (Variables|Default|GetIsTheTraitor))))))) (not (Variables|Default|GetDuelMode)) _isnamelessmode)))))))

(fn TriggerInitialDialogue
  (bind _asbp_player (Utilities|Casting|CastToBP_Player (Pawn|GetControlledPawn)))
  (bind _asdialogue_box_ui (Utilities|Casting|CastToDialogueBoxUI (UserInterface|GetUserWidgetObject (Variables|/Game/Blueprint/BP_Player.BP_Player_C|GetDialogueWidget _asbp_player))))
  (Default|UpdateDialogueText _asdialogue_box_ui (.OutItem (Utilities|Array|Random (Utilities|Array|MakeArray (Variables|Default|GetStartDialogue1) (Variables|Default|GetStartDialogue2) (Variables|Default|GetStartDialogue3) (Variables|Default|GetStartDialogue4)))) true (Variables|/Game/UI/BP_GameInstance.BP_GameInstance_C|GetisNamelessMode (Variables|Default|GetAs%20BP%20Game%20Instance))))

(fn CacheDialogueBox)

(fn EnableDuelMode
  (AI|Components|Blackboard|SetValueasBool (Variables|Default|GetPlayerAI_Blackboard) (Variables|Default|GetIsDuelModeKeyName) true)
  (Variables|Default|SetDuelMode true))

(fn TriggerDuelDialogue
  (bind _as_bp_game_instance (Variables|Default|GetAs%20BP%20Game%20Instance))
  (bind _as_bp_game_mode (Variables|Default|GetAs%20BP%20Game%20Mode))
  (bind _canbepaused (Variables|/Game/Blueprint/BP_GameMode.BP_GameMode_C|GetCanBePaused _as_bp_game_mode))
  (bind _isnamelessmode (Variables|/Game/UI/BP_GameInstance.BP_GameInstance_C|GetisNamelessMode _as_bp_game_instance))
  (bind _asbp_player (Utilities|Casting|CastToBP_Player (Pawn|GetControlledPawn)))
  (if (not (Variables|/Game/Blueprint/BP_Player.BP_Player_C|GetDead _asbp_player))
    (bind _asdialogue_box_ui (Utilities|Casting|CastToDialogueBoxUI (UserInterface|GetUserWidgetObject (Variables|/Game/Blueprint/BP_Player.BP_Player_C|GetDialogueWidget _asbp_player))))
    (if (Variables|/Game/Blueprint/BP_Player.BP_Player_C|GetCanAttack _asbp_player)
      (Default|UpdateDialogueText _asdialogue_box_ui (.OutItem (Utilities|Array|Random (Utilities|Array|MakeArray (Variables|Default|GetDuelDialogue1) (Variables|Default|GetDuelDialogue2) (Variables|Default|GetDuelDialogue3) (Variables|Default|GetDuelDialogue4)))) _canbepaused _isnamelessmode)
      (else
        (Default|UpdateDialogueText _asdialogue_box_ui (.OutItem (Utilities|Array|Random (Utilities|Array|MakeArray (Variables|Default|GetDuelDialogue_NoGlove1) (Variables|Default|GetDuelDialogue_NoGlove2) (Variables|Default|GetDuelDialogue_NoGlove3)))) _canbepaused _isnamelessmode)))))

(fn CacheGameMode
  (bind _asbp_game_mode (Utilities|Casting|CastToBP_GameMode (Game|GetGameMode)))
  (bind _output_get (Variables|Default|SetAs%20BP%20Game%20Mode _asbp_game_mode))
  (return _output_get))

(fn CacheGameInstance
  (bind _asbp_game_instance (Utilities|Casting|CastToBP_GameInstance (Game|GetGameInstance)))
  (Variables|Default|SetAs%20BP%20Game%20Instance _asbp_game_instance))

(fn HideDialogueBoxforNamelessMode
  (if (Variables|/Game/UI/BP_GameInstance.BP_GameInstance_C|GetisNamelessMode (Variables|Default|GetAs%20BP%20Game%20Instance))
    (bind _asbp_player (Utilities|Casting|CastToBP_Player (Pawn|GetControlledPawn)))
    (Widget|RemovefromParent (UserInterface|GetUserWidgetObject (Variables|/Game/Blueprint/BP_Player.BP_Player_C|GetDialogueWidget _asbp_player)))))

(fn TriggerDeadDialogue
  (params (Damage%20Causer%20Name :type Text) (Killed%20By%20Bomb? :type Boolean))
  (bind _as_bp_game_instance (Variables|Default|GetAs%20BP%20Game%20Instance))
  (bind _duelmode (Variables|Default|GetDuelMode))
  (bind _returnvalue (not _duelmode))
  (bind _isnamelessmode (Variables|/Game/UI/BP_GameInstance.BP_GameInstance_C|GetisNamelessMode _as_bp_game_instance))
  (bind _asbp_player (Utilities|Casting|CastToBP_Player (Pawn|GetControlledPawn)))
  (bind _asdialogue_box_ui (Utilities|Casting|CastToDialogueBoxUI (UserInterface|GetUserWidgetObject (Variables|/Game/Blueprint/BP_Player.BP_Player_C|GetDialogueWidget _asbp_player))))
  (if Killed%20By%20Bomb?
    (Default|ForceUpdateDialogueText _asdialogue_box_ui (Utilities|Text|ToText(String) (Utilities|String|Append (Utilities|String|ToString(Text) Damage%20Causer%20Name) (Utilities|String|ToString(Text) (Variables|Default|Getbombed%20me)))) _returnvalue _isnamelessmode)
    (else
      (Default|ForceUpdateDialogueText _asdialogue_box_ui (Utilities|Text|ToText(String) (Utilities|String|Append (Utilities|String|ToString(Text) Damage%20Causer%20Name) (Utilities|String|ToString(Text) (Variables|Default|Getpunched%20me)))) _returnvalue _isnamelessmode))))