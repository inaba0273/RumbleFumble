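; BP_IdChange_Innocent is an overlap trigger that turns a traitor BP_Player back into an innocent.
; On overlap it clears IsTraitor, plays a sound and particle, and refreshes the player's identity widget.
; It stops that player's vibration unless they hold the detective item, then decrements traitor-overlap counts on players within their detector, stopping vibration at zero.
; The PLAY VFX AND SFX function only prints a "become Traitor" message and is not called here.
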(event EventBeginPlay)

(event Collision|EventActorBeginOverlap
  (params (OtherActor :type Actor%20Object%20Reference))
  (bind _asbp_player (Utilities|Casting|CastToBP_Player OtherActor))
  (if (Variables|/Game/Blueprint/BP_Player.BP_Player_C|GetIsTraitor _asbp_player)
    (Variables|/Game/Blueprint/BP_Player.BP_Player_C|SetIsTraitor _asbp_player false)
    (Audio|PlaySoundatLocation "/Game/Assets/Sounds/EnvironmentSFX/SpeedUP_1.SpeedUP_1" (Transformation|GetActorLocation) "0, 0, 0" 1.0 0.75 0.0 0 0 0)
    (Components|Activation|Activate (Variables|/Game/Blueprint/BP_Player.BP_Player_C|GetIdChangeParticle_Innocent _asbp_player) false)
    (bind _asplayer_identity_ui (Utilities|Casting|CastToPlayerIdentityUI (UserInterface|GetUserWidgetObject (Variables|/Game/Blueprint/BP_Player.BP_Player_C|GetPlayer%20Identity%20Widget _asbp_player))))
    (Default|UpdatePlayerIdentityText _asplayer_identity_ui _asbp_player)
    (if (Variables|/Game/Blueprint/BP_Player.BP_Player_C|GethasDetectiveItem _asbp_player)
      _
      (else
        (Default|ControllerStopVibration _asbp_player)))
    (Utilities|IsValid _asbp_player
      (:Is%20Valid
        (for _array_element (Collision|GetOverlappingActors (Variables|/Game/Blueprint/BP_Player.BP_Player_C|GetDetectorCollider _asbp_player) "/Game/Blueprint/BP_Player.BP_Player_C" :!class /Script/Engine.PrimitiveComponent)
          (if (not (== _array_element _asbp_player))
            (bind _asbp_player_2 (Utilities|Casting|CastToBP_Player _array_element))
            (Math|Integer|DecrementInt (Variables|/Game/Blueprint/BP_Player.BP_Player_C|GetOverlap%20Traitor%20Count _asbp_player_2)
              (:%20%20
                (if (== (Variables|/Game/Blueprint/BP_Player.BP_Player_C|GetOverlap%20Traitor%20Count _asbp_player_2) 0)
                  (Variables|/Game/Blueprint/BP_Player.BP_Player_C|SetIsOverlappingWithTraitor _asbp_player_2 false)
                  (Default|ControllerStopVibration _asbp_player_2))))))))))

(fn ConstructionScript)

(fn PLAYVFXANDSFX
  (params (BP_Player :type BP%20Player%20Object%20Reference))
  (Development|PrintString (Utilities|String|Append (Utilities|GetObjectName BP_Player) " become " " Traitor")))