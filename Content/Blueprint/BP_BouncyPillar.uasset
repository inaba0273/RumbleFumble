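; BP_BouncyPillar is an actor that bounces the player away when they hit it.
; On hit it plays a bounce sound, then launches BP_Player along the player's forward vector mirrored by the hit normal, scaled by BounceForce.
; A DoOnce gate reset after a short random delay throttles repeat bounces, though a non-player hit fails the cast and leaves the gate closed.
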(event EventBeginPlay)

(event Collision|EventActorBeginOverlap
  (params (OtherActor :type Actor%20Object%20Reference)))

(event EventTick
  (params (DeltaSeconds :type Float%20%28single-precision%29)))

(event Collision|EventHit
  (params (MyComp :type Primitive%20Component%20Object%20Reference) (Other :type Actor%20Object%20Reference) (OtherComp :type Primitive%20Component%20Object%20Reference) (bSelfMoved :type Boolean) (HitLocation :type Vector :default "0, 0, 0") (HitNormal :type Vector :default "0, 0, 0") (NormalImpulse :type Vector :default "0, 0, 0") (Hit :type Hit%20Result%20Structure%20%28by%20ref%29))
  (Utilities|FlowControl|DoOnce false :!label _label
    (:Completed
      (Audio|PlaySoundatLocation "/Game/Assets/Sounds/EnvironmentSFX/Bounce_SoundCue.Bounce_SoundCue" HitLocation "0, 0, 0" (Math|Random|RandomFloatinRange 0.45 0.5) 1.0 0.0 0 0 0)
      (bind _asbp_player (Utilities|Casting|CastToBP_Player Other))
      (Character|LaunchCharacter _asbp_player (* (Math|Vector|MirrorVectorbyNormal (Transformation|GetActorForwardVector _asbp_player) (.Normal (Collision|BreakHitResult Hit))) (Variables|Default|GetBounce%20Force)) false false)
      (Utilities|FlowControl|Delay (Math|Random|RandomFloatinRange 0.15 0.22))
      (Development|PrintString "Reset")
      (goto _label Reset))))

(fn ConstructionScript)