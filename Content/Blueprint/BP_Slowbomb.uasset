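; BP_Slowbomb is a timed bomb that slows players caught in its range when it explodes.
; After a randomized delay, it lights its fuse effect and sound, then uses timers to steadily grow the mesh until detonation.
; The explosion calls PlayerFreeze on overlapping BP_Player actors, plays its effects, destroys the mesh and decrements the game mode's spawned item count.
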(event Custom|Start%20Fuze
  (Components|Activation|Activate (Variables|Default|GetFuze) false)
  (bind _returnvalue (Audio|SpawnSoundatLocation "/Game/Assets/Sounds/Bomb_Fuze.Bomb_Fuze" (Transformation|GetWorldLocation (Variables|Default|GetBomb_Mesh)) "0, 0, 0" 0.2 1.0 0.0 0 0))
  (Variables|Default|SetFuze%20Sound _returnvalue)
  (Utilities|Time|SetTimerbyFunctionName 0 "Bomb Scale Up" 0.1 true)
  (Utilities|Time|SetTimerbyFunctionName 0 "Bomb Explode" 5.0))

(event EventBeginPlay
  (|CallParentFunction)
  (Utilities|FlowControl|Delay (Math|Random|RandomFloatinRange 4.5 5.5))
  (CallFunction|StartFuze))

(event Collision|EventActorBeginOverlap
  (params (OtherActor :type Actor%20Object%20Reference))
  (|CallParentFunction OtherActor) ; This node is disabled and will not be called.\nDrag off pins to build functionality.
)

(event EventTick
  (params (DeltaSeconds :type Float%20%28single-precision%29))
  (|CallParentFunction DeltaSeconds) ; This node is disabled and will not be called.\nDrag off pins to build functionality.
)

(fn ConstructionScript
  (|CallParentFunction))

(fn BombScaleUp
  (Transformation|SetWorldScale3D (Variables|Default|GetBomb_Mesh) (+ (Variables|Default|GetNew%20Scale) "0.005000,0.005000,0.005000"))
  (Variables|Default|SetNew%20Scale (+ (Variables|Default|GetNew%20Scale) "0.005000,0.005000,0.005000")))

(fn BombExplode
  (bind _fuze_sound (Variables|Default|GetFuze%20Sound))
  (Components|Activation|Deactivate (Variables|Default|GetFuze))
  (if (Utilities|IsValid _fuze_sound)
    (Audio|Components|Audio|Stop _fuze_sound))
  (Components|Activation|Activate (Variables|Default|GetExplosion) false)
  (for _array_element (Collision|GetOverlappingActors (Variables|Default|GetBomb%20Range) "/Game/Blueprint/BP_Player.BP_Player_C" :!class /Script/Engine.PrimitiveComponent)
    (bind _asbp_player (Utilities|Casting|CastToBP_Player _array_element))
    (Default|PlayerFreeze _asbp_player)
    (Development|PrintString "PLAYER SLOW DOWN" true true "(R=0.000000,G=0.660000,B=1.000000,A=1.000000)" 8.0))
  (Class|KismetSystemLibrary|PauseTimer 0 "Bomb Scale Up")
  (bind _returnvalue (Audio|SpawnSoundatLocation "/Game/Assets/Sounds/EnvironmentSFX/Bomb_Small_Cue.Bomb_Small_Cue" (Transformation|GetWorldLocation (Variables|Default|GetExplosion)) "0, 0, 0" 0.5 1.0 0.0 0 0))
  (Variables|Default|SetExplosion%20Sound _returnvalue)
  (Components|DestroyComponent (Variables|Default|GetBomb_Mesh))
  ;[1 1 1] Not in use
  (bind _asbp_game_mode (Utilities|Casting|CastToBP_GameMode (Game|GetGameMode)))
  (Math|Integer|DecrementInt (Variables|/Game/Blueprint/BP_GameMode.BP_GameMode_C|GetSpawnedItemCount _asbp_game_mode)))