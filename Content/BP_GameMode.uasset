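; Game mode for a local multiplayer game with innocent and traitor sides and a shared fixed camera.
; On BeginPlay it derives traitor and innocent counts from the max player count, without assigning roles to players.
; It then creates the extra local players, spawns and possesses an indexed BP_Player for each, and stores them in Players.
; It points the first controller's view at the first BP_FixedCamera found in the level.
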(event Custom|Find%20Camera%20Actor
  (bind _outactors (Actor|GetAllActorsOfClass "/Game/BP_FixedCamera.BP_FixedCamera_C"))
  (Variables|Default|SetMainCamera (Utilities|Array|Get(acopy) _outactors)))

(event EventBeginPlay
  (Utilities|FlowControl|Sequence
    (:then_0
      (CallFunction|SetInnocentandTraitorCount)
      (CallFunction|SpawnPlayers)
      (CallFunction|FindCameraActor))
    (:then_1
      (Game|Player|SetViewTargetwithBlend (Game|GetPlayerController 0) (Variables|Default|GetMainCamera) 0.0 "VTBlend_Linear" 0.0 false))))

(event EventTick
  (params (DeltaSeconds :type Float%20%28single-precision%29)))

(fn ConstructionScript)

(fn SpawnPlayers
  (bind _max_player_count (Variables|Default|GetMax%20Player%20Count))
  (bind _returnvalue (- _max_player_count 1))
  ;[1 1 1] Create Player 1, 2, 3
  (for _index (range 1 _returnvalue)
    (Class|GameplayStatics|CreatePlayer _index))
  ;[1 1 1] Spawn and Posses Player Character 0, 1, 2, 3
  (for _index_2 (range 0 _returnvalue)
    (bind _returnvalue_2 (Game|SpawnActorfromClass "/Game/BP_Player.BP_Player_C" (Math|Transform|MakeTransform "0, 0,2000.000000") "Undefined" 0 _index_2 1e+01 false false 0))
    (Pawn|Possess (Game|GetPlayerController _index_2) _returnvalue_2)
    (Utilities|Array|AddUnique (Variables|Default|GetPlayers) _returnvalue_2)))

(fn SetInnocentandTraitorCount
  (switch int (Variables|Default|GetMax%20Player%20Count)
    (:4
      (Variables|Default|SetTraitor%20Count 1))
    (:5
      (Variables|Default|SetTraitor%20Count 2))
    (:6
      (Variables|Default|SetTraitor%20Count 2))
    (:7
      (Variables|Default|SetTraitor%20Count 3))
    (:8
      (Variables|Default|SetTraitor%20Count 3)))
  (Variables|Default|SetInnocent%20Count (- (Variables|Default|GetMax%20Player%20Count) (Variables|Default|GetTraitor%20Count))))