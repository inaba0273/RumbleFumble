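; Conveyor belt actor that carries overlapping actors along its mesh's forward vector and periodically reverses direction.
; Tick offsets each actor inside the Box by Speed and delta time, without sweeping.
; The construction script creates a dynamic material for arrow color, scale and scroll speed.
; After a startup delay, a looping timer with random extra delay flips Speed and arrow scale, printing a debug message.
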(event Custom|Change%20Conveyer%20Direction
  (Utilities|FlowControl|Delay (Math|Random|RandomFloatinRange 0.0 8.0))
  (CallFunction|ChangeDirection))

(event EventBeginPlay
  (Utilities|FlowControl|Delay 15.0)
  (Utilities|Time|SetTimerbyEvent (delegate Custom|Change%20Conveyer%20Direction) 8.0 true))

(event EventTick
  (params (DeltaSeconds :type Float%20%28single-precision%29))
  (for _array_element (Collision|GetOverlappingActors (Variables|Default|GetBox) 0 :!class /Script/Engine.PrimitiveComponent)
    (Transformation|AddActorWorldOffset _array_element (* (Math|Vector|GetForwardVector (Transformation|GetWorldRotation (Variables|Default|GetStaticMesh))) (* DeltaSeconds (Variables|Default|GetSpeed))))))

(fn ConstructionScript
  (bind _staticmesh (Variables|Default|GetStaticMesh))
  (bind _returnvalue (Rendering|Material|CreateDynamicMaterialInstance _staticmesh 0 "/Game/Meshes/Conveyer/Comveyer_M.Comveyer_M" "None" :!class /Script/Engine.PrimitiveComponent))
  (Variables|Default|SetArrow%20Material%20Instance _returnvalue)
  (Rendering|Material|SetMaterial _staticmesh 0 _returnvalue)
  (Rendering|Material|SetVectorParameterValue _returnvalue "Color" (Variables|Default|GetColor) :!class /Script/Engine.MaterialInstanceDynamic)
  (Rendering|Material|SetScalarParameterValue _returnvalue "X Scale" (Variables|Default|GetArrow%20Scales) :!class /Script/Engine.MaterialInstanceDynamic)
  (Rendering|Material|SetScalarParameterValue _returnvalue "X Speed" (Variables|Default|GetArrow%20Speed) :!class /Script/Engine.MaterialInstanceDynamic))

(fn ChangeDirection
  (Variables|Default|SetSpeed (* -1 (Variables|Default|GetSpeed)))
  (Rendering|Material|SetScalarParameterValue (Variables|Default|GetArrow%20Material%20Instance) "X Scale" (* -1 (Variables|Default|GetArrow%20Scales)) :!class /Script/Engine.MaterialInstanceDynamic)
  (Variables|Default|SetArrow%20Scales (* -1 (Variables|Default|GetArrow%20Scales)))
  (Development|PrintString "Direction Changed"))