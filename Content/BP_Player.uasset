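; Player pawn for a game of up to eight numbered players, with axis-driven movement and smoothed rotation of its cube mesh.
; BeginPlay teleports it to the PlayerStart tagged with its number, sets its arrow and health bar color, and fills the name widget with IsTraitor.
; Hits apply damage to the other actor (marked temporary); received damage subtracts a fixed DamageAmount, updates the health widget and destroys the pawn at zero.
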(event EventBeginPlay
  ;[1 1 1] Spawn Player and Set Player Color
  (CallFunction|SpawnFunction)
  (CallFunction|SetColor)
  ;[1 1 1] Cast to HealthUI and set Health Bar color
  (CallFunction|GetHealthUIReference)
  ;[1 1 1] Cast to Player Name UI and set Player Name
  (CallFunction|DisplayPlayerNameUI))

(event EventTick
  (params (DeltaSeconds :type Float%20%28single-precision%29))
  ;[1 1 1] Rotate Character when received input
  (CallFunction|CharacterRotation DeltaSeconds))

(event Game|Damage|EventAnyDamage
  (params (Damage :type Float%20%28single-precision%29) (DamageType :type Damage%20Type%20Object%20Reference) (InstigatedBy :type Controller%20Object%20Reference) (DamageCauser :type Actor%20Object%20Reference))
  (bind _damage_amount (Variables|Default|GetDamage%20Amount))
  ;[1 1 1] Decrease Health when damaged
  (bind _health (CallFunction|DecreaseHealth _damage_amount))
  (Development|PrintString (Utilities|String|Append "Player " (Utilities|String|ToString(Integer) (Variables|Default|GetplayerInt)) "  health decreased by " (Utilities|String|ToString(Float) _damage_amount) ", current health is " (Utilities|String|ToString(Float) _health)))
  (Variables|/Game/UI/HealthUI.HealthUI_C|SetHealth (Variables|Default|GetHealth%20Widget%20REF) (Variables|Default|GetHealth))
  (if (<= _health 0.0)
    (Variables|Default|SetDead true)
    (Actor|DestroyActor)))

(event Collision|EventHit
  (params (MyComp :type Primitive%20Component%20Object%20Reference) (Other :type Actor%20Object%20Reference) (OtherComp :type Primitive%20Component%20Object%20Reference) (bSelfMoved :type Boolean) (HitLocation :type Vector :default "0, 0, 0") (HitNormal :type Vector :default "0, 0, 0") (NormalImpulse :type Vector :default "0, 0, 0") (Hit :type Hit%20Result%20Structure%20%28by%20ref%29))
  ;[1 1 1] When player collide with other player, will deal damage //TO BE CHANGED LATER
  (CallFunction|DealDamage Other))

(event Input|ActionEvents|InputActionSelfDestroy
  (params (Key :type Key%20Structure :default "None"))
  ;[1 1 1] Self Kill Debug Button
  (:Pressed
    (Actor|DestroyActor)))

(event Input|AxisEvents|InputAxisMoveForward
  (params (AxisValue :type Float%20%28single-precision%29))
  ;[1 1 1] Basic Movements
  (Pawn|Input|AddMovementInput (Math|Vector|MakeVector (Variables|Default|GetmoveSpeed) 0.0 0.0) AxisValue false))

(event Input|AxisEvents|InputAxisMoveRight
  (params (AxisValue :type Float%20%28single-precision%29))
  ;[1 1 1] Basic Movements
  (Pawn|Input|AddMovementInput (Math|Vector|MakeVector 0.0 (Variables|Default|GetmoveSpeed) 0.0) AxisValue false))

(fn ConstructionScript)

(fn SpawnFunction
  ;[1 1 1] Get All Possible Spawn Point In The Level
  (bind _outactors (Actor|GetAllActorsOfClass "/Script/Engine.PlayerStart"))
  (for _array_element _outactors
    ;[1 1 1] Set Player Spawn Point
    (if (Utilities|Name|Equal(Name) (Variables|/Script/Engine.PlayerStart|GetPlayerStartTag _array_element) (Utilities|String|StringToName (Utilities|String|Append "player" (Utilities|String|ToString(Integer) (Variables|Default|GetplayerInt)))))
      (bind _output_get (Variables|Default|SetspawnLocation (Transformation|GetActorTransform _array_element)))
      (Transformation|SetActorTransform _output_get false true))))

(fn SetColor
  (bind _player5color (Variables|Default|GetPlayer5Color))
  (bind _player1color (Variables|Default|GetPlayer1Color))
  (bind _player2color (Variables|Default|GetPlayer2Color))
  (bind _player3color (Variables|Default|GetPlayer3Color))
  (bind _player4color (Variables|Default|GetPlayer4Color))
  (bind _arrow1 (Variables|Default|GetArrow1))
  (bind _player8color (Variables|Default|GetPlayer8Color))
  (bind _player7color (Variables|Default|GetPlayer7Color))
  (bind _player6color (Variables|Default|GetPlayer6Color))
  (switch int (Variables|Default|GetplayerInt)
    (:0
      (Components|Arrow|SetArrowColor(LinearColor) _arrow1 _player1color)
      (Variables|Default|SetCurrentPlayerColor _player1color))
    (:1
      (Components|Arrow|SetArrowColor(LinearColor) _arrow1 _player2color)
      (Variables|Default|SetCurrentPlayerColor _player2color))
    (:2
      (Components|Arrow|SetArrowColor(LinearColor) _arrow1 _player3color)
      (Variables|Default|SetCurrentPlayerColor _player3color))
    (:3
      (Components|Arrow|SetArrowColor(LinearColor) _arrow1 _player4color)
      (Variables|Default|SetCurrentPlayerColor _player4color))
    (:4
      (Components|Arrow|SetArrowColor(LinearColor) _arrow1 _player5color)
      (Variables|Default|SetCurrentPlayerColor _player5color))
    (:5
      (Components|Arrow|SetArrowColor(LinearColor) _arrow1 _player6color)
      (Variables|Default|SetCurrentPlayerColor _player6color))
    (:6
      (Components|Arrow|SetArrowColor(LinearColor) _arrow1 _player7color)
      (Variables|Default|SetCurrentPlayerColor _player7color))
    (:7
      (Components|Arrow|SetArrowColor(LinearColor) _arrow1 _player8color)
      (Variables|Default|SetCurrentPlayerColor _player8color))))

(fn DealDamage
  (params (DamagedActor :type Actor%20Object%20Reference))
  (Game|Damage|ApplyDamage DamagedActor (Variables|Default|GetDamage%20Amount) 0 0))

(fn DecreaseHealth
  (params (Damage :type Float%20%28single-precision%29))
  (bind _output_get (Variables|Default|SetHealth (- (Variables|Default|GetHealth) Damage)))
  (return _output_get))

(fn CharacterRotation
  (params (A :type Float%20%28single-precision%29))
  (if (or (!= (Input|AxisValues|GetMoveForward) 0.0) (!= (Input|AxisValues|GetMoveRight) 0.0))
    ;[1 1 1] Set Wanted Direction
    (Variables|Default|Setdirection (Math|Vector|MakeVector (Input|AxisValues|GetMoveForward) (Input|AxisValues|GetMoveRight) 0.0))
    (Transformation|SetWorldRotation (Variables|Default|GetCube) (Math|Rotator|Lerp(Rotator) (Transformation|GetWorldRotation (Variables|Default|GetCube)) (Math|Conversions|RotationFromXVector (Variables|Default|Getdirection)) (* A (Variables|Default|GetrotationSpeed)) true) false false)))

(fn IsAlive
  (return (not (Variables|Default|GetDead))))

(fn GetReferencefromHealthUI
  (bind _ashealth_ui (Utilities|Casting|CastToHealthUI (UserInterface|GetUserWidgetObject (Variables|Default|GetHealth%20Bar))))
  (Variables|Default|SetHealth%20Widget%20REF _ashealth_ui))

(fn SetHealthBarColor
  (Appearance|SetColorandOpacity (Variables|Default|GetHealth%20Widget%20REF) (Variables|Default|GetCurrentPlayerColor) :!class /Script/UMG.UserWidget))

(fn DisplayPlayerNameUI
  (bind _asplayer_name_ui (Utilities|Casting|CastToPlayerNameUI (UserInterface|GetUserWidgetObject (Variables|Default|GetPlayer%20Name%20Widget))))
  (bind _output_get (Variables|Default|SetPlayerName%20REF _asplayer_name_ui))
  (Variables|/Game/UI/PlayerNameUI.PlayerNameUI_C|SetPlayerName _output_get (Utilities|Text|ToText(Boolean) (Variables|Default|GetIsTraitor))))

(fn GetHealthUIReference
  (bind _ashealth_ui (Utilities|Casting|CastToHealthUI (UserInterface|GetUserWidgetObject (Variables|Default|GetHealth%20Bar))))
  (bind _output_get (Variables|Default|SetHealth%20Widget%20REF _ashealth_ui))
  (Appearance|SetColorandOpacity _output_get (Variables|Default|GetCurrentPlayerColor) :!class /Script/UMG.UserWidget))