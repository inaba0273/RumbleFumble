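; Level pipe actor that teleports any actor entering one of its four pipe openings to the exit of the opposite pipe.
; BeginPlay binds overlap events on the left, right, front and back entry components, pairing left with right and front with back.
; A shared TeleportObjects function moves the overlapping actor to the target exit component's world location without sweeping, changing only position, not rotation.
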(event Custom|Enters%20Left%20Pipe
  (params (OverlappedComponent :type Primitive%20Component%20Object%20Reference) (OtherActor :type Actor%20Object%20Reference) (OtherComp :type Primitive%20Component%20Object%20Reference) (OtherBodyIndex :type Integer) (bFromSweep :type Boolean) (SweepResult :type Hit%20Result%20Structure%20%28by%20ref%29))
  (CallFunction|TeleportObjects OtherActor (Variables|Default|GetPipe_Right_Out)))

(event Custom|Enters%20Right%20Pipe
  (params (OverlappedComponent :type Primitive%20Component%20Object%20Reference) (OtherActor :type Actor%20Object%20Reference) (OtherComp :type Primitive%20Component%20Object%20Reference) (OtherBodyIndex :type Integer) (bFromSweep :type Boolean) (SweepResult :type Hit%20Result%20Structure%20%28by%20ref%29))
  (CallFunction|TeleportObjects OtherActor (Variables|Default|GetPipe_Left_Out)))

(event Custom|Enters%20Front%20Pipe
  (params (OverlappedComponent :type Primitive%20Component%20Object%20Reference) (OtherActor :type Actor%20Object%20Reference) (OtherComp :type Primitive%20Component%20Object%20Reference) (OtherBodyIndex :type Integer) (bFromSweep :type Boolean) (SweepResult :type Hit%20Result%20Structure%20%28by%20ref%29))
  (CallFunction|TeleportObjects OtherActor (Variables|Default|GetPipe_Back_Out)))

(event Custom|Enters%20Back%20Pipe
  (params (OverlappedComponent :type Primitive%20Component%20Object%20Reference) (OtherActor :type Actor%20Object%20Reference) (OtherComp :type Primitive%20Component%20Object%20Reference) (OtherBodyIndex :type Integer) (bFromSweep :type Boolean) (SweepResult :type Hit%20Result%20Structure%20%28by%20ref%29))
  (CallFunction|TeleportObjects OtherActor (Variables|Default|GetPipe_Front_Out)))

(event EventBeginPlay
  (Collision|BindEventtoOnComponentBeginOverlap (Variables|Default|GetPipe_Left_In) (delegate Custom|Enters%20Left%20Pipe))
  (Collision|BindEventtoOnComponentBeginOverlap (Variables|Default|GetPipe_Right_In) (delegate Custom|Enters%20Right%20Pipe))
  (Collision|BindEventtoOnComponentBeginOverlap (Variables|Default|GetPipe_Front_In) (delegate Custom|Enters%20Front%20Pipe))
  (Collision|BindEventtoOnComponentBeginOverlap (Variables|Default|GetPipe_Back_In) (delegate Custom|Enters%20Back%20Pipe)))

(event Collision|EventActorBeginOverlap
  (params (OtherActor :type Actor%20Object%20Reference)))

(event EventTick
  (params (DeltaSeconds :type Float%20%28single-precision%29)))

(fn ConstructionScript)

(fn TeleportObjects
  (params (Object%20To%20Be%20Teleported :type Actor%20Object%20Reference) (Target%20Location :type Scene%20Component%20Object%20Reference))
  (Transformation|SetActorLocation Object%20To%20Be%20Teleported (Transformation|GetWorldLocation Target%20Location) false true))